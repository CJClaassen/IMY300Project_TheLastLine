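; Player controller for the top-down game that drives the Knight pawn's camera-relative movement, mouse-facing aim, attack, block, abilities, camera zoom and pausing.
; Interact activates props in range for points or picks up ability cards.
; Discard and swap modes repurpose the Q, E and R ability keys to edit slots.
; Notify functions push slot, level, cooldown and interaction-prompt changes to the HUD's gameplay widget.
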(event Custom|LookAtMouse
  (bind _returnvalue (Pawn|GetControlledPawn))
  (bind (_hitresult _returnvalue_2) (Game|Player|GetHitResultUnderCursorbyChannel "TraceTypeQuery1" true))
  ;[1 1 1] Look At Mouse
  (Utilities|IsValid _returnvalue
    (:Is%20Valid
      (if (and _returnvalue_2 (not (Variables|Default|GetpreventInput)))
        (Transformation|SetActorRotation _returnvalue (Math|Rotator|MakeRotator 0.0 0.0 (.yaw (Math|Conversions|RotationFromXVector (Math|Vector|GetUnitDirection(Vector) (Transformation|GetActorLocation _returnvalue) (.Location (Collision|BreakHitResult _hitresult)))))))
        (else
          (Transformation|SetActorRotation _returnvalue (Variables|Default|GetPlayerRotation)))))))

(event EventBeginPlay
  ;[1 1 1] Initialize player movement
  (Variables|Default|SetbShowMouseCursor true)
  (bind _asabstract_character (Utilities|Casting|CastToAbstractCharacter (Pawn|GetControlledPawn)))
  (Variables|/Game/Characters/AbstractCharacter.AbstractCharacter_C|SetplayerIndex _asabstract_character (Class|GameplayStatics|GetPlayerControllerID self))
  (Variables|/Game/Characters/AbstractCharacter.AbstractCharacter_C|SetisAI _asabstract_character false)
  (Variables|/Script/Engine.CharacterMovementComponent|SetMaxWalkSpeed (Variables|/Script/Engine.Character|GetCharacterMovement _asabstract_character) (Variables|/Game/Characters/AbstractCharacter.AbstractCharacter_C|GetMovementSpeed _asabstract_character))
  (bind _astop_down_game_mode (Utilities|Casting|CastToTopDownGameMode (Game|GetGameMode)))
  (Default|PlayLevelAmbience _astop_down_game_mode)
  (bind _astop_down_game_mode_2 (Utilities|Casting|CastToTopDownGameMode (Game|GetGameMode)))
  (Variables|Default|SetGameMode _astop_down_game_mode_2))

(event EventTick
  (params (DeltaSeconds :type Float%20%28single-precision%29))
  (Variables|Default|SetDeltaSeconds DeltaSeconds)
  (if (not (Game|IsGamePaused))
    (CallFunction|LookatMouse)
    (CallFunction|UpdatePlayerRotationandZoom)))

(event Input|ActionEvents|InputActionAbilityE
  (params (Key :type Key%20Structure))
  ;[1 1 1] Ability Activations
  (:Pressed
    (if (not (Variables|Default|GetisDiscarding))
      (if (not (Variables|Default|GetisSwapping))
        ;;[1 1 1] Cast Ability E
        (bind _asabstract_character (Utilities|Casting|CastToAbstractCharacter (Pawn|GetControlledPawn)))
        (Default|AbilityE _asabstract_character)
        (else
          ;;[1 1 1] Swap Abilities with E
          (if (!= (Variables|Default|GetSelectedAbility1) -1)
            (bind _asknight_bp (Utilities|Casting|CastToKnight_BP (Pawn|GetControlledPawn)))
            (bind _successfull (Default|SwapAbilities _asknight_bp (Variables|Default|GetSelectedAbility1) 1))
            (if _successfull
              (CallFunction|NotifyonSwap (Variables|Default|GetSelectedAbility1) 1)
              (else
                (Variables|Default|SetSelectedAbility1 -1)))
            (Variables|Default|SetisSwapping false)
            (bind _asuser_interface_hud (Utilities|Casting|CastToUserInterfaceHud (HUD|GetHUD)))
            (Default|ToggleSwaponCards (Variables|/Game/UI/UserInterfaceHud.UserInterfaceHud_C|GetGameplayWidget _asuser_interface_hud))
            (else
              (Variables|Default|SetSelectedAbility1 1)
              (bind _asuser_interface_hud_2 (Utilities|Casting|CastToUserInterfaceHud (HUD|GetHUD)))
              (Default|SelectAbilityforSwap (Variables|/Game/UI/UserInterfaceHud.UserInterfaceHud_C|GetGameplayWidget _asuser_interface_hud_2) (Variables|Default|GetSelectedAbility1))
              (if (Variables|/Game/GameData/GameModes/TopDownGameMode.TopDownGameMode_C|GetisTutorial (Variables|Default|GetGameMode))
                _)))))
      (else
        ;;[1 1 1] Discards Ability E
        (bind _asknight_bp_2 (Utilities|Casting|CastToKnight_BP (Pawn|GetControlledPawn)))
        (Default|DiscardAbility _asknight_bp_2 1)
        (Variables|Default|SetisDiscarding false)
        (Math|Integer|DecrementInt (Variables|Default|GetNumberOfAbilities)
          (:%20%20
            (CallFunction|NotifyonAbilityChange 1)
            (bind _asuser_interface_hud_3 (Utilities|Casting|CastToUserInterfaceHud (HUD|GetHUD)))
            (Default|ToggleDiscardonCards (Variables|/Game/UI/UserInterfaceHud.UserInterfaceHud_C|GetGameplayWidget _asuser_interface_hud_3))))))))

(event Input|ActionEvents|InputActionAbilityQ
  (params (Key :type Key%20Structure))
  ;[1 1 1] Ability Activations
  (:Pressed
    (if (not (Variables|Default|GetisDiscarding))
      (if (not (Variables|Default|GetisSwapping))
        ;;[1 1 1] Casting ability Q
        (bind _asabstract_character (Utilities|Casting|CastToAbstractCharacter (Pawn|GetControlledPawn)))
        (Default|AbilityQ _asabstract_character)
        (else
          ;;[1 1 1] Swap Abilities with Q
          (if (!= (Variables|Default|GetSelectedAbility1) -1)
            (bind _asknight_bp (Utilities|Casting|CastToKnight_BP (Pawn|GetControlledPawn)))
            (bind _successfull (Default|SwapAbilities _asknight_bp (Variables|Default|GetSelectedAbility1)))
            (if _successfull
              (CallFunction|NotifyonSwap (Variables|Default|GetSelectedAbility1))
              (else
                (Variables|Default|SetSelectedAbility1 -1)))
            (Variables|Default|SetisSwapping false)
            (bind _asuser_interface_hud (Utilities|Casting|CastToUserInterfaceHud (HUD|GetHUD)))
            (Default|ToggleSwaponCards (Variables|/Game/UI/UserInterfaceHud.UserInterfaceHud_C|GetGameplayWidget _asuser_interface_hud))
            (else
              (Variables|Default|SetSelectedAbility1 0)
              (bind _asuser_interface_hud_2 (Utilities|Casting|CastToUserInterfaceHud (HUD|GetHUD)))
              (Default|SelectAbilityforSwap (Variables|/Game/UI/UserInterfaceHud.UserInterfaceHud_C|GetGameplayWidget _asuser_interface_hud_2) (Variables|Default|GetSelectedAbility1))
              (if (Variables|/Game/GameData/GameModes/TopDownGameMode.TopDownGameMode_C|GetisTutorial (Variables|Default|GetGameMode))
                _)))))
      (else
        ;;[1 1 1] Discards Ability Q
        (bind _asknight_bp_2 (Utilities|Casting|CastToKnight_BP (Pawn|GetControlledPawn)))
        (Default|DiscardAbility _asknight_bp_2)
        (Variables|Default|SetisDiscarding false)
        (Math|Integer|DecrementInt (Variables|Default|GetNumberOfAbilities)
          (:%20%20
            (CallFunction|NotifyonAbilityChange)
            (bind _asuser_interface_hud_3 (Utilities|Casting|CastToUserInterfaceHud (HUD|GetHUD)))
            (Default|ToggleDiscardonCards (Variables|/Game/UI/UserInterfaceHud.UserInterfaceHud_C|GetGameplayWidget _asuser_interface_hud_3))))))))

(event Input|ActionEvents|InputActionAbilityR
  (params (Key :type Key%20Structure))
  ;[1 1 1] Ability Activations
  (:Pressed
    (if (not (Variables|Default|GetisDiscarding))
      (if (not (Variables|Default|GetisSwapping))
        ;;[1 1 1] Cast Ability R
        (bind _asabstract_character (Utilities|Casting|CastToAbstractCharacter (Pawn|GetControlledPawn)))
        (Default|AbilityR _asabstract_character)
        (else
          ;;[1 1 1] Swap Abilities with R
          (if (!= (Variables|Default|GetSelectedAbility1) -1)
            (bind _asknight_bp (Utilities|Casting|CastToKnight_BP (Pawn|GetControlledPawn)))
            (bind _successfull (Default|SwapAbilities _asknight_bp (Variables|Default|GetSelectedAbility1) 2))
            (if _successfull
              (CallFunction|NotifyonSwap (Variables|Default|GetSelectedAbility1) 2)
              (else
                (Variables|Default|SetSelectedAbility1 -1)))
            (Variables|Default|SetisSwapping false)
            (bind _asuser_interface_hud (Utilities|Casting|CastToUserInterfaceHud (HUD|GetHUD)))
            (Default|ToggleSwaponCards (Variables|/Game/UI/UserInterfaceHud.UserInterfaceHud_C|GetGameplayWidget _asuser_interface_hud))
            (else
              (Variables|Default|SetSelectedAbility1 2)
              (bind _asuser_interface_hud_2 (Utilities|Casting|CastToUserInterfaceHud (HUD|GetHUD)))
              (Default|SelectAbilityforSwap (Variables|/Game/UI/UserInterfaceHud.UserInterfaceHud_C|GetGameplayWidget _asuser_interface_hud_2) (Variables|Default|GetSelectedAbility1))
              (if (Variables|/Game/GameData/GameModes/TopDownGameMode.TopDownGameMode_C|GetisTutorial (Variables|Default|GetGameMode))
                _)))))
      (else
        ;;[1 1 1] Discards Ability R
        (bind _asknight_bp_2 (Utilities|Casting|CastToKnight_BP (Pawn|GetControlledPawn)))
        (Default|DiscardAbility _asknight_bp_2 2)
        (Variables|Default|SetisDiscarding false)
        (Math|Integer|DecrementInt (Variables|Default|GetNumberOfAbilities)
          (:%20%20
            (CallFunction|NotifyonAbilityChange 2)
            (bind _asuser_interface_hud_3 (Utilities|Casting|CastToUserInterfaceHud (HUD|GetHUD)))
            (Default|ToggleDiscardonCards (Variables|/Game/UI/UserInterfaceHud.UserInterfaceHud_C|GetGameplayWidget _asuser_interface_hud_3))))))))

(event Input|ActionEvents|InputActionInteract
  (params (Key :type Key%20Structure))
  (bind _abilitycard (Variables|Default|GetAbilityCard))
  (bind _propinrange (Variables|Default|GetPropInRange))
  (bind _cost (Default|GetActivationCost _propinrange))
  (bind _abilitytype (Variables|/Game/Abilities/Pickup/PickUpAbility_BP.PickUpAbility_BP_C|GetAbilityType _abilitycard))
  ;[1 1 1] Interaction execution (ussually with a prop/trap/abilities)
  (:Pressed
    (Utilities|IsValid (Variables|Default|GetPropInRange)
      (:Is%20Valid
        ;;[1 1 1] Handle the activation of the props
        (bind _asknight_bp (Utilities|Casting|CastToKnight_BP (Pawn|GetControlledPawn)))
        (if (Default|IsReady (Variables|Default|GetPropInRange))
          (if (>= (Variables|/Game/Characters/AbstractCharacter.AbstractCharacter_C|GetPoints _asknight_bp) _cost)
            (Default|UpdatePlayerPoints _asknight_bp (* -1 _cost))
            (Default|Activate (Variables|Default|GetPropInRange) (Class|GameplayStatics|GetPlayerControllerID self)))
          (else
            (Development|PrintString "Hello"))))
      (:Is%20Not%20Valid
        ;;[1 1 1] Handle the ability pickups
        (Utilities|IsValid (Variables|Default|GetAbilityCard)
          (:Is%20Valid
            (bind _asknight_bp_2 (Utilities|Casting|CastToKnight_BP (Pawn|GetControlledPawn)))
            (bind _indexassigned (Default|SetAbility _asknight_bp_2 _abilitytype))
            (if (>= _indexassigned 0)
              (CallFunction|NotifyonAbilityChange _indexassigned _abilitytype)
              (Actor|DestroyActor (Variables|Default|GetAbilityCard))))
          (:Is%20Not%20Valid
            (Development|PrintString "Out of reach")))))))

(event Input|ActionEvents|InputActionSwapAbilities
  (params (Key :type Key%20Structure))
  ;[1 1 1] Ability Activations
  ;;[1 1 1] Trigger Swapping event
  (:Pressed
    (bind _output_get (Variables|Default|SetisSwapping (not (Variables|Default|GetisSwapping))))
    (if _output_get
      (Variables|Default|SetSelectedAbility1 -1)
      (Variables|Default|SetisDiscarding false))
    (bind _asuser_interface_hud (Utilities|Casting|CastToUserInterfaceHud (HUD|GetHUD)))
    (Default|ToggleSwaponCards (Variables|/Game/UI/UserInterfaceHud.UserInterfaceHud_C|GetGameplayWidget _asuser_interface_hud))))

(event Input|ActionEvents|InputActionDiscardAbility
  (params (Key :type Key%20Structure))
  ;[1 1 1] Ability Activations
  ;;[1 1 1] Trigger Discarding event
  (:Pressed
    (Variables|Default|SetisDiscarding (not (Variables|Default|GetisDiscarding)))
    (if true
      (Variables|Default|SetSelectedAbility1 -1)
      (Variables|Default|SetisSwapping false))
    (bind _asuser_interface_hud (Utilities|Casting|CastToUserInterfaceHud (HUD|GetHUD)))
    (Default|ToggleDiscardonCards (Variables|/Game/UI/UserInterfaceHud.UserInterfaceHud_C|GetGameplayWidget _asuser_interface_hud))))

(event Input|ActionEvents|InputActionPauseGame
  (params (Key :type Key%20Structure))
  (:Pressed
    (bind _astop_down_game_mode (Utilities|Casting|CastToTopDownGameMode (Game|GetGameMode)))
    (if (or (not (Game|IsGamePaused)) (Variables|/Game/Maps/MapHandler_BP.MapHandler_BP_C|GetisTutorialDisplayed (Variables|/Game/GameData/GameModes/TopDownGameMode.TopDownGameMode_C|GetMapHandler _astop_down_game_mode)))
      (Game|SetGamePaused true)
      (bind _asuser_interface_hud (Utilities|Casting|CastToUserInterfaceHud (HUD|GetHUD)))
      (bind _widget (Default|LoadUI _asuser_interface_hud "PauseMenu"))
      (Widget|SetVisibility _widget "Visible")
      (Input|SetInputModeUIOnly self _widget "DoNotLock")
      (Variables|Default|SetbShowMouseCursor true)
      (Development|PrintString "Display menu")
      (else
        (Game|SetGamePaused false)
        (bind _asuser_interface_hud_2 (Utilities|Casting|CastToUserInterfaceHud (HUD|GetHUD)))
        (bind _widget_2 (Default|LoadUI _asuser_interface_hud_2 "PauseMenu"))
        (Widget|SetVisibility _widget_2 "Hidden")
        (Default|LoadUI _asuser_interface_hud_2 "Gameplay")
        (Development|PrintString "Hide menu")
        (Input|SetInputModeGameOnly self)
        (Variables|Default|SetbShowMouseCursor false)
        (Variables|Default|SetbShowMouseCursor false)))))

(event Input|ActionEvents|InputActionBasicAttack
  (params (Key :type Key%20Structure))
  (bind _preventinput (Variables|Default|GetpreventInput))
  (bind _returnvalue (not _preventinput))
  (:Pressed
    (Development|PrintString (Utilities|String|ToString(Boolean) _returnvalue))
    (if _returnvalue
      ;[1 1 1] Prevent click and hold
      (if (not (Variables|Default|GetAttackSequence))
        (bind _asknight_bp (Utilities|Casting|CastToKnight_BP (Pawn|GetControlledPawn)))
        (Default|TryBasicAttack _asknight_bp))))
  (:Released
    (if (not (Variables|Default|GetpreventInput))
      (Variables|Default|SetAttackSequence false))))

(event Input|ActionEvents|InputActionBlock
  (params (Key :type Key%20Structure))
  (:Pressed
    (if (not (Variables|Default|GetpreventInput))
      (bind _asknight_bp (Utilities|Casting|CastToKnight_BP (Pawn|GetControlledPawn)))
      (Default|TryBlock _asknight_bp)))
  (:Released
    (if (not (Variables|Default|GetpreventInput))
      (bind _asknight_bp_2 (Utilities|Casting|CastToKnight_BP (Pawn|GetControlledPawn)))
      (Default|ReleaseBlock _asknight_bp_2))))

(event Input|ActionEvents|InputActionZoomCamera
  (params (Key :type Key%20Structure))
  (:Pressed
    (switch string (Utilities|String|ToString(Text) (Class|KismetInputLibrary|KeyGetDisplayName Key))
      (:Mouse%20Wheel%20Up
        (bind _asabstract_character (Utilities|Casting|CastToAbstractCharacter (Pawn|GetControlledPawn)))
        (if (> (Variables|/Script/Engine.SpringArmComponent|GetTargetArmLength (Variables|/Game/Characters/AbstractCharacter.AbstractCharacter_C|GetSpringArm _asabstract_character)) 2.5e+02)
          (Variables|/Script/Engine.SpringArmComponent|SetTargetArmLength (Variables|/Game/Characters/AbstractCharacter.AbstractCharacter_C|GetSpringArm _asabstract_character) (- (Variables|/Script/Engine.SpringArmComponent|GetTargetArmLength (Variables|/Game/Characters/AbstractCharacter.AbstractCharacter_C|GetSpringArm _asabstract_character)) 5e+01))))
      (:Mouse%20Wheel%20Down
        (bind _asabstract_character_2 (Utilities|Casting|CastToAbstractCharacter (Pawn|GetControlledPawn)))
        (if (> 1.5e+03 (Variables|/Script/Engine.SpringArmComponent|GetTargetArmLength (Variables|/Game/Characters/AbstractCharacter.AbstractCharacter_C|GetSpringArm _asabstract_character_2)))
          (Variables|/Script/Engine.SpringArmComponent|SetTargetArmLength (Variables|/Game/Characters/AbstractCharacter.AbstractCharacter_C|GetSpringArm _asabstract_character_2) (+ (Variables|/Script/Engine.SpringArmComponent|GetTargetArmLength (Variables|/Game/Characters/AbstractCharacter.AbstractCharacter_C|GetSpringArm _asabstract_character_2)) 1e+02)))))))

(event Input|AxisEvents|InputAxisMoveRight
  (params (AxisValue :type Float%20%28single-precision%29))
  (bind _returnvalue (Pawn|GetControlledPawn))
  ;[1 1 1] Movement
  (if (not (Variables|Default|GetpreventInput))
    (bind _output_get (Variables|Default|SetAxisScaleRight AxisValue))
    (Utilities|IsValid _returnvalue
      (:Is%20Valid
        (Pawn|Input|AddMovementInput _returnvalue (Math|Vector|GetRightVector (Variables|/Script/Engine.PlayerCameraManager|GetTransformComponent (Variables|Default|GetPlayerCameraManager))) _output_get false)))))

(event Input|AxisEvents|InputAxisMoveUp
  (params (AxisValue :type Float%20%28single-precision%29))
  (bind _returnvalue (Pawn|GetControlledPawn))
  ;[1 1 1] Movement
  (if (not (Variables|Default|GetpreventInput))
    (bind _output_get (Variables|Default|SetAxisScale AxisValue))
    (Utilities|IsValid _returnvalue
      (:Is%20Valid
        (Pawn|Input|AddMovementInput _returnvalue (Math|Vector|GetUpVector (Variables|/Script/Engine.PlayerCameraManager|GetTransformComponent (Variables|Default|GetPlayerCameraManager))) _output_get false)))))

(fn ConstructionScript
  (Variables|Default|SetAbilityCard 0)
  (Variables|Default|SetPropInRange 0))

(fn NotifyOfInteraction
  (params (FixedDescription :type String) (Variable%20Input :type String))
  (bind _asuser_interface_hud (Utilities|Casting|CastToUserInterfaceHud (HUD|GetHUD self)))
  (if (Widget|IsVisible (Variables|/Game/UI/UserInterfaceHud.UserInterfaceHud_C|GetGameplayWidget _asuser_interface_hud))
    _
    (else
      (Default|LoadUI _asuser_interface_hud "Gameplay")))
  (Default|DisplayInteraction (Variables|/Game/UI/UserInterfaceHud.UserInterfaceHud_C|GetGameplayWidget _asuser_interface_hud) "F" FixedDescription Variable%20Input))

(fn GetAbility
  (switch string ""))

(fn RemoveInteractionNotification
  (bind _asuser_interface_hud (Utilities|Casting|CastToUserInterfaceHud (HUD|GetHUD self)))
  (if (Widget|IsVisible (Variables|/Game/UI/UserInterfaceHud.UserInterfaceHud_C|GetGameplayWidget _asuser_interface_hud))
    _
    (else
      (Default|LoadUI _asuser_interface_hud "Gameplay")))
  (Default|HideInteraction (Variables|/Game/UI/UserInterfaceHud.UserInterfaceHud_C|GetGameplayWidget _asuser_interface_hud)))

(fn NotifyonSwap
  (params (AbilityX :type Integer) (AbilityY :type Integer))
  (bind _asuser_interface_hud (Utilities|Casting|CastToUserInterfaceHud (HUD|GetHUD self)))
  (Default|LoadUI _asuser_interface_hud "Gameplay")
  (Default|UpdateAbilitySwap (Variables|/Game/UI/UserInterfaceHud.UserInterfaceHud_C|GetGameplayWidget _asuser_interface_hud) AbilityX AbilityY)
  (bind _asknight_bp (Utilities|Casting|CastToKnight_BP (Pawn|GetControlledPawn)))
  (bind _slotlevel (Default|GetAbilitySlotDetails _asknight_bp AbilityX))
  (Default|UpdateAbilityLevel (Variables|/Game/UI/UserInterfaceHud.UserInterfaceHud_C|GetGameplayWidget _asuser_interface_hud) AbilityX _slotlevel)
  (bind _asknight_bp_2 (Utilities|Casting|CastToKnight_BP (Pawn|GetControlledPawn)))
  (bind _slotlevel_2 (Default|GetAbilitySlotDetails _asknight_bp_2 AbilityY))
  (Default|UpdateAbilityLevel (Variables|/Game/UI/UserInterfaceHud.UserInterfaceHud_C|GetGameplayWidget _asuser_interface_hud) AbilityY _slotlevel_2))

(fn NotifyonAbilityChange
  (params (SlotIndex :type Integer) (AbilityType :type Cast%20Abilities%20BP%20Class%20Reference))
  (bind _asuser_interface_hud (Utilities|Casting|CastToUserInterfaceHud (HUD|GetHUD self)))
  (if (Widget|IsVisible (Variables|/Game/UI/UserInterfaceHud.UserInterfaceHud_C|GetGameplayWidget _asuser_interface_hud))
    _
    (else
      (Default|LoadUI _asuser_interface_hud "Gameplay")))
  (Default|UpdateAbilitySlot (Variables|/Game/UI/UserInterfaceHud.UserInterfaceHud_C|GetGameplayWidget _asuser_interface_hud) SlotIndex AbilityType))

(fn NotifyonAbilityLevelUp
  (params (AbilitySlotIndex :type Integer) (NewLevel :type Integer))
  (bind _asuser_interface_hud (Utilities|Casting|CastToUserInterfaceHud (HUD|GetHUD self)))
  (Default|LoadUI _asuser_interface_hud "Gameplay")
  (Default|UpdateAbilityLevel (Variables|/Game/UI/UserInterfaceHud.UserInterfaceHud_C|GetGameplayWidget _asuser_interface_hud) AbilitySlotIndex NewLevel))

(fn NotifyonPlayerLevelUp)

(fn NotifyonAbilityCast
  (params (Ability :type Cast%20Abilities%20BP%20Object%20Reference) (AbilitySlotIndex :type Integer))
  (bind _asuser_interface_hud (Utilities|Casting|CastToUserInterfaceHud (HUD|GetHUD self)))
  (if (Widget|IsVisible (Variables|/Game/UI/UserInterfaceHud.UserInterfaceHud_C|GetGameplayWidget _asuser_interface_hud))
    _
    (else
      (Default|LoadUI _asuser_interface_hud "Gameplay")))
  (Default|AbilityCastedEvent (Variables|/Game/UI/UserInterfaceHud.UserInterfaceHud_C|GetGameplayWidget _asuser_interface_hud) AbilitySlotIndex (Variables|/Game/Abilities/CastAbilities/CastAbilities_BP.CastAbilities_BP_C|GetCooldown Ability)))

(fn UpdatePlayerRotationandZoom
  (bind _zoomrate (Variables|Default|GetZoomRate))
  (if (Variables|Default|GetActivateArrows)
    (bind _asknight_bp (Utilities|Casting|CastToKnight_BP (Pawn|GetControlledPawn)))
    (bind _canchange (Default|OnCameraChange _asknight_bp (Variables|Default|GetZoom) (Variables|Default|GetTurnLeft)))
    (if _canchange
      (bind _asabstract_character (Utilities|Casting|CastToAbstractCharacter (Pawn|GetControlledPawn)))
      (switch int (Variables|Default|GetTurnLeft)
        (:Default
          (switch int (Variables|Default|GetZoom)
            (:0
              (Variables|Default|SetDistanceUpdateRate (* _zoomrate -1.0))
              (if (>= (Variables|/Script/Engine.SpringArmComponent|GetTargetArmLength (Variables|/Game/Characters/AbstractCharacter.AbstractCharacter_C|GetSpringArm _asabstract_character)) 3.5e+02)
                (Variables|/Script/Engine.SpringArmComponent|SetTargetArmLength (Variables|/Game/Characters/AbstractCharacter.AbstractCharacter_C|GetSpringArm _asabstract_character) (+ (Variables|/Script/Engine.SpringArmComponent|GetTargetArmLength (Variables|/Game/Characters/AbstractCharacter.AbstractCharacter_C|GetSpringArm _asabstract_character)) (Variables|Default|GetDistanceUpdateRate)) :!label _label)))
            (:1
              (Variables|Default|SetDistanceUpdateRate _zoomrate)
              (if (<= (Variables|/Script/Engine.SpringArmComponent|GetTargetArmLength (Variables|/Game/Characters/AbstractCharacter.AbstractCharacter_C|GetSpringArm _asabstract_character)) 2e+03)
                (goto _label)))))
        (:0
          (Variables|Default|SetTurnRate -0.5)
          (Transformation|SetWorldRotation (Variables|/Game/Characters/AbstractCharacter.AbstractCharacter_C|GetSpringArm _asabstract_character) (Math|Rotator|MakeRotator (.roll (Transformation|GetWorldRotation (Variables|/Game/Characters/AbstractCharacter.AbstractCharacter_C|GetSpringArm _asabstract_character))) (.pitch (Transformation|GetWorldRotation (Variables|/Game/Characters/AbstractCharacter.AbstractCharacter_C|GetSpringArm _asabstract_character))) (+ (.yaw (Transformation|GetWorldRotation (Variables|/Game/Characters/AbstractCharacter.AbstractCharacter_C|GetSpringArm _asabstract_character))) (Variables|Default|GetTurnRate))) false false :!label _label_2))
        (:1
          (Variables|Default|SetTurnRate 0.5)
          (goto _label_2))))))

(fn DisableMovement
  (Variables|Default|SetpreventInput true)
  (Variables|Default|SetbShowMouseCursor true))

(fn EnableMovement
  (Variables|Default|SetpreventInput false)
  (Variables|Default|SetbShowMouseCursor false))

(fn HideMouseCursor
  (Variables|Default|SetbShowMouseCursor false))

(fn ShowMouseCursor
  (Variables|Default|SetbShowMouseCursor true))