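; AI controller for skeleton enemies that chases the Knight and attacks when close.
; A looping timer started on BeginPlay periodically issues a move toward the first Knight_BP actor found in the world.
; After each move request, it checks the pawn's distance to player 0's pawn and triggers the Skeleton_BP heavy attack within range.
; The SearchForEnemy function is an empty stub.
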(event Custom|Search%20for%20Player
  (bind _returnvalue (Pawn|GetControlledPawn))
  (Utilities|IsValid _returnvalue
    (:Is%20Valid
      (bind _outactors (Actor|GetAllActorsOfClass "/Game/Characters/PlayableCharacters/Knight_BP.Knight_BP_C"))
      (AI|AIMoveTo _returnvalue (Transformation|GetActorLocation (Utilities|Array|Get(acopy) _outactors)) (Utilities|Array|Get(acopy) _outactors) 5e+01 false
        (:then
          (if (<= (Transformation|GetDistanceTo (Pawn|GetControlledPawn) (Game|Player|GetPlayerPawn 0)) 3e+02)
            (bind _asskeleton_bp (Utilities|Casting|CastToSkeleton_BP (Pawn|GetControlledPawn)))
            (Default|HeavyAttack _asskeleton_bp)))))))

(event EventBeginPlay
  (Utilities|Time|SetTimerbyEvent (delegate Custom|Search%20for%20Player) 0.5 true))

(event EventTick
  (params (DeltaSeconds :type Float%20%28single-precision%29)))

(fn ConstructionScript)

(fn SearchforEnemy
  (return 0))