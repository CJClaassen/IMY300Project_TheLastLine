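; Staff projectile that deals magic damage to the first enemy it hits, then destroys itself.
; Sphere overlap resolves the target as either an overlapped character or the holder of an overlapped item, then rejects teammates via the firing holder's team.
; A one-shot tag blocks repeat hits, damage comes from the holder, and a random sword-hit sound plays at the target.
; Debug strings print along the hit path.
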(event OnComponentBeginOverlap(Sphere)
  (params (OverlappedComponent :type Primitive%20Component%20Object%20Reference) (OtherActor :type Actor%20Object%20Reference) (OtherComp :type Primitive%20Component%20Object%20Reference) (OtherBodyIndex :type Integer) (bFromSweep :type Boolean) (SweepResult :type Hit%20Result%20Structure%20%28by%20ref%29))
  (bind _holder (Variables|Default|GetHolder))
  (Development|PrintString (Utilities|GetDisplayName OtherComp) true true "(R=1.000000,G=0.000000,B=0.000000,A=1.000000)" 1e+01)
  (Development|PrintString (Utilities|GetDisplayName OtherActor) true true "(R=1.000000,G=0.000000,B=0.000000,A=1.000000)" 1e+01)
  (Utilities|IsValid (Variables|Default|GetHolder)
    (:Is%20Valid
      (bind _asitem_bp (Utilities|Casting|CastToItemBP OtherActor)
        (:then
          (Development|PrintString "Staff Hit Object" true true "(R=1.000000,G=0.000000,B=0.000000,A=1.000000)" 1e+01)
          (Variables|Default|SetAttackedActor (Variables|/Game/Items/ItemBP.ItemBP_C|GetHolder _asitem_bp)))
        (:CastFailed
          (bind _asabstract_character (Utilities|Casting|CastToAbstractCharacter OtherActor))
          (Development|PrintString "Staff Hit Player" true true "(R=1.000000,G=0.000000,B=0.000000,A=1.000000)" 1e+01)
          (Variables|Default|SetAttackedActor _asabstract_character)))
      (Utilities|IsValid (Variables|Default|GetAttackedActor)
        (:Is%20Valid
          (if (!= (Variables|/Game/Characters/AbstractCharacter.AbstractCharacter_C|GetTeamNumber (Variables|Default|GetAttackedActor)) (Variables|Default|GetHolderTeam))
            (if (== 0 (Variables|Default|GetCurrentTag))
              (Development|PrintString "Staff Yes Damage tag" true true "(R=1.000000,G=0.000000,B=0.000000,A=1.000000)" 1e+01)
              (Variables|Default|SetCurrentTag 1)
              (Utilities|IsValid _holder
                (:Is%20Valid
                  (CallFunction|GetDamage)
                  (Audio|PlaySoundatLocation (CallFunction|ChooseSound) (Transformation|GetActorLocation (Variables|Default|GetAttackedActor)) "0, 0, 0" (* (Default|GetSoundEffectVolume (CallFunction|GetGameMode)) 0.6) 1.0 0.0 "/Game/Items/Staff/StaffProjectile_Auttenation.StaffProjectile_Auttenation" "/Game/Items/Sword/SwordHitConcurrency.SwordHitConcurrency" 0)
                  (Game|Damage|ApplyDamage (Variables|Default|GetAttackedActor) (Variables|Default|GetDamage) (Pawn|GetController _holder) 0 "/Game/GameData/Damages/DamageType_Magic.DamageType_Magic_C")
                  (Actor|DestroyActor))
                (:Is%20Not%20Valid
                  (Development|PrintString "Staff Not Valid holder" true true "(R=1.000000,G=0.000000,B=0.000000,A=1.000000)" 1e+01)))
              (else
                (Development|PrintString "Staff Not Damage tag" true true "(R=1.000000,G=0.000000,B=0.000000,A=1.000000)" 1e+01)))
            (else
              (Development|PrintString "Staff No Damge same team" true true "(R=1.000000,G=0.000000,B=0.000000,A=1.000000)" 1e+01))))))
    (:Is%20Not%20Valid
      (Development|PrintString "No Valid Holder" true true "(R=1.000000,G=0.000000,B=0.000000,A=1.000000)" 1e+01))))

(event EventBeginPlay
  (Variables|Default|SetCurrentTag 0))

(event Collision|EventActorBeginOverlap
  (params (OtherActor :type Actor%20Object%20Reference)))

(event EventTick
  (params (DeltaSeconds :type Float%20%28single-precision%29)))

(fn ConstructionScript)

(fn GetDamage
  (bind _output_get (Variables|Default|SetDamage (Variables|/Game/Characters/AbstractCharacter.AbstractCharacter_C|GetDamage (Variables|Default|GetHolder))))
  (Development|PrintString (Utilities|String|Append (Utilities|String|MakeLiteralString "Damage : ") (Utilities|String|ToString(Float) _output_get)) true true "(R=1.000000,G=0.000000,B=0.000000,A=1.000000)" 1e+01))

(fn ChooseSound
  (switch int (Math|Random|RandomIntegerinRangefromStream 0 1 (LocalVariables|GetSeed))
    (:0
      (return "/Game/Items/Sword/SwordHit2.SwordHit2"))
    (:1
      (return "/Game/Items/Sword/SwordHit3.SwordHit3"))))