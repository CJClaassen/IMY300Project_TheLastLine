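; Arrow projectile for the bow that deals physical damage to enemy characters when its box overlaps them during an attack.
; A hit on a sword redirects to its holder, then a team check and one-hit tag prevent friendly or repeat damage.
; Damage comes from the arrow's holder, with random impact sounds and debug prints.
; After hitting, the arrow stops moving, simulates physics and destroys itself after a delay.
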(event OnComponentBeginOverlap(Box)
  (params (OverlappedComponent :type Primitive%20Component%20Object%20Reference) (OtherActor :type Actor%20Object%20Reference) (OtherComp :type Primitive%20Component%20Object%20Reference) (OtherBodyIndex :type Integer) (bFromSweep :type Boolean) (SweepResult :type Hit%20Result%20Structure%20%28by%20ref%29))
  (bind _holder (Variables|Default|GetHolder))
  (Development|PrintString (Utilities|GetDisplayName OtherComp) true true "(R=1.000000,G=0.000000,B=0.000000,A=1.000000)" 0.1)
  (Development|PrintString (Utilities|GetDisplayName OtherActor) true true "(R=1.000000,G=0.000000,B=0.000000,A=1.000000)" 0.1)
  (if (Variables|Default|GetInAttack)
    (Utilities|IsValid (Variables|Default|GetHolder)
      (:Is%20Valid
        (bind _assword_1_bp (Utilities|Casting|CastToSword1_BP OtherActor)
          (:then
            (Variables|Default|SetAttackedActor (Variables|/Game/Items/Sword/Sword1_BP.Sword1_BP_C|GetHolder _assword_1_bp)))
          (:CastFailed
            (bind _asabstract_character (Utilities|Casting|CastToAbstractCharacter OtherActor))
            (Development|PrintString "Arrow Hit Player" true true "(R=1.000000,G=0.000000,B=0.000000,A=1.000000)" 0.1)
            (Variables|Default|SetAttackedActor _asabstract_character)))
        (if (!= (Variables|/Game/Characters/AbstractCharacter.AbstractCharacter_C|GetTeamNumber (Variables|Default|GetAttackedActor)) (Variables|Default|GetHolderTeam))
          (if (== 0 (Variables|Default|GetCurrentTag))
            (Development|PrintString "Yes Damage tag" true true "(R=1.000000,G=0.000000,B=0.000000,A=1.000000)" 0.1)
            (Variables|Default|SetCurrentTag 1)
            (Utilities|IsValid _holder
              (:Is%20Valid
                (CallFunction|GetDamage)
                (Audio|PlaySoundatLocation (CallFunction|ChooseSound) (Transformation|GetActorLocation (Variables|Default|GetAttackedActor)) "0, 0, 0" 0.6 1.0 0.0 0 "/Game/Items/Sword/SwordHitConcurrency.SwordHitConcurrency" 0)
                (Game|Damage|ApplyDamage (Variables|Default|GetAttackedActor) (Variables|Default|GetDamage) (Pawn|GetController _holder) 0 "/Game/GameData/Damages/DamageType_Physical.DamageType_Physical_C")
                (CallFunction|HitSomething)
                (Audio|PlaySoundatLocation "/Game/Sound/Archer/ArrowHit_Cue.ArrowHit_Cue" (Transformation|GetActorLocation (Variables|Default|GetAttackedActor)) "0, 0, 0" 1.0 1.0 0.0 0 0 0))
              (:Is%20Not%20Valid
                (Development|PrintString "Not Valid holder" true true "(R=1.000000,G=0.000000,B=0.000000,A=1.000000)" 0.1)))
            (else
              (Development|PrintString "Not Damage tag" true true "(R=1.000000,G=0.000000,B=0.000000,A=1.000000)" 0.1)))
          (else
            (Development|PrintString "No Damge same team" true true "(R=1.000000,G=0.000000,B=0.000000,A=1.000000)" 0.1)))))))

(event Custom|HitSomething
  (Variables|Default|SetIsMoving false)
  (Physics|SetSimulatePhysics (Variables|Default|GetArrowMesh) true)
  (Utilities|FlowControl|Delay 1e+01)
  (Actor|DestroyActor))

(event EventBeginPlay
  (Variables|Default|SetCurrentTag 0))

(event Collision|EventActorBeginOverlap
  (params (OtherActor :type Actor%20Object%20Reference)))

(event EventTick
  (params (DeltaSeconds :type Float%20%28single-precision%29)))

(fn ConstructionScript)

(fn GetDamage
  (bind _output_get (Variables|Default|SetDamage (Variables|/Game/Characters/AbstractCharacter.AbstractCharacter_C|GetDamage (Variables|Default|GetHolder))))
  (Development|PrintString (Utilities|String|Append (Utilities|String|MakeLiteralString "Damage : ") (Utilities|String|ToString(Float) _output_get)) true true "(R=1.000000,G=0.000000,B=0.000000,A=1.000000)" 1e+01))

(fn ChooseSound
  (switch int (Math|Random|RandomIntegerinRangefromStream 0 1 (LocalVariables|GetSeed))
    (:0
      (return "/Game/Items/Sword/SwordHit2.SwordHit2"))
    (:1
      (return "/Game/Items/Sword/SwordHit3.SwordHit3"))))