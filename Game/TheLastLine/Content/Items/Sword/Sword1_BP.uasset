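; Sword weapon actor that deals physical damage to enemy characters it overlaps.
; On overlap, it compares the other AbstractCharacter's TeamNumber with its Holder's, skipping teammates.
; Damage is copied from the Holder on each hit and applied with the Holder as causer and its controller as instigator.
; Holder is not assigned here, and debug prints report construction and a missing Holder.
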(event EventBeginPlay)

(event Collision|EventActorBeginOverlap
  (params (OtherActor :type Actor%20Object%20Reference))
  (bind _holder (Variables|Default|GetHolder))
  (Utilities|IsValid OtherActor
    (:Is%20Valid
      (bind _asabstract_character (Utilities|Casting|CastToAbstractCharacter OtherActor))
      (Variables|Default|SetAttackedActor _asabstract_character)
      (CallFunction|GetHolderTeam)
      (if (!= (Variables|/Game/Characters/AbstractCharacter.AbstractCharacter_C|GetTeamNumber _asabstract_character) (Variables|Default|GetHolderTeam))
        (Utilities|FlowControl|Sequence
          (:then_0
            (CallFunction|GetDamage))
          (:then_1
            (Utilities|IsValid _holder
              (:Is%20Valid
                (Game|Damage|ApplyDamage (Variables|Default|GetAttackedActor) (Variables|Default|GetDamage) (Pawn|GetController _holder) _holder "/Game/GameData/Damages/DamageType_Physical.DamageType_Physical_C"))
              (:Is%20Not%20Valid
                (Development|PrintString "No Holder")))))))))

(event EventTick
  (params (DeltaSeconds :type Float%20%28single-precision%29)))

(fn ConstructionScript
  (Development|PrintString "Created a sword" true true "(R=0.000000,G=0.660000,B=1.000000,A=1.000000)" 2e+01))

(fn GetDamage
  (bind _holder (Variables|Default|GetHolder))
  (Utilities|IsValid _holder
    (:Is%20Valid
      (Variables|Default|SetDamage (Variables|/Game/Characters/AbstractCharacter.AbstractCharacter_C|GetDamage _holder)))))

(fn GetHolderTeam
  (bind _holder (Variables|Default|GetHolder))
  (Utilities|IsValid _holder
    (:Is%20Valid
      (bind _output_get (Variables|Default|SetHolderTeam (Variables|/Game/Characters/AbstractCharacter.AbstractCharacter_C|GetTeamNumber _holder))))
    (:Is%20Not%20Valid
      (Development|PrintString "Holder not valid"))))