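; Ability spawner actor that places PickUpAbility_BP pickups at every AbilitySpawnLocation in the level on BeginPlay, then every three minutes on a looping timer.
; UpdateAbilities hides each location's marker cube, spawns pickups there and assigns their ability types, without removing earlier pickups.
; GenerateAbilitiesToSpawn picks consecutive Abilities entries from a random start index, capped by location and ability counts.
; Tick accumulates a Seed value that nothing shown reads.
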(event Custom|UpdateAbilities
  (for _array_element (Variables|Default|GetAbilitySpawnLocations)
    ;[1 1 1] Spawn a random ability at the spawn location
    (Rendering|Material|SetMaterial (Variables|/Game/GameData/System/AbilitySpawner/AbilitySpawnLocation.AbilitySpawnLocation_C|GetCube _array_element) 0 "/Game/GameData/GlobalMaterials/M_InvisibleMaterial.M_InvisibleMaterial"))
  (bind _output_get (Variables|Default|SetNumSpawnLocations (Utilities|Array|Length (Variables|Default|GetAbilitySpawnLocations))))
  (bind _abilities_chosen (CallFunction|GenerateAbilitiestoSpawn _output_get))
  (for (_array_element_2 _array_index) _abilities_chosen
    (bind _returnvalue (Game|SpawnActorfromClass "/Game/Abilities/Pickup/PickUpAbility_BP.PickUpAbility_BP_C" (Math|Transform|MakeTransform (Transformation|GetActorLocation (Utilities|Array|Get(acopy) (Variables|Default|GetAbilitySpawnLocations) _array_index)) "0, 0, 0" "1,1,1") "AlwaysSpawn" 0 0))
    ;;[1 1 1] do not delete
    (Variables|/Game/Abilities/Pickup/PickUpAbility_BP.PickUpAbility_BP_C|SetAbilityType _returnvalue _array_element_2)
    (Default|ClasstoName _returnvalue _array_element_2)))

(event EventBeginPlay
  (bind _outactors (Actor|GetAllActorsOfClass "/Game/GameData/System/AbilitySpawner/AbilitySpawnLocation.AbilitySpawnLocation_C"))
  (Variables|Default|SetAbilitySpawnLocations _outactors)
  (CallFunction|UpdateAbilities)
  (Utilities|Time|SetTimerbyEvent (delegate Custom|UpdateAbilities) 1.8e+02 true))

(event Collision|EventActorBeginOverlap
  (params (OtherActor :type Actor%20Object%20Reference)))

(event EventTick
  (params (DeltaSeconds :type Float%20%28single-precision%29))
  (Variables|Default|SetSeed (+ (Variables|Default|GetSeed) DeltaSeconds)))

(fn ConstructionScript)

(fn GenerateAbilitiestoSpawn
  (params (NumberOfSpawnPoints :type Integer))
  (LocalVariables|SetNumOfSpawnPoints NumberOfSpawnPoints)
  (LocalVariables|SetNumberOfAbilities (Utilities|Array|Length (Variables|Default|GetAbilities)))
  (Class|KismetMathLibrary|SeedRandomStream (Math|Random|MakeRandomStream (.days (Media|MediaPlayer|GetDuration))))
  (LocalVariables|SetSelectedIndex (Math|Integer|%(Integer) (Math|Random|RandomInteger 1000000) (LocalVariables|GetNumberOfAbilities)))
  (while (and (< (LocalVariables|GetCounter) (LocalVariables|GetNumOfSpawnPoints)) (< (LocalVariables|GetCounter) (LocalVariables|GetNumberOfAbilities)))
    (Utilities|Array|SetArrayElem (LocalVariables|GetSelectedAbilties) (LocalVariables|GetCounter) (Utilities|Array|Get(acopy) (Variables|Default|GetAbilities) (LocalVariables|GetSelectedIndex)) true)
    (if (>= (LocalVariables|GetSelectedIndex) (LocalVariables|GetNumberOfAbilities))
      (LocalVariables|SetSelectedIndex 0)
      (else
        (Math|Integer|IncrementInt (LocalVariables|GetSelectedIndex)
          (:%20%20
            (Math|Integer|IncrementInt (LocalVariables|GetCounter)))))))
  (return (LocalVariables|GetSelectedAbilties)))

(fn UpdateSpawnLocation
  (bind _outactors (Actor|GetAllActorsOfClass "/Game/GameData/System/AbilitySpawner/AbilitySpawnLocation.AbilitySpawnLocation_C"))
  (Variables|Default|SetAbilitySpawnLocations _outactors)
  (CallFunction|UpdateAbilities))

(fn SpawnAbility)