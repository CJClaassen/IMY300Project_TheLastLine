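; Wave spawner actor that builds enemy AI waves from a health budget and spawns them at AISpawnLocation points cached on BeginPlay.
; Unit counts per type are rolled by probability until the budget drops below the cheapest unit, with bosses capped by difficulty-scaled wave number.
; SpawnWaveV2 rolls and spawns in one call; SimulateNumberOfUnits and SpawnNumberOfUnits split those steps.
; The older SpawnWave's spawn loop is disconnected.
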(event Custom|Wait
  (params (Seconds :type Float%20%28single-precision%29))
  (Utilities|FlowControl|Delay Seconds))

(event EventBeginPlay
  (bind _outactors (Actor|GetAllActorsOfClass "/Game/GameData/System/WaveSpawner/AISpawnLocation.AISpawnLocation_C"))
  (for _array_element _outactors
    (Utilities|Array|Add (Variables|Default|GetspawnLocations) (Transformation|GetActorLocation _array_element)))
  (Development|PrintString (Utilities|String|Append "Number of spawn locations: " (Utilities|String|ToString(Integer) (Utilities|Array|Length (Variables|Default|GetspawnLocations)))) true true "(R=1.000000,G=0.011645,B=0.000000,A=1.000000)" 1e+01))

(event Collision|EventActorBeginOverlap
  (params (OtherActor :type Actor%20Object%20Reference)))

(event EventTick
  (params (DeltaSeconds :type Float%20%28single-precision%29)))

(fn ConstructionScript)

(fn SpawnWave
  (params (typeOfUnits :type Array%20of%20Abstract%20Character%20Class%20References) (ProbabilityOfUnits :type Array%20of%20Floats%20%28single-precision%29) (MaximumHealth :type Float%20%28single-precision%29) (CurrentWave :type Integer) (UnitBehaviourtree :type Array%20of%20Behavior%20Tree%20Object%20References) (UnitLevel :type Array%20of%20Integers))
  (LocalVariables|Set_TypeOfUnits typeOfUnits)
  (LocalVariables|Set_ProbabilityOfUnits ProbabilityOfUnits)
  (LocalVariables|Set_CurrentWave CurrentWave)
  (LocalVariables|SetRemainingHealth MaximumHealth)
  (LocalVariables|SetBehaviourTrees UnitBehaviourtree))

(fn SpawnWaveV2
  (params (UnitLevel :type Array%20of%20Integers) (UnitHealth :type Array%20of%20Floats%20%28single-precision%29) (isBossUnit :type Array%20of%20Booleans) (ProbabilityOfUnits :type Array%20of%20Floats%20%28single-precision%29) (typeOfUnits :type Array%20of%20Abstract%20Character%20Class%20References) (UnitBehaviourtree :type Array%20of%20Behavior%20Tree%20Object%20References) (CurrentWave :type Integer%20%28by%20ref%29) (Difficulty :type Integer%20%28by%20ref%29) (MaximumHealth :type Float%20%28single-precision%29%20%28by%20ref%29))
  (bind _spawnlocations (Variables|Default|GetspawnLocations))
  ;[1 1 1] Initialize variables
  (LocalVariables|Set_UnitLevel UnitLevel)
  (LocalVariables|Set_UnitHealth UnitHealth)
  (LocalVariables|Set_IsBossUnit isBossUnit)
  (LocalVariables|Set_ProbabilityOfUnits ProbabilityOfUnits)
  (LocalVariables|Set_TypeOfUnits typeOfUnits)
  (LocalVariables|SetBehaviourTrees UnitBehaviourtree)
  (LocalVariables|Set_CurrentWave (* CurrentWave Difficulty))
  (LocalVariables|SetRemainingHealth MaximumHealth)
  (LocalVariables|SetMAX%20NUMBER%20OF%20BOSSES (/ (LocalVariables|Get_CurrentWave) 10))
  (LocalVariables|SetLowestHealth (.MinValue (Math|Float|MinOfFloatArray (LocalVariables|Get_UnitHealth))))
  ;[1 1 1] Initialize number of units created per type, with the number of unit types
  (for _array_element (LocalVariables|Get_TypeOfUnits)
    (Utilities|Array|Add (LocalVariables|GetNumberOfTypeUnits) 0))
  ;[1 1 1] Simulate the number and type of units
  (while (>= (LocalVariables|GetRemainingHealth) (LocalVariables|GetLowestHealth))
    (Utilities|FlowControl|Sequence
      (:then_0
        (LocalVariables|SetCurrentNumberOfBosses (CallFunction|CountNumberOfBosses (LocalVariables|GetNumberOfTypeUnits) (LocalVariables|Get_IsBossUnit))))
      (:then_1
        (bind _array_index (Utilities|Array|ForEachLoopwithBreak (LocalVariables|Get_ProbabilityOfUnits))
          (:LoopBody
            ;;[1 1 1] Check if there is enough health left
            (if (not (< (LocalVariables|GetRemainingHealth) (Utilities|Array|Get(acopy) (LocalVariables|Get_UnitHealth) _array_index)))
              (if (not (and (Utilities|Array|Get(acopy) (LocalVariables|Get_IsBossUnit) _array_index) (== (LocalVariables|GetCurrentNumberOfBosses) (LocalVariables|GetMAX%20NUMBER%20OF%20BOSSES))))
                (if (<= (Math|Random|RandomFloatinRange 0.0 1e+02) (Utilities|Array|Get(acopy) (LocalVariables|Get_ProbabilityOfUnits) _array_index))
                  (Math|Integer|IncrementInt (Utilities|Array|Get(acopy) (LocalVariables|GetNumberOfTypeUnits) _array_index)
                    (:%20%20
                      (LocalVariables|SetRemainingHealth (- (LocalVariables|GetRemainingHealth) (Utilities|Array|Get(acopy) (LocalVariables|Get_UnitHealth) _array_index)))))))))))))
  ;[1 1 1] Spawning the enemy wave
  (for (_array_element_2 _array_index_2) (LocalVariables|GetNumberOfTypeUnits)
    (Development|PrintText (Utilities|Text|FormatText "{Skeleton type}: {units} units" _array_index_2 _array_element_2) true true "(R=0.992148,G=0.177083,B=1.000000,A=1.000000)" 1e+01)
    (for _index (range 1 _array_element_2)
      (bind _returnvalue (AI|SpawnAIFromClass (Utilities|Array|Get(acopy) (LocalVariables|Get_TypeOfUnits) _array_index_2) (Utilities|Array|Get(acopy) (LocalVariables|GetBehaviourTrees) _array_index_2) (Utilities|Array|Get(acopy) _spawnlocations (Math|Random|RandomIntegerinRange 0 (- (Utilities|Array|Length _spawnlocations) 1))) "0, 0, 0" false))
      (Utilities|IsValid _returnvalue
        (:Is%20Valid
          (Math|Integer|IncrementInt (LocalVariables|GetNumber%20of%20Units)))
        (:Is%20Not%20Valid
          (Development|PrintString "Failed to spawn in wave")))))
  (return (LocalVariables|GetNumber%20of%20Units)))

(fn CountNumberOfBosses
  (params (Number%20of%20Units%20per%20type :type Array%20of%20Integers) (IsBossUnit :type Array%20of%20Booleans))
  (for (_array_element _array_index) Number%20of%20Units%20per%20type
    (if (Utilities|Array|Get(acopy) IsBossUnit _array_index)
      (LocalVariables|SetnumberOfBosses (+ _array_element (LocalVariables|GetnumberOfBosses)))))
  (return (LocalVariables|GetnumberOfBosses)))

(fn SimulateNumberOfUnits
  (params (UnitLevel :type Array%20of%20Integers) (UnitHealth :type Array%20of%20Floats%20%28single-precision%29) (isBossUnit :type Array%20of%20Booleans) (ProbabilityOfUnits :type Array%20of%20Floats%20%28single-precision%29) (typeOfUnits :type Array%20of%20Abstract%20Character%20Class%20References) (UnitBehaviourtree :type Array%20of%20Behavior%20Tree%20Object%20References) (CurrentWave :type Integer%20%28by%20ref%29) (Difficulty :type Integer%20%28by%20ref%29) (MaximumHealth :type Float%20%28single-precision%29%20%28by%20ref%29))
  ;[1 1 1] Initialize variables
  (LocalVariables|Set_UnitLevel UnitLevel)
  (LocalVariables|Set_UnitHealth UnitHealth)
  (LocalVariables|Set_IsBossUnit isBossUnit)
  (LocalVariables|Set_ProbabilityOfUnits ProbabilityOfUnits)
  (LocalVariables|Set_TypeOfUnits typeOfUnits)
  (LocalVariables|SetBehaviourTrees UnitBehaviourtree)
  (LocalVariables|Set_CurrentWave (* CurrentWave Difficulty))
  (LocalVariables|SetRemainingHealth MaximumHealth)
  (LocalVariables|SetMAX%20NUMBER%20OF%20BOSSES (/ (LocalVariables|Get_CurrentWave) 10))
  (LocalVariables|SetLowestHealth (.MinValue (Math|Float|MinOfFloatArray (LocalVariables|Get_UnitHealth))))
  ;[1 1 1] Initialize number of units created per type, with the number of unit types
  (for _array_element (LocalVariables|Get_TypeOfUnits)
    (Utilities|Array|Add (LocalVariables|GetNumberOfTypeUnits) 0))
  ;[1 1 1] Simulate the number and type of units
  (while (>= (LocalVariables|GetRemainingHealth) (LocalVariables|GetLowestHealth))
    (Utilities|FlowControl|Sequence
      (:then_0
        (LocalVariables|SetCurrentNumberOfBosses (CallFunction|CountNumberOfBosses (LocalVariables|GetNumberOfTypeUnits) (LocalVariables|Get_IsBossUnit))))
      (:then_1
        (bind _array_index (Utilities|Array|ForEachLoopwithBreak (LocalVariables|Get_ProbabilityOfUnits))
          (:LoopBody
            ;;[1 1 1] Check if there is enough health left
            (if (not (< (LocalVariables|GetRemainingHealth) (Utilities|Array|Get(acopy) (LocalVariables|Get_UnitHealth) _array_index)))
              (if (not (and (Utilities|Array|Get(acopy) (LocalVariables|Get_IsBossUnit) _array_index) (== (LocalVariables|GetCurrentNumberOfBosses) (LocalVariables|GetMAX%20NUMBER%20OF%20BOSSES))))
                (if (<= (Math|Random|RandomFloatinRange 0.0 1e+02) (Utilities|Array|Get(acopy) (LocalVariables|Get_ProbabilityOfUnits) _array_index))
                  (Math|Integer|IncrementInt (Utilities|Array|Get(acopy) (LocalVariables|GetNumberOfTypeUnits) _array_index)
                    (:%20%20
                      (LocalVariables|SetRemainingHealth (- (LocalVariables|GetRemainingHealth) (Utilities|Array|Get(acopy) (LocalVariables|Get_UnitHealth) _array_index)))))))))))))
  (return (LocalVariables|GetNumberOfTypeUnits)))

(fn SpawnNumberOfUnits
  (params (NumberOfUnits :type Spawngroup%20Structure%20%28by%20ref%29) (typeOfUnits :type Array%20of%20Abstract%20Character%20Class%20References) (UnitBehaviourtree :type Array%20of%20Behavior%20Tree%20Object%20References))
  (bind _spawnlocations (Variables|Default|GetspawnLocations))
  (bind _returnvalue (Utilities|Array|Length _spawnlocations))
  (bind _returnvalue_2 (- _returnvalue 1))
  (bind _returnvalue_3 (Math|Random|RandomIntegerinRange 0 _returnvalue_2))
  (bind _output (Utilities|Array|Get(acopy) _spawnlocations _returnvalue_3))
  ;[1 1 1] Initialize variables
  (LocalVariables|SetNumberOfTypeUnits NumberOfUnits)
  (LocalVariables|Set_TypeOfUnits typeOfUnits)
  (LocalVariables|SetBehaviourTrees UnitBehaviourtree)
  ;[1 1 1] Spawning the enemy wave
  (for (_array_element _array_index) (.unitsspawn (LocalVariables|GetNumberOfTypeUnits))
    (bind _output_get (LocalVariables|SetNumTypeUnitsToCreate _array_element))
    (Development|PrintText (Utilities|Text|FormatText "Spawn {unit} units" _output_get) true true "(R=0.000000,G=0.660000,B=1.000000,A=1.000000)" 1e+01)
    (for _index (range 1 _output_get)
      (bind _returnvalue_4 (AI|SpawnAIFromClass (Utilities|Array|Get(acopy) (LocalVariables|Get_TypeOfUnits) _array_index) (Utilities|Array|Get(acopy) (LocalVariables|GetBehaviourTrees) _array_index) (Math|Vector|MakeVector (+ (.x _output) (Math|Random|RandomFloatinRange -3e+02 3e+02)) (+ (.y _output) (Math|Random|RandomFloatinRange -3e+02 3e+02)) (.z _output)) "0, 0, 0" false))
      (Utilities|IsValid _returnvalue_4
        (:Is%20Valid
          (Math|Integer|IncrementInt (LocalVariables|GetNumber%20of%20Units)
            (:%20%20
              (Math|Integer|DecrementInt (Utilities|Array|Get(acopy) (.unitsspawn (LocalVariables|GetNumberOfTypeUnits)) _array_index)))))
        (:Is%20Not%20Valid
          (LocalVariables|SetNumberOfTypeUnits (Utilities|Struct|MakeSpawngroup (.unitsspawn (LocalVariables|GetNumberOfTypeUnits)) true))))))
  (return (LocalVariables|GetNumberOfTypeUnits) (LocalVariables|GetNumber%20of%20Units)))