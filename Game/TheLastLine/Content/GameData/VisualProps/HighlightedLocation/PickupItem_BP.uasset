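; Interactable sword-and-shield pickup that advances an objective, built on a parent prop with a heading-only widget.
; LinkHandler stores the objective handler, spawns the item actors and places the pickup.
; Knights overlapping the radius-scaled sphere get a prompt and register it as their controller's PropInRange.
; Activate gives items to tutorial knights, then for any knight updates the objective and destroys itself if the handler is valid.
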(event OnComponentBeginOverlap(ActivationRadius)
  (params (OverlappedComponent :type Primitive%20Component%20Object%20Reference) (OtherActor :type Actor%20Object%20Reference) (OtherComp :type Primitive%20Component%20Object%20Reference) (OtherBodyIndex :type Integer) (bFromSweep :type Boolean) (SweepResult :type Hit%20Result%20Structure%20%28by%20ref%29))
  (bind _asknight_bp (Utilities|Casting|CastToKnight_BP OtherActor))
  (bind _ascustom_player_controller_bp (Utilities|Casting|CastToCustomPlayerController_BP (Pawn|GetController _asknight_bp)))
  (Default|NotifyOfInteraction _ascustom_player_controller_bp "Pickup" "Sword & Shield")
  (Variables|/Game/Controllers/PlayerControllers/CustomPlayerController_BP.CustomPlayerController_BP_C|SetPropInRange _ascustom_player_controller_bp self)
  (CallFunction|DisplayWidget _asknight_bp)
  (Development|PrintString "Hello"))

(event OnComponentEndOverlap(ActivationRadius)
  (params (OverlappedComponent :type Primitive%20Component%20Object%20Reference) (OtherActor :type Actor%20Object%20Reference) (OtherComp :type Primitive%20Component%20Object%20Reference) (OtherBodyIndex :type Integer))
  (bind _asknight_bp (Utilities|Casting|CastToKnight_BP OtherActor))
  (bind _ascustom_player_controller_bp (Utilities|Casting|CastToCustomPlayerController_BP (Pawn|GetController _asknight_bp)))
  (Default|RemoveInteractionNotification _ascustom_player_controller_bp)
  (Variables|/Game/Controllers/PlayerControllers/CustomPlayerController_BP.CustomPlayerController_BP_C|SetPropInRange _ascustom_player_controller_bp 0)
  (CallFunction|HideWidget))

(event EventBeginPlay
  (Variables|Default|SetCooldownTime 0.0)
  (CallFunction|RecalculateSphere (Variables|Default|GetRadius))
  (Variables|Default|SetDisplayHeadingOnly true)
  (|CallParentFunction))

(event EventActivate
  (params (PlayerIndex :type Integer))
  (bind _returnvalue (Game|Player|GetPlayerPawn PlayerIndex))
  (bind _handler (Variables|Default|GetHandler))
  (bind _astutorial_knight_bp (Utilities|Casting|CastToTutorialKnight_BP _returnvalue)
    (:then
      (Default|PickUpItems _astutorial_knight_bp (Variables|Default|GetItem) true))
    (:CastFailed
      (Utilities|Casting|CastToKnight_BP _returnvalue)))
  (Utilities|IsValid _handler
    (:Is%20Valid
      (Default|UpdateObjective _handler (Variables|Default|GetObjectiveName) (Variables|Default|GetSection))
      (Actor|DestroyActor))))

(fn ConstructionScript
  (|CallParentFunction))

(fn LinkHandler
  (params (handler :type Map%20Handler%20BP%20Object%20Reference) (ObjectiveID :type Name) (Section :type String) (Addon :type Array%20of%20Item%20BP%20Class%20References) (Location :type Array%20of%20Transforms) (PickupLocation :type Vector) (PickupScale :type Vector :default "1.000000,1.000000,1.000000"))
  (Variables|Default|SetHandler handler)
  (Variables|Default|SetObjectiveName ObjectiveID)
  (Variables|Default|SetSection Section)
  (for (_array_element _array_index) Addon
    (bind _returnvalue (Game|SpawnActorfromClass _array_element (Utilities|Array|Get(acopy) Location _array_index) "AdjustIfPossibleButAlwaysSpawn" 0 0))
    (Utilities|Array|SetArrayElem (Variables|Default|GetItem) _array_index _returnvalue true))
  (Transformation|SetActorLocation PickupLocation false false)
  (Transformation|SetActorScale3D PickupScale))

(fn CanActivateOfDistance
  (return true))

(fn RecalculateSphere
  (params (New%20Radius :type Float%20%28single-precision%29))
  (bind _activationradius (Variables|Default|GetActivationRadius))
  (bind _returnvalue (Transformation|GetWorldScale _activationradius))
  (Variables|Default|SetRadius New%20Radius)
  (Transformation|SetWorldScale3D _activationradius (Math|Vector|MakeVector (* (.x _returnvalue) (/ (Variables|Default|GetRadius) (Variables|/Script/Engine.SphereComponent|GetSphereRadius (Variables|Default|GetSphere)))) (* (.y _returnvalue) (/ (Variables|Default|GetRadius) (Variables|/Script/Engine.SphereComponent|GetSphereRadius (Variables|Default|GetSphere)))) (* (.z _returnvalue) (/ (Variables|Default|GetRadius) (Variables|/Script/Engine.SphereComponent|GetSphereRadius (Variables|Default|GetSphere)))))))