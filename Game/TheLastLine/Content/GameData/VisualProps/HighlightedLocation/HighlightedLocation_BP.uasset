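; HighlightedLocation_BP is a location marker that reports to an objective handler when the TutorialKnight_BP reaches it.
; It starts with an invisible material, and LinkToHandler stores the handler, objective name and section, then switches MoveLocation to the move indicator material.
; Overlap by the knight calls UpdateObjective with the objective name and an empty section rather than the stored one, regardless of whether the marker is shown.
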(event OnComponentBeginOverlap(MoveLocation)
  (params (OverlappedComponent :type Primitive%20Component%20Object%20Reference) (OtherActor :type Actor%20Object%20Reference) (OtherComp :type Primitive%20Component%20Object%20Reference) (OtherBodyIndex :type Integer) (bFromSweep :type Boolean) (SweepResult :type Hit%20Result%20Structure%20%28by%20ref%29))
  (Utilities|Casting|CastToTutorialKnight_BP OtherActor)
  (Development|PrintString "update")
  (Default|UpdateObjective (Variables|Default|GetHandler) (Variables|Default|GetObjectiveName)))

(event EventBeginPlay
  (Rendering|Material|SetMaterial (Variables|Default|GetMoveLocation) 0 "/Game/GameData/GlobalMaterials/M_InvisibleMaterial.M_InvisibleMaterial"))

(event Collision|EventActorBeginOverlap
  (params (OtherActor :type Actor%20Object%20Reference)))

(event EventTick
  (params (DeltaSeconds :type Float%20%28single-precision%29)))

(fn ConstructionScript)

(fn LinktoHandler
  (params (Handler :type Map%20Handler%20BP%20Object%20Reference) (ObjectiveName :type Name) (Section :type String))
  (Variables|Default|SetHandler Handler)
  (Variables|Default|SetObjectiveName ObjectiveName)
  (Variables|Default|SetSection Section)
  (Rendering|Material|SetMaterial (Variables|Default|GetMoveLocation) 0 "/Game/GameData/VisualProps/RadiusIndicator/MInstance_MoveIndicator.MInstance_MoveIndicator"))