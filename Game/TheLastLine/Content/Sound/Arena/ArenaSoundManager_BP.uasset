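; Arena sound manager Blueprint that plays a background sound on BeginPlay and adds crowd reaction sounds for enemy and player deaths.
; UpdateCrowd switches on the action and spawns an audio component under a separate concurrency setting, louder for enemy deaths than player deaths.
; Each reaction has two branches chosen from a random stream seeded by whole game seconds, but a Max of 1 always selects the first.
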(event EventBeginPlay
  (bind _returnvalue (AddComponent|AddAudioComponent false))
  (bind _output_get (Variables|Default|SetBackgroundSound _returnvalue))
  (Variables|/Script/Engine.AudioComponent|SetConcurrencySettings _output_get "/Game/Sound/Arena/Idle/BackgroundConcurrency.BackgroundConcurrency")
  (Audio|Components|Audio|SetVolumeMultiplier _output_get 2.0 :!class /Script/Engine.AudioComponent)
  (Audio|Components|Audio|Play _output_get 0.0))

(event Collision|EventActorBeginOverlap
  (params (OtherActor :type Actor%20Object%20Reference)))

(event EventTick
  (params (DeltaSeconds :type Float%20%28single-precision%29)))

(fn ConstructionScript)

(fn UpdateCrowd
  (params (Action :type String))
  (LocalVariables|SetStream (Math|Random|MakeRandomStream (Math|Float|Truncate (Utilities|Time|GetGameTimeinSeconds))))
  (switch string Action
    (:Enemy_Death
      (switch int (Class|KismetMathLibrary|RandomIntegerfromStream 1 (LocalVariables|GetStream))
        (:0
          (bind _returnvalue (AddComponent|AddAudioComponent false))
          (bind _output_get (Variables|Default|SetAdditionalSound _returnvalue))
          (Variables|/Script/Engine.AudioComponent|SetConcurrencySettings _output_get "/Game/Sound/Arena/AdditionalBackgroundConcurrency.AdditionalBackgroundConcurrency"))
        (:1
          (bind _returnvalue_2 (AddComponent|AddAudioComponent false))
          (bind _output_get_2 (Variables|Default|SetAdditionalSound _returnvalue_2))
          (Variables|/Script/Engine.AudioComponent|SetConcurrencySettings _output_get_2 "/Game/Sound/Arena/AdditionalBackgroundConcurrency.AdditionalBackgroundConcurrency")))
      (Audio|Components|Audio|SetVolumeMultiplier (Variables|Default|GetAdditionalSound) 2.0 :!class /Script/Engine.AudioComponent)
      (Audio|Components|Audio|Play (Variables|Default|GetAdditionalSound) 0.0))
    (:Player_Death
      ;[1 1 1] when player dies
      (switch int (Class|KismetMathLibrary|RandomIntegerfromStream 1 (LocalVariables|GetStream))
        (:0
          (bind _returnvalue_3 (AddComponent|AddAudioComponent false))
          (bind _output_get_3 (Variables|Default|SetAdditionalSound _returnvalue_3))
          (Variables|/Script/Engine.AudioComponent|SetConcurrencySettings _output_get_3 "/Game/Sound/Arena/AdditionalBackgroundConcurrency.AdditionalBackgroundConcurrency"))
        (:1
          (bind _returnvalue_4 (AddComponent|AddAudioComponent false))
          (bind _output_get_4 (Variables|Default|SetAdditionalSound _returnvalue_4))
          (Variables|/Script/Engine.AudioComponent|SetConcurrencySettings _output_get_4 "/Game/Sound/Arena/AdditionalBackgroundConcurrency.AdditionalBackgroundConcurrency")))
      (Audio|Components|Audio|SetVolumeMultiplier (Variables|Default|GetAdditionalSound) 0.6 :!class /Script/Engine.AudioComponent)
      (Audio|Components|Audio|Play (Variables|Default|GetAdditionalSound) 0.0))))