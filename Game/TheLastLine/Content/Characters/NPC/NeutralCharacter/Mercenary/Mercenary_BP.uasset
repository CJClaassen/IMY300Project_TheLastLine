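; Neutral Mercenary NPC, a melee character that sets its stats in construction and spawns a socketed sword and shield on BeginPlay.
; MeleeAttack turns it via timeline, plays a random attack montage and arms the weapon.
; Damage triggers hit reactions unless mid-attack, while a camera-facing dynamic-material health bar animates lost health and tracks timed regen.
; PlayDead detaches the controller, then destroys character and gear after a delay.
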(event Custom|CreateWeapon
  (bind _returnvalue (Transformation|GetActorTransform))
  (bind _self self)
  (Utilities|FlowControl|Sequence
    (:then_0
      (bind _returnvalue_2 (Game|SpawnActorfromClass "/Game/Items/Sword/Sword1_BP.Sword1_BP_C" _returnvalue "Undefined" 0 _self))
      (Variables|Default|SetWeapon _returnvalue_2)
      (Variables|/Game/Items/ItemBP.ItemBP_C|SetHolder _returnvalue_2 self)
      (Variables|/Game/Items/ItemBP.ItemBP_C|SetHolderTeam _returnvalue_2 (Variables|Default|GetTeamNumber))
      (Transformation|AttachComponentToComponent (Variables|/Script/Engine.Actor|GetRootComponent _returnvalue_2) (Variables|Character|GetMesh) "SwordSocket" "SnapToTarget" "SnapToTarget" "SnapToTarget" false))
    (:then_1
      (bind _returnvalue_3 (Game|SpawnActorfromClass "/Game/Items/Shield/RoundShield2_BP.RoundShield2_BP_C" _returnvalue "Undefined" 0 _self))
      (Variables|Default|SetShield _returnvalue_3)
      (Transformation|AttachComponentToComponent (Variables|/Script/Engine.Actor|GetRootComponent _returnvalue_3) (Variables|Character|GetMesh) "ShieldSocket" "SnapToTarget" "SnapToTarget" "SnapToTarget" false))))

(event Custom|Attack
  (switch int (Math|Random|RandomIntegerinRange 0 1)
    (:Default
      (Animation|PlayAnimMontage "/Game/Characters/NPC/NeutralCharacter/Mercenary/Assets/Mercenary_Attack2__Montage.Mercenary_Attack2__Montage" 1.5 "None" :!label _label))
    (:0
      (Animation|PlayAnimMontage "/Game/Characters/NPC/NeutralCharacter/Mercenary/Assets/Mercenary_Attack1_Montage.Mercenary_Attack1_Montage" 1.5 "None"))
    (:1
      (goto _label)))
  (Variables|/Game/Items/ItemBP.ItemBP_C|SetInAttack (Variables|Default|GetWeapon) true))

(event Custom|FaceTarget
  (params (TargetActor :type Actor%20Object%20Reference))
  (bind _self self)
  (Utilities|IsValid TargetActor
    (:Is%20Valid
      (bind _turntrack (Timeline|Timeline_0 PlayFromStart)
        (:Update
          (Utilities|IsValid TargetActor
            (:Is%20Valid
              (Transformation|SetActorRotation (Math|Rotator|Lerp(Rotator) (Transformation|GetActorRotation _self) (Math|Rotator|MakeRotator 0.0 0.0 (+ (.yaw (Math|Rotator|FindLookatRotation (Transformation|GetActorLocation _self) (Transformation|GetActorLocation TargetActor))) -45.0)) _turntrack true)))))))))

(event Custom|RunIn
  (Animation|PlayAnimMontage "/Game/Characters/NPC/NeutralCharacter/Mercenary/Assets/Mercenary_DrawSword_Montage.Mercenary_DrawSword_Montage" 1.0 "None"))

(event Custom|LookAtTarget
  (params (TargetActor :type Actor%20Object%20Reference))
  (bind _returnvalue (Transformation|GetActorLocation TargetActor))
  (bind _self self)
  (bind _returnvalue_2 (Transformation|GetActorLocation _self))
  (bind _returnvalue_3 (Math|Rotator|FindLookatRotation _returnvalue_2 _returnvalue))
  (Transformation|SetActorRotation (Math|Rotator|MakeRotator (.roll _returnvalue_3) (.pitch _returnvalue_3) (+ (.yaw _returnvalue_3) -45.0))))

(event Custom|HealthRegen
  (if (not (CallFunction|IsDead))
    (Variables|Default|SetHealth (Math|Float|Clamp(Float) (+ (Variables|Default|GetHealth) (/ (Variables|Default|GetHealthRegenValue) 1e+01)) 0.0 (Variables|Default|GetMaxHealth)))
    (CallFunction|UpdateHealth)))

(event Custom|UpdateHealth
  (Rendering|Material|SetScalarParameterValue (Variables|Default|GetHealthBar) "NewHealthPercentage" (* (/ (Variables|Default|GetHealth) (Variables|Default|GetMaxHealth)) 1e+02) :!class /Script/Engine.MaterialInstanceDynamic))

(event EventBeginPlay
  (|CallParentFunction)
  (CallFunction|CreateWeapon)
  (Utilities|Time|SetTimerbyEvent (delegate Custom|HealthRegen) 0.2 true))

(event Collision|EventActorBeginOverlap
  (params (OtherActor :type Actor%20Object%20Reference))
  (|CallParentFunction OtherActor) ; This node is disabled and will not be called.\nDrag off pins to build functionality.
)

(event EventTick
  (params (DeltaSeconds :type Float%20%28single-precision%29))
  (bind _returnvalue (Game|GetPlayerCameraManager 0))
  (bind _healthbarcontainer (Variables|Default|GetHealthBarContainer))
  (bind _returnvalue_2 (Transformation|GetWorldLocation _healthbarcontainer))
  (bind _returnvalue_3 (Camera|GetCameraLocation _returnvalue))
  (bind _returnvalue_4 (- _returnvalue_3 _returnvalue_2))
  (bind _returnvalue_5 (Math|Rotator|MakeRotfromZ _returnvalue_4))
  (|CallParentFunction DeltaSeconds)
  (Utilities|FlowControl|Sequence
    (:then_0
      (if (Variables|Default|GetNeedsAnimation)
        (CallFunction|AnimateDamageTaken (Variables|Default|GetHealthBar) DeltaSeconds)))
    (:then_1
      (Transformation|SetWorldRotation _healthbarcontainer (Math|Rotator|MakeRotator (.roll _returnvalue_5) (.pitch _returnvalue_5) (.yaw _returnvalue_5)) false false))))

(event EventMeleeAttack
  (params (TaregtActor :type Actor%20Object%20Reference))
  (CallFunction|FaceTarget TaregtActor)
  (CallFunction|Attack))

(event Game|Damage|EventAnyDamage
  (params (Damage :type Float%20%28single-precision%29) (DamageType :type Damage%20Type%20Object%20Reference) (InstigatedBy :type Controller%20Object%20Reference) (DamageCauser :type Actor%20Object%20Reference))
  (if (not (CallFunction|IsDead))
    (|CallParentFunction Damage DamageType InstigatedBy DamageCauser)
    (CallFunction|UpdateHealth)
    (Variables|Default|SetNeedsAnimation true)
    (if (== (Utilities|String|FindSubstring (Utilities|GetObjectName (Animation|Montage|GetCurrentActiveMontage (Components|SkeletalMesh|GetAnimInstance (Variables|Character|GetMesh)))) "Mercenary_Attack" true) -1)
      (switch int (Math|Random|RandomIntegerinRange 0 1)
        (:Default
          (Animation|PlayAnimMontage "/Game/Characters/NPC/NeutralCharacter/Mercenary/Assets/Mercenary_Hit1_Montage.Mercenary_Hit1_Montage" 1.0 "None" :!label _label))
        (:0
          (goto _label))
        (:1
          (Animation|PlayAnimMontage "/Game/Characters/NPC/NeutralCharacter/Mercenary/Assets/Mercenary_Hit2_Montage.Mercenary_Hit2_Montage" 1.0 "None"))))))

(event EventPlayDead
  (|CallParentFunction)
  (Class|Pawn|DetachfromControllerPendingDestroy)
  (Utilities|FlowControl|Delay 15.0)
  (Utilities|FlowControl|Sequence
    (:then_0
      (Actor|DestroyActor (Variables|Default|GetWeapon)))
    (:then_1
      (Actor|DestroyActor (Variables|Default|GetShield)))
    (:then_2
      (Actor|DestroyActor self))))

(event EventAnimateDamageTaken
  (params (Material :type Material%20Instance%20Dynamic%20Object%20Reference) (DeltaSeconds :type Float%20%28single-precision%29))
  (if (<= (Variables|Default|GetHealth) (Variables|Default|GetAnimateHealth))
    (Rendering|Material|SetVectorParameterValue Material "DamagedHealthColor" "(R=0.960784,G=0.349020,B=0.000000,A=1.000000)" :!class /Script/Engine.MaterialInstanceDynamic)
    (Rendering|Material|SetScalarParameterValue Material "isDamage" 1.0 :!class /Script/Engine.MaterialInstanceDynamic)
    (Variables|Default|SetAnimateHealth (- (Variables|Default|GetAnimateHealth) (* DeltaSeconds 3e+01)))
    (Rendering|Material|SetScalarParameterValue Material "OldHealthPercentage" (* (/ (Variables|Default|GetAnimateHealth) (Variables|Default|GetMaxHealth)) 1e+02) :!class /Script/Engine.MaterialInstanceDynamic)
    (else
      (Variables|Default|SetNeedsAnimation false))))

(fn ConstructionScript
  (|CallParentFunction)
  (Utilities|FlowControl|Sequence
    (:then_0
      (bind _output_get (Variables|Default|SetHealth 1.5e+02))
      (Variables|Default|SetMaxHealth _output_get))
    (:then_1
      (Variables|Default|SetDamage 12.0))
    (:then_2
      (Variables|Default|SetPhysicalResist 0.2))
    (:then_3
      (Variables|Default|SetMagicalResist 0.0))
    (:then_4
      (Variables|Default|SetMovementSpeed 3.5e+02))
    (:then_5
      (Variables|Default|SetXPGain 80))
    (:then_6
      (Variables|Default|SetisLarge false))
    (:then_7
      (Variables|Default|SetTeamNumber 0))
    (:then_8
      (bind _returnvalue (Rendering|Material|CreateDynamicMaterialInstance (Variables|Default|GetHealthBarContainer) 0 "/Game/Characters/NPC/HealthMaterials/M_Health.M_Health" "None" :!class /Script/Engine.PrimitiveComponent))
      (bind _output_get_2 (Variables|Default|SetHealthBar _returnvalue))
      (Rendering|Material|SetVectorParameterValue _output_get_2 "HealthColor" "(R=0.018538,G=0.916667,B=0.000000,A=1.000000)" :!class /Script/Engine.MaterialInstanceDynamic))))