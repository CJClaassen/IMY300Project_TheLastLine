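; Activatable mercenary recruitment building, set up like a trap with a cost, that spawns a mercenary behind a gate.
; Activate asks the game mode's MapHandler to spawn one with a go-to point, then timelines lift and lower the gate, restoring the mercenary's WorldDynamic collision before closing.
; Activations within 1.5 seconds of the last are delayed, and IsReady compares the MapHandler's mercenary count to MaxMercs.
; The construction script places spawn and go-to markers from offsets.
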(event EventBeginPlay
  (|CallParentFunction))

(event EventTick
  (params (DeltaSeconds :type Float%20%28single-precision%29))
  (|CallParentFunction DeltaSeconds))

(event EventActivate
  (params (PlayerIndex :type Integer))
  (bind _gate (Variables|Default|GetGate))
  (|CallParentFunction PlayerIndex)
  (if (>= (- (Utilities|Time|GetGameTimeinSeconds) (Variables|Default|GetActivationTime)) 1.5)
    _
    (else
      (Utilities|FlowControl|Delay 1.5)))
  (Variables|Default|SetActivationTime (Utilities|Time|GetGameTimeinSeconds))
  (bind _astop_down_game_mode (Utilities|Casting|CastToTopDownGameMode (Game|GetGameMode)))
  (bind _mercenary (Default|SpawnMercenary (Variables|/Game/GameData/GameModes/TopDownGameMode.TopDownGameMode_C|GetMapHandler _astop_down_game_mode) (Transformation|GetWorldLocation (Variables|Default|GetSpawnSphere)) (Transformation|GetWorldLocation (Variables|Default|GetGoToSphere))))
  (bind _liftgate (Timeline|Timeline_LiftGate PlayFromStart)
    (:Update
      (Transformation|SetRelativeLocation _gate (Math|Vector|MakeVector 0.0 0.0 (* _liftgate 2e+02)) false false))
    (:Finished
      (Utilities|IsValid _mercenary
        (:Is%20Valid
          (Utilities|FlowControl|Delay 1.0)
          (Collision|SetCollisionResponsetoChannel (Variables|/Script/Engine.Character|GetCapsuleComponent _mercenary) "ECC_WorldDynamic" "ECR_Block")
          (bind _lowergate (Timeline|Timeline_Lower PlayFromStart)
            (:Update
              (Transformation|SetRelativeLocation _gate (Math|Vector|MakeVector 0.0 0.0 (* _lowergate 2e+02)) false false))))
        (:Is%20Not%20Valid
          (Timeline|Timeline_Lower PlayFromStart))))))

(fn ConstructionScript
  (bind _sphereradius (Variables|Default|GetSphereRadius))
  (bind _returnvalue (/ _sphereradius 1e+02))
  (|CallParentFunction)
  (Rendering|SetVisibility (Variables|Default|GetDamageRadius) false false)
  (Transformation|SetWorldScale3D (Variables|Default|GetActivationRadius) (Math|Vector|MakeVector _returnvalue _returnvalue (Math|Float|Clamp(Float) (/ _returnvalue 2.5) 1.0 5e+02)))
  (Variables|Default|SetTrapName "Recruit Mercemary")
  (Variables|Default|SetActivationCost 500)
  (Transformation|SetWorldLocation (Variables|Default|GetSpawnSphere) (+ (Transformation|GetActorLocation self) (Variables|Default|GetSpawnLocation)) false false)
  (Transformation|SetWorldLocation (Variables|Default|GetGoToSphere) (+ (Transformation|GetActorLocation) (Variables|Default|GetGoToLocation)) false false))

(fn IsReady
  (return (> (Variables|Default|GetMaxMercs) (CallFunction|GetNumMercs))))

(fn GetNumMercs
  (bind _astop_down_game_mode (Utilities|Casting|CastToTopDownGameMode (Game|GetGameMode)))
  (Utilities|IsValid (Variables|/Game/GameData/GameModes/TopDownGameMode.TopDownGameMode_C|GetMapHandler _astop_down_game_mode)
    (:Is%20Valid
      (return (Variables|/Game/Maps/MapHandler_BP.MapHandler_BP_C|GetNumMercenaries (Variables|/Game/GameData/GameModes/TopDownGameMode.TopDownGameMode_C|GetMapHandler _astop_down_game_mode))))
    (:Is%20Not%20Valid
      (return 0))))