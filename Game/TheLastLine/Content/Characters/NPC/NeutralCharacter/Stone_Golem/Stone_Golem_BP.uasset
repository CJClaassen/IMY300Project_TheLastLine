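; Stone golem neutral NPC that sleeps until activated, then runs for a limited lifetime before going dormant again.
; Sleeping spawns a linked activator beneath it and runs the idle behavior tree; waking destroys the activator, plays a montage, switches to the active tree and starts the deactivation timer.
; Its stomp grows an indicator via timeline, then briefly expands a zero-radius sphere to collect living characters through overlaps and deal physical damage.
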(event OnComponentBeginOverlap(StompArea)
  (params (OverlappedComponent :type Primitive%20Component%20Object%20Reference) (OtherActor :type Actor%20Object%20Reference) (OtherComp :type Primitive%20Component%20Object%20Reference) (OtherBodyIndex :type Integer) (bFromSweep :type Boolean) (SweepResult :type Hit%20Result%20Structure%20%28by%20ref%29))
  (bind _asabstract_character (Utilities|Casting|CastToAbstractCharacter OtherActor))
  (if (not (Default|IsDead _asabstract_character))
    (Utilities|Array|Add (Variables|Default|GetTargetsToDamage) _asabstract_character)))

(event Custom|GoToSleep
  (bind _returnvalue (Transformation|GetActorLocation))
  (bind _self self)
  (bind _returnvalue_2 (AI|GetAIController _self))
  ;[1 1 1] Deactivates Golemn
  (Variables|Default|SetisActivated false)
  (bind _returnvalue_3 (Game|SpawnActorfromClass "/Game/Traps/GolemnActivator/GolemnActivator_BP.GolemnActivator_BP_C" (Math|Transform|MakeTransform (Math|Vector|MakeVector (.x _returnvalue) (.y _returnvalue) (- (.z _returnvalue) 1e+02)) "0, 0, 0" "3.000000,3.000000,2.000000") "Undefined" 0 0))
  (bind _output_get (Variables|Default|SetGolemnActivator _returnvalue_3))
  (Default|LinktoGolemn _output_get 0 (Utilities|Array|Get(acopy) (Utilities|Array|MakeArray self)))
  (Variables|/Game/Traps/ActivateAbleProps.ActivateAbleProps_C|SetActivatedTime _output_get (Utilities|Time|GetGameTimeinSeconds))
  ;;[1 1 1] Update behaviour tree whether is it activated or not
  (AI|Navigation|StopMovement _returnvalue_2)
  (AI|RunBehaviorTree _returnvalue_2 "/Game/Controllers/AIController/Stone_Golem/StoneGolem_Idle_BT.StoneGolem_Idle_BT"))

(event Custom|WakeUp
  ;[1 1 1] Activates Golemn
  (Actor|DestroyActor (Variables|Default|GetGolemnActivator))
  (Variables|Default|SetGolemnActivator 0)
  (Variables|Default|SetActivatedTime (Utilities|Time|GetGameTimeinSeconds))
  (Variables|Default|SetisActivated true)
  (bind _returnvalue (Animation|PlayAnimMontage "/Game/Characters/NPC/NeutralCharacter/Stone_Golem/Animations/Stone_Golem_Armature_WakeUp_Montage.Stone_Golem_Armature_WakeUp_Montage" 1.0 "None"))
  (Utilities|FlowControl|Delay _returnvalue)
  (Utilities|Time|SetTimerbyEvent (delegate Custom|Deactivate) (Variables|Default|GetLifeDuration))
  (AI|RunBehaviorTree (AI|GetAIController self) "/Game/Controllers/AIController/Stone_Golem/StoneGolem_BT.StoneGolem_BT"))

(event Custom|Deactivate
  (CallFunction|GotoSleep))

(event Custom|StompAttack
  (bind _stompareaindicator (Variables|Default|GetStompAreaIndicator))
  (Animation|PlayAnimMontage "/Game/Characters/NPC/NeutralCharacter/Stone_Golem/Animations/Stone_Golem_Stomp_Montage.Stone_Golem_Stomp_Montage" 1.0 "None")
  (bind _grow (Timeline|Timeline_0 PlayFromStart)
    (:Update
      (Transformation|SetRelativeScale3D _stompareaindicator (Math|Vector|MakeVector (* _grow 7.0) (* _grow 7.0) (* _grow 7.0)))
      (Rendering|SetVisibility (Variables|Default|GetStompAreaIndicator) true false))
    (:Finished
      (Components|Sphere|SetSphereRadius (Variables|Default|GetStompArea) 3e+02 true)
      (Rendering|SetVisibility _stompareaindicator false false)
      (CallFunction|StompDamage))))

(event EventBeginPlay
  (|CallParentFunction)
  (Utilities|IsValid (Variables|Default|GetGolemnActivator)
    (:Is%20Valid
      (Actor|DestroyActor (Variables|Default|GetGolemnActivator)))
    (:Is%20Not%20Valid
      _))
  (CallFunction|GotoSleep)
  (Variables|Default|SetisActivated true)
  (Components|Sphere|SetSphereRadius (Variables|Default|GetStompArea) 0.0 true)
  (Rendering|SetVisibility (Variables|Default|GetStompAreaIndicator) false false))

(event Collision|EventActorBeginOverlap
  (params (OtherActor :type Actor%20Object%20Reference))
  (|CallParentFunction OtherActor) ; This node is disabled and will not be called.\nDrag off pins to build functionality.
)

(event EventTick
  (params (DeltaSeconds :type Float%20%28single-precision%29))
  (|CallParentFunction DeltaSeconds) ; This node is disabled and will not be called.\nDrag off pins to build functionality.
)

(fn ConstructionScript
  (|CallParentFunction)
  (Utilities|FlowControl|Sequence
    (:then_0
      (bind _output_get (Variables|Default|SetHealth 1e+03))
      (Variables|Default|SetMaxHealth _output_get))
    (:then_1
      (Variables|Default|SetDamage 5e+01))
    (:then_2
      (Variables|Default|SetPhysicalResist 0.5))
    (:then_3
      (Variables|Default|SetMagicalResist 0.2))
    (:then_4
      (bind _output_get_2 (Variables|Default|SetMovementSpeed 1e+02))
      (Variables|/Script/Engine.CharacterMovementComponent|SetMaxWalkSpeed (Variables|Character|GetCharacterMovement) _output_get_2))
    (:then_5
      (Variables|Default|SetXPGain 0))
    (:then_6
      (Variables|Default|SetisLarge true))
    (:then_7
      (Variables|Default|SetTeamNumber 1))
    (:then_8
      (Variables|Default|SetActivationCost 500))))

(fn StompDamage
  (bind _self self)
  (for _array_element (Variables|Default|GetTargetsToDamage)
    (Game|Damage|ApplyDamage _array_element (Variables|Default|GetDamage) (AI|GetAIController _self) _self "/Game/GameData/Damages/DamageType_Physical.DamageType_Physical_C"))
  (Components|Sphere|SetSphereRadius (Variables|Default|GetStompArea) 0.0 true)
  (Utilities|Array|Clear (Variables|Default|GetTargetsToDamage)))