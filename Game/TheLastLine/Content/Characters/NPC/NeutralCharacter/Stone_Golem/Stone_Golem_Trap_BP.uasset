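; Stone Golem trap, a child Blueprint of a parent trap class that takes a player index on activation.
; Activation calls the parent logic, sets the Active flag and plays a montage on the Golem skeletal mesh.
; The construction script hides the DamageRadius component and sets the trap's display name and activation cost.
; No damage logic appears in this Blueprint, and its BeginPlay and Tick nodes are disabled.
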(event Custom|CustomEvent
  (params (PlayerIndex :type Integer))
  (|CallParentFunction PlayerIndex)
  (Variables|Default|SetActive true)
  (Animation|Montage|PlayMontage (Variables|Default|GetGolem) 0))

(event EventBeginPlay
  (|CallParentFunction) ; This node is disabled and will not be called.\nDrag off pins to build functionality.
)

(event EventTick
  (params (DeltaSeconds :type Float%20%28single-precision%29))
  (|CallParentFunction DeltaSeconds) ; This node is disabled and will not be called.\nDrag off pins to build functionality.
)

(fn ConstructionScript
  (|CallParentFunction)
  (Rendering|SetVisibility (Variables|Default|GetDamageRadius) false false)
  (Variables|Default|SetTrapName "Stone Golem")
  (Variables|Default|SetActivationCost 800))