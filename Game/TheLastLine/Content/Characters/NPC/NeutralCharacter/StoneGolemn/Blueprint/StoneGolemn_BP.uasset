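; Stone golem character that starts dormant with a linked GolemnActivator actor, wakes for a timed lifespan, then sleeps again; it never reports dead.
; StompAtt grows StompArea on a timeline, collecting living overlapped characters, then StompAttack deals them physical damage and resets the area.
; AbilityQ is a cooldown-gated stomp calling StompAttack mid-animation without growing the area; AbilityE only plays a montage.
; The construction script sets its stats.
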(event OnComponentBeginOverlap(StompArea)
  (params (OverlappedComponent :type Primitive%20Component%20Object%20Reference) (OtherActor :type Actor%20Object%20Reference) (OtherComp :type Primitive%20Component%20Object%20Reference) (OtherBodyIndex :type Integer) (bFromSweep :type Boolean) (SweepResult :type Hit%20Result%20Structure%20%28by%20ref%29))
  (bind _asabstract_character (Utilities|Casting|CastToAbstractCharacter OtherActor))
  (if (not (CallFunction|IsDead _asabstract_character))
    (Utilities|Array|Add (Variables|Default|GetTargetsToDamage) _asabstract_character)
    (bind _result (Math|Integer|IncrementInt (Variables|Default|GetCounter))
      (:%20%20
        (Development|PrintString (Utilities|String|ToString(Integer) _result) true true "(R=1.000000,G=0.000000,B=0.000000,A=1.000000)" 3e+01)))))

(event OnComponentEndOverlap(ActivationTrigger)
  (params (OverlappedComponent :type Primitive%20Component%20Object%20Reference) (OtherActor :type Actor%20Object%20Reference) (OtherComp :type Primitive%20Component%20Object%20Reference) (OtherBodyIndex :type Integer)))

(event OnComponentEndOverlap(StompArea)
  (params (OverlappedComponent :type Primitive%20Component%20Object%20Reference) (OtherActor :type Actor%20Object%20Reference) (OtherComp :type Primitive%20Component%20Object%20Reference) (OtherBodyIndex :type Integer)))

(event Custom|GoToSleep
  (bind _returnvalue (Transformation|GetActorLocation))
  ;[1 1 1] Deactivates Golemn
  (Variables|Statue|SetisActivated false)
  (bind _returnvalue_2 (Game|SpawnActorfromClass "/Game/Traps/GolemnActivator/GolemnActivator_BP.GolemnActivator_BP_C" (Math|Transform|MakeTransform (Math|Vector|MakeVector (.x _returnvalue) (.y _returnvalue) (- (.z _returnvalue) 1e+02)) "0, 0, 0" "3.000000,3.000000,2.000000") "Undefined" 0 0))
  (bind _output_get (Variables|Statue|SetGolemnActivator _returnvalue_2))
  (Default|LinktoGolemn _output_get (Utilities|Array|Get(acopy) (Utilities|Array|MakeArray self)))
  (Variables|/Game/Traps/ActivateAbleProps.ActivateAbleProps_C|SetActivatedTime _output_get (Utilities|Time|GetGameTimeinSeconds)))

(event Custom|WakeUp
  ;[1 1 1] Activates Golemn
  (Actor|DestroyActor (Variables|Statue|GetGolemnActivator))
  (Variables|Statue|SetGolemnActivator 0)
  (Variables|Statue|SetActivatedTime (Utilities|Time|GetGameTimeinSeconds))
  (Variables|Statue|SetisActivated true)
  (bind _returnvalue (Animation|PlayAnimMontage "/Game/Characters/NPC/NeutralCharacter/Stone_Golem/Animations/Stone_Golem_Armature_WakeUp_Montage.Stone_Golem_Armature_WakeUp_Montage" 1.0 "None"))
  (Utilities|FlowControl|Delay _returnvalue)
  (Utilities|Time|SetTimerbyEvent (delegate Custom|Deactivate) (Variables|InAction|GetLifeDuration)))

(event Custom|Deactivate
  (CallFunction|GotoSleep))

(event Custom|StompAtt
  (Animation|PlayAnimMontage "/Game/Characters/NPC/NeutralCharacter/Stone_Golem/Animations/Stone_Golem_Stomp_Montage.Stone_Golem_Stomp_Montage" 1.0 "None")
  (bind _grow (Timeline|Timeline_GrowDamageArea Play)
    (:Update
      (Transformation|SetRelativeScale3D (Variables|Default|GetStompArea) (Math|Vector|MakeVector _grow _grow _grow)))
    (:Finished
      (CallFunction|StompAttack))))

(event EventBeginPlay
  ;[1 1 1] Link Golemn to an activator class, when it is a statue
  (Utilities|IsValid (Variables|Statue|GetGolemnActivator)
    (:Is%20Valid
      (Actor|DestroyActor (Variables|Statue|GetGolemnActivator)))
    (:Is%20Not%20Valid
      _))
  (CallFunction|GotoSleep)
  (Rendering|SetVisibility (Variables|Default|GetStompRadiusIndicator) true false)
  (Transformation|SetRelativeScale3D (Variables|Default|GetStompArea) "0, 0, 0"))

(event Collision|EventActorBeginOverlap
  (params (OtherActor :type Actor%20Object%20Reference))
  (|CallParentFunction OtherActor) ; This node is disabled and will not be called.\nDrag off pins to build functionality.
)

(event EventTick
  (params (DeltaSeconds :type Float%20%28single-precision%29)))

(event EventAbilityQ
  (bind _mesh (Variables|Character|GetMesh))
  ;[1 1 1] Stomp
  (bind _canuse (CallFunction|CanUseAbilityQ))
  (if _canuse
    (Utilities|FlowControl|Sequence
      (:then_0
        (if (not (Variables|Default|GetisAI))
          (CallFunction|DisableCharacterInput)
          (Variables|InAction|SetAbilityQActivatedTime (Utilities|Time|GetGameTimeinSeconds))))
      (:then_1
        (Components|Animation|PlayAnimation _mesh "/Game/Characters/NPC/NeutralCharacter/StoneGolemn/Assets/Animations/Stone_Golemm_Anim_Armature_Stomp.Stone_Golemm_Anim_Armature_Stomp" false)
        (Utilities|FlowControl|Delay 1.766667)
        (CallFunction|StompAttack)
        (Utilities|FlowControl|Delay 2.566667)
        (Components|Animation|SetAnimationMode _mesh "AnimationBlueprint")
        (CallFunction|EnableCharacterInput)))))

(event EventAbilityE
  ;[1 1 1] Sweep
  (Animation|Montage|PlayMontage (Variables|Character|GetMesh) "/Game/Characters/NPC/NeutralCharacter/StoneGolemn/Assets/Animations/StoneGolemnStompMontage.StoneGolemnStompMontage"))

(fn ConstructionScript
  (Utilities|FlowControl|Sequence
    (:then_0
      (bind _output_get (Variables|Default|SetHealth 1e+03))
      (Variables|Default|SetMaxHealth _output_get))
    (:then_1
      (Variables|Default|SetDamage 5e+01))
    (:then_2
      (Variables|Default|SetPhysicalResist 0.5))
    (:then_3
      (Variables|Default|SetMagicalResist 0.0))
    (:then_4
      (Variables|Default|SetMovementSpeed 1.5e+02))
    (:then_5
      (Variables|Default|SetXPGain 0))
    (:then_6
      (Variables|Default|SetisLarge true))
    (:then_7
      (Variables|Default|SetTeamNumber 1))))

(fn StompAttack
  (bind _self self)
  (for _array_element (Variables|Default|GetTargetsToDamage)
    (Game|Damage|ApplyDamage _array_element (Variables|Default|GetDamage) (AI|GetAIController _self) _self "/Game/GameData/Damages/DamageType_Physical.DamageType_Physical_C"))
  (Transformation|SetRelativeScale3D (Variables|Default|GetStompArea) "0, 0, 0")
  (Utilities|Array|Clear (Variables|Default|GetTargetsToDamage)))

(fn IsDead
  (return false))

(fn CanUseAbilityQ
  (return (<= (Variables|InAction|GetCooldownQtime) (- (Utilities|Time|GetGameTimeinSeconds) (Variables|InAction|GetAbilityQActivatedTime)))))