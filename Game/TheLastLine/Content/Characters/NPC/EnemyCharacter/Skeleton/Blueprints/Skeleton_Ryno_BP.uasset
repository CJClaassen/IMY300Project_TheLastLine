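; Skeleton enemy character that sets its stats at construction, plays a rising montage on spawn and carries a spawned sword.
; Melee attacks turn it toward the player with a timeline and randomly play a heavy or stab montage.
; Damage plays a hit reaction and rewards the Knight with points, XP and ability-slot XP, varying by damage causer.
; The health bar billboards to the camera, and kills show a rising gain widget.
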(event Custom|StabAttack
  (Animation|PlayAnimMontage "/Game/Characters/NPC/EnemyCharacter/Skeleton/Assets/Montages/Skeleton_StabAttack_Montage.Skeleton_StabAttack_Montage" 1.0 "None"))

(event Custom|HeavyAttack
  (Animation|PlayAnimMontage "/Game/Characters/NPC/EnemyCharacter/Skeleton/Assets/Montages/Skeleton_HeavyAttack_Montage.Skeleton_HeavyAttack_Montage" 0.8 "None"))

(event Custom|UpdateHealthbarRotate
  (bind _healthbar (Variables|Default|GetHealthBar))
  (Utilities|IsValid _healthbar
    (:Is%20Valid
      (Transformation|SetWorldRotation _healthbar (Math|Rotator|FindLookatRotation (Transformation|GetWorldLocation _healthbar) (Transformation|GetActorLocation (Game|GetPlayerCameraManager 0))) false false))))

(event Custom|ShowPointGain
  (bind _gainwidget (Variables|Default|GetGainWidget))
  (bind _gainwidget_2 (Variables|Default|GetGainWidget))
  (bind _relativelocation (Variables|/Script/Engine.SceneComponent|GetRelativeLocation _gainwidget))
  (CallFunction|UpdateGainWidgetRotate)
  (Rendering|SetVisibility _gainwidget_2 true false)
  (bind _moveup (Timeline|MoveWidgetUp_Timeline PlayFromStart)
    (:Update
      (Transformation|SetRelativeLocation _gainwidget (Math|Vector|MakeVector (.x _relativelocation) (.y _relativelocation) (+ (.z _relativelocation) _moveup)) false false))
    (:Finished
      (Rendering|SetVisibility _gainwidget_2 false false))))

(event Custom|SetUpHealthBar
  (bind _asenemy_health_bar_widget (Utilities|Casting|CastToEnemyHealthBar_Widget (UserInterface|GetUserWidgetObject (Variables|Default|GetHealthBar))))
  (Default|SetOwner _asenemy_health_bar_widget self)
  (if (Variables|Default|GetHealthBarToggle)
    (CallFunction|ShowHealthBar)
    (else
      (CallFunction|HideHealthBar))))

(event Custom|CreateWeapon
  (bind _returnvalue (Game|SpawnActorfromClass "/Game/Items/Sword/Sword1_BP.Sword1_BP_C" (Transformation|GetActorTransform) "Undefined" 0 self))
  (Variables|Default|SetWeapon _returnvalue)
  (Variables|/Game/Items/ItemBP.ItemBP_C|SetHolder _returnvalue self)
  (Variables|/Game/Items/ItemBP.ItemBP_C|SetHolderTeam _returnvalue (Variables|Default|GetTeamNumber))
  (Transformation|AttachComponentToComponent _returnvalue (Variables|Character|GetMesh) "WeaponSocket" "SnapToTarget" "SnapToTarget" "SnapToTarget" false))

(event Custom|HideHealthBar
  (Rendering|SetVisibility (Variables|Default|GetHealthBar) false false))

(event Custom|ShowHealthBar
  (Rendering|SetVisibility (Variables|Default|GetHealthBar) true false))

(event Custom|UpdateSpeed
  (bind _charactermovement (Variables|Character|GetCharacterMovement))
  (Variables|/Script/Engine.CharacterMovementComponent|SetMaxWalkSpeed _charactermovement (+ (Class|MovementComponent|GetMaxSpeed _charactermovement) 5e+01)))

(event Custom|FacePlayer
  (bind _self self)
  (bind _turntrack (Timeline|Timeline_0 PlayFromStart)
    (:Update
      (Transformation|SetActorRotation (Math|Rotator|Lerp(Rotator) (Transformation|GetActorRotation _self) (Math|Rotator|MakeRotator 0.0 0.0 (.yaw (Math|Rotator|FindLookatRotation (Transformation|GetActorLocation _self) (Transformation|GetActorLocation (Game|Player|GetPlayerPawn 0))))) _turntrack true)))))

(event Custom|Walk
  (Variables|/Script/Engine.CharacterMovementComponent|SetMaxWalkSpeed (Variables|Character|GetCharacterMovement) 1e+02))

(event Custom|Run
  (Variables|/Script/Engine.CharacterMovementComponent|SetMaxWalkSpeed (Variables|Character|GetCharacterMovement) 6e+02))

(event Custom|HandleAttack)

(event Custom|Summoned
  (Animation|PlayAnimMontage "/Game/Characters/NPC/EnemyCharacter/Skeleton_Mage/Animations/Skeleton_Summoned_Rising_Montage.Skeleton_Summoned_Rising_Montage" 1.75 "None")
  (Utilities|FlowControl|Delay 3.0))

(event Custom|UpdateGainWidgetRotate
  (bind _returnvalue (Game|GetPlayerCameraManager 0))
  (bind _gainwidget (Variables|Default|GetGainWidget))
  (bind _returnvalue_2 (Transformation|GetWorldLocation _gainwidget))
  (bind _returnvalue_3 (Transformation|GetActorLocation _returnvalue))
  (bind _returnvalue_4 (Math|Rotator|FindLookatRotation _returnvalue_2 _returnvalue_3))
  (Utilities|IsValid _gainwidget
    (:Is%20Valid
      (Transformation|SetWorldRotation _gainwidget (Math|Rotator|MakeRotator (.roll _returnvalue_4) (.pitch _returnvalue_4) (.yaw _returnvalue_4)) false false))))

(event EventBeginPlay
  (|CallParentFunction)
  (CallFunction|ToggleHealthBar)
  (Variables|/Script/Engine.CharacterMovementComponent|SetMaxWalkSpeed (Variables|Character|GetCharacterMovement) (Variables|Default|GetMovementSpeed))
  (CallFunction|CreateWeapon)
  (bind _outactors (Actor|GetAllActorsOfClass "/Game/Sound/Arena/ArenaSoundManager_BP.ArenaSoundManager_BP_C"))
  (Variables|Default|SetSoundManager (Utilities|Array|Get(acopy) _outactors))
  (bind _astop_down_game_mode (Utilities|Casting|CastToTopDownGameMode (Game|GetGameMode)))
  (Variables|Default|SetMapName (Variables|/Game/GameData/GameModes/TopDownGameMode.TopDownGameMode_C|GetcurrentMap _astop_down_game_mode))
  (CallFunction|Summoned)
  (CallFunction|SetUpHealthBar)
  (Rendering|SetVisibility (Variables|Default|GetGainWidget) false false))

(event Collision|EventActorBeginOverlap
  (params (OtherActor :type Actor%20Object%20Reference)))

(event EventTick
  (params (DeltaSeconds :type Float%20%28single-precision%29))
  (|CallParentFunction DeltaSeconds)
  (CallFunction|UpdateHealthbarRotate))

(event EventAbilityE
  (CallFunction|HeavyAttack))

(event EventAbilityQ
  (CallFunction|StabAttack))

(event EventPlayDead
  (|CallParentFunction)
  (Variables|Default|SethasIndicated true)
  (Class|Pawn|DetachfromControllerPendingDestroy)
  (Components|DestroyComponent (Variables|Default|GetHealthBar)))

(event Game|Damage|EventAnyDamage
  (params (Damage :type Float%20%28single-precision%29) (DamageType :type Damage%20Type%20Object%20Reference) (InstigatedBy :type Controller%20Object%20Reference) (DamageCauser :type Actor%20Object%20Reference))
  (bind _xpgain (Variables|Default|GetXPGain))
  (bind _xpgain_2 (Variables|Default|GetXPGain))
  (bind _returnvalue (/ _xpgain_2 2))
  (if (not (CallFunction|IsDead))
    (|CallParentFunction Damage DamageType InstigatedBy DamageCauser)
    (Animation|PlayAnimMontage "/Game/Characters/NPC/EnemyCharacter/Skeleton/Assets/Montages/Skeleton_Hit1_Montage.Skeleton_Hit1_Montage" 2.0 "None")
    (Utilities|IsValid InstigatedBy
      (:Is%20Valid
        (bind _ascustom_player_controller_bp (Utilities|Casting|CastToCustomPlayerController_BP InstigatedBy))
        (bind _asknight_bp (Utilities|Casting|CastToKnight_BP (Pawn|GetControlledPawn _ascustom_player_controller_bp)))
        (bind _ascast_abilities_bp (Utilities|Casting|CastToCastAbilities_BP DamageCauser)
          (:then
            (if (CallFunction|IsDead)
              (CallFunction|ShowPointGain)
              (Default|UpdateAbilitySlot _asknight_bp (Variables|/Game/Abilities/CastAbilities/CastAbilities_BP.CastAbilities_BP_C|GetAbilitySlotIndex _ascast_abilities_bp) (* (Math|Conversions|ToFloat(Integer) (Variables|Default|GetXPGain)) (Variables|/Game/Abilities/CastAbilities/CastAbilities_BP.CastAbilities_BP_C|GetXpModifier _ascast_abilities_bp)))
              ;[1 1 1] Give player points upon skeleton death
              (Default|UpdatePlayerPoints _asknight_bp _xpgain :!label _label)
              ;[1 1 1] Give Player XP upon skeleton death
              (CallFunction|UpdateGainWidget _xpgain (Variables|Default|GetXPGain))
              (Default|UpdatePlayerXP _asknight_bp (Math|Conversions|ToFloat(Integer) (Variables|Default|GetXPGain)) :!label _label_2)
              (Collision|SetCollisionEnabled (Variables|Default|GetCapsuleComponent) "NoCollision")
              (else
                (Default|UpdateAbilitySlot _asknight_bp (Variables|/Game/Abilities/CastAbilities/CastAbilities_BP.CastAbilities_BP_C|GetAbilitySlotIndex _ascast_abilities_bp) (Variables|/Game/Abilities/CastAbilities/CastAbilities_BP.CastAbilities_BP_C|GetXpGainAlternative _ascast_abilities_bp)))))
          (:CastFailed
            (Utilities|Casting|CastToActivateAbleProps DamageCauser
              (:then
                (if (CallFunction|IsDead)
                  (CallFunction|ShowPointGain)
                  (Default|UpdatePlayerPoints _asknight_bp _returnvalue)
                  (CallFunction|UpdateGainWidget _returnvalue (Variables|Default|GetXPGain))
                  (goto _label_2)))
              (:CastFailed
                (if (CallFunction|IsDead)
                  (CallFunction|ShowPointGain)
                  (goto _label)
                  (else
                    (Development|PrintString "PeanutsHello")))))))))))

(event EventDestroyed
  (bind _weapon (Variables|Default|GetWeapon))
  (Utilities|IsValid _weapon
    (:Is%20Valid
      (Actor|DestroyActor _weapon))))

(event EventMeleeAttack
  (CallFunction|FacePlayer)
  (switch int (Math|Random|RandomIntegerinRange 0 1)
    (:Default
      (CallFunction|HeavyAttack :!label _label))
    (:0
      (goto _label))
    (:1
      (CallFunction|StabAttack))))

(event EventToggleHealthBar
  (Utilities|IsValid (Variables|Default|GetHealthBar)
    (:Is%20Valid
      (|CallParentFunction)
      (if (Variables|Default|GetHealthBarToggle)
        (CallFunction|HideHealthBar)
        (else
          (CallFunction|ShowHealthBar))))))

(fn ConstructionScript
  ;[1 1 1] Initialize Character stats
  (Variables|Default|SetHealth 5e+01)
  (Variables|Default|SetDamage 5.0)
  (Variables|Default|SetPhysicalResist 0.0)
  (Variables|Default|SetMagicalResist -0.2)
  (Variables|Default|SetMovementSpeed 505.0)
  (Variables|Default|SetXPGain 40)
  (Variables|Default|SetisLarge false)
  (Variables|Default|SetTeamNumber 2))

(fn UpdateGainWidget
  (params (Gold :type Integer) (XP :type Integer))
  (bind _asenemy_gain_widget (Utilities|Casting|CastToEnemyGain_Widget (UserInterface|GetUserWidgetObject (Variables|Default|GetGainWidget))))
  (Default|UpdateDisplay _asenemy_gain_widget Gold XP))