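; Skeleton melee enemy for the top-down game, with a rising summon intro, sword, random heavy/stab attacks and a Battle Rage buff.
; Damage writes timed aggro to the AI Blackboard, animates a dynamic-material health bar and, on player kills, awards Knight points and XP with a floating gain widget.
; When linked to a mage, it polls on a timer to die alongside that mage and counts as a summoned kill in game stats.
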(event Custom|StabAttack
  (Animation|PlayAnimMontage "/Game/Characters/NPC/EnemyCharacter/Skeleton/Assets/Montages/Skeleton_StabAttack_Montage.Skeleton_StabAttack_Montage" 1.0 "None"))

(event Custom|HeavyAttack
  (Animation|PlayAnimMontage "/Game/Characters/NPC/EnemyCharacter/Skeleton/Assets/Montages/Skeleton_Attack_Heavy_V2_Montage.Skeleton_Attack_Heavy_V2_Montage" 0.8 "None"))

(event Custom|UpdateHealth
  (bind _plane (Variables|Default|GetPlane))
  (bind _m_healthbar (Variables|Default|GetM_HealthBar))
  (Utilities|IsValid _m_healthbar
    (:Is%20Valid
      (Rendering|Material|SetScalarParameterValue _m_healthbar "NewHealthPercentage" (Math|Float|Clamp(Float) (* (/ (Variables|Default|GetHealth) (Variables|Default|GetMaxHealth)) 1e+02) 0.0 1e+02) :!class /Script/Engine.MaterialInstanceDynamic)
      (if (CallFunction|IsDead)
        (Utilities|FlowControl|Delay 3.0)
        (Utilities|IsValid _plane
          (:Is%20Valid
            (Rendering|SetVisibility _plane false false)))))))

(event Custom|ShowPointGain
  (bind _gainwidget (Variables|Default|GetGainWidget))
  (bind _gainwidget_2 (Variables|Default|GetGainWidget))
  (bind _relativelocation (Variables|/Script/Engine.SceneComponent|GetRelativeLocation _gainwidget))
  (CallFunction|UpdateGainWidgetRotate)
  (Rendering|SetVisibility _gainwidget_2 true false)
  (bind _moveup (Timeline|MoveWidgetUp_Timeline PlayFromStart)
    (:Update
      (Transformation|SetRelativeLocation _gainwidget (Math|Vector|MakeVector (.x _relativelocation) (.y _relativelocation) (+ (.z _relativelocation) _moveup)) false false))
    (:Finished
      (Rendering|SetVisibility _gainwidget_2 false false))))

(event Custom|TurnAround
  (bind _self self)
  (bind _returnvalue (Transformation|GetActorRotation _self))
  (Variables|Turn|SetZRot (.yaw _returnvalue))
  (if (Math|Random|RandomBool)
    (Variables|Turn|SetTurnDirection 1.0)
    (bind _turncurve (Timeline|TurnAround_Timeline PlayFromStart)
      (:Update
        (Transformation|SetActorRotation (Math|Rotator|MakeRotator (.roll _returnvalue) (.pitch _returnvalue) (Math|Float|Lerp (Variables|Turn|GetZRot) (+ (Variables|Turn|GetZRot) (* (Math|Random|RandomFloatinRange 9e+01 1.8e+02) (Variables|Turn|GetTurnDirection))) _turncurve)))))
    (else
      (Variables|Turn|SetTurnDirection -1.0)
      (Timeline|TurnAround_Timeline PlayFromStart))))

(event Custom|CheckMage'sBeing
  (bind _linkedmage (Variables|Default|GetLinkedMage))
  (if (Default|IsDead _linkedmage)
    (Utilities|Time|ClearandInvalidateTimerbyHandle (Variables|Default|GetTimer_0))
    (Game|Damage|ApplyDamage self 1e+03 0 _linkedmage "/Game/GameData/Damages/DamageType_Magic.DamageType_Magic_C")))

(event Custom|SpawnSummonCircle
  (bind _summoningcircle (Variables|Default|GetSummoningCircle))
  (bind _returnvalue (Rendering|Material|CreateDynamicMaterialInstance "/Game/Abilities/Enemies/SummoningCircle_Mat.SummoningCircle_Mat" "None" :!class /Script/Engine.KismetMaterialLibrary))
  (bind (_direction _glowcurve _opacitycurve _rotationcurve) (Timeline|SummonCircle_Timeline PlayFromStart)
    (:Update
      (Rendering|Material|SetScalarParameterValue _returnvalue "GlowValue" _glowcurve :!class /Script/Engine.MaterialInstanceDynamic)
      (Rendering|Material|SetScalarParameterValue _returnvalue "OpacityValue" _opacitycurve :!class /Script/Engine.MaterialInstanceDynamic)
      (Transformation|SetRelativeRotation _summoningcircle (Math|Rotator|MakeRotator 0.0 0.0 _rotationcurve) false false)
      (Rendering|Material|SetMaterialbyName _summoningcircle (Utilities|Array|Get(acopy) (Class|MeshComponent|GetMaterialSlotNames _summoningcircle)) _returnvalue))
    (:Finished
      (Components|DestroyComponent _summoningcircle))))

(event Custom|SetAggroed
  (params (TargetEnemy :type Actor%20Object%20Reference))
  (bind _returnvalue (Utilities|Name|MakeLiteralName "PlayerIsTarget"))
  (bind _self self)
  (bind _returnvalue_2 (AI|GetAIController _self))
  (bind _returnvalue_3 (AI|GetBlackboard _returnvalue_2))
  (Variables|Default|SetAggroed true)
  (Utilities|IsValid _returnvalue_3
    (:Is%20Valid
      (AI|Components|Blackboard|SetValueasBool _returnvalue_3 (Utilities|Name|MakeLiteralName "Aggroed") true :!label _label)
      (AI|Components|Blackboard|SetValueasObject _returnvalue_3 (Utilities|Name|MakeLiteralName "TargetActor") TargetEnemy)
      (Utilities|Casting|CastToKnight_BP TargetEnemy
        (:then
          (AI|Components|Blackboard|SetValueasBool _returnvalue_3 _returnvalue true))
        (:CastFailed
          (AI|Components|Blackboard|SetValueasBool _returnvalue_3 _returnvalue false))))
    (:Is%20Not%20Valid
      (Development|PrintString "NO VALID BLACKBOARD!!!" true true "(R=0.369408,G=1.000000,B=0.000000,A=1.000000)" 1e+02)
      (Utilities|FlowControl|Delay 0.2)
      (Utilities|IsValid (AI|GetBlackboard self)
        (:Is%20Valid
          (goto _label))
        (:Is%20Not%20Valid
          _))))
  (Utilities|Time|SetTimerbyEvent (delegate Custom|LoseAggro) 2e+01))

(event Custom|FacePlayer
  (bind _self self)
  (bind _turntrack (Timeline|Timeline_0 PlayFromStart)
    (:Update
      (Transformation|SetActorRotation (Math|Rotator|Lerp(Rotator) (Transformation|GetActorRotation _self) (Math|Rotator|MakeRotator 0.0 0.0 (.yaw (Math|Rotator|FindLookatRotation (Transformation|GetActorLocation _self) (Transformation|GetActorLocation (Game|Player|GetPlayerPawn 0))))) _turntrack true)))))

(event Custom|PlayDeathSound
  (bind _self self)
  (bind _returnvalue (Transformation|GetActorLocation _self))
  (bind _astop_down_game_mode (Utilities|Casting|CastToTopDownGameMode (Game|GetGameMode)))
  (switch int (Math|Random|RandomIntegerinRange 0 1)
    (:Default
      (Audio|PlaySoundatLocation "/Game/Sound/Skeleton/Skeleton_Death_1_Cue.Skeleton_Death_1_Cue" _returnvalue "0, 0, 0" (Default|GetSoundEffectVolume _astop_down_game_mode) 1.0 0.0 "/Game/Sound/Skeleton/Skeleton_Death_Attenuation.Skeleton_Death_Attenuation" "/Game/Sound/Skeleton/Skeleton_Death_Concurrency.Skeleton_Death_Concurrency" 0 :!label _label))
    (:0
      (goto _label))
    (:1
      (Audio|PlaySoundatLocation "/Game/Sound/Skeleton/Skeleton_Death_2_Cue.Skeleton_Death_2_Cue" _returnvalue "0, 0, 0" (Default|GetSoundEffectVolume _astop_down_game_mode) 1.0 0.0 "/Game/Sound/Skeleton/Skeleton_Death_Attenuation.Skeleton_Death_Attenuation" "/Game/Sound/Skeleton/Skeleton_Death_Concurrency.Skeleton_Death_Concurrency" 0))))

(event Custom|SetUpHealthBar
  (bind _astop_down_game_mode (Utilities|Casting|CastToTopDownGameMode (Game|GetGameMode)))
  (bind _output_get (Variables|Default|SetHealthBarToggle (Variables|/Game/GameData/GameModes/TopDownGameMode.TopDownGameMode_C|GetToggleEnemyHealth _astop_down_game_mode)))
  (Development|PrintString (Utilities|String|Append "Skeleton says: " (Utilities|String|ToString(Boolean) _output_get)))
  (Rendering|SetVisibility (Variables|Default|GetPlane) (Variables|Default|GetHealthBarToggle) false))

(event Custom|LoseAggro
  (bind _self self)
  (bind _returnvalue (AI|GetBlackboard _self))
  (Variables|Default|SetAggroed false)
  (Utilities|IsValid _returnvalue
    (:Is%20Valid
      _)
    (:Is%20Not%20Valid
      (Development|PrintString "NO VALID BLACKBOARD!!!" true true "(R=0.369408,G=1.000000,B=0.000000,A=1.000000)" 1e+02)
      (Utilities|FlowControl|Delay 0.2)))
  (AI|Components|Blackboard|SetValueasBool _returnvalue (Utilities|Name|MakeLiteralName "Aggroed") false))

(event Custom|CreateWeapon
  (bind _returnvalue (Game|SpawnActorfromClass "/Game/Items/Sword/Sword1_BP.Sword1_BP_C" (Transformation|GetActorTransform) "Undefined" 0 self))
  (Variables|Default|SetWeapon _returnvalue)
  (Variables|/Game/Items/ItemBP.ItemBP_C|SetHolder _returnvalue self)
  (Variables|/Game/Items/ItemBP.ItemBP_C|SetHolderTeam _returnvalue (Variables|Default|GetTeamNumber))
  (Transformation|AttachComponentToComponent _returnvalue (Variables|Character|GetMesh) "WeaponSocket" "SnapToTarget" "SnapToTarget" "SnapToTarget" false))

(event Custom|UpdateSpeed
  (bind _charactermovement (Variables|Character|GetCharacterMovement))
  (Variables|/Script/Engine.CharacterMovementComponent|SetMaxWalkSpeed _charactermovement (+ (Class|MovementComponent|GetMaxSpeed _charactermovement) 5e+01)))

(event Custom|FaceTarget
  (params (TargetActor :type Actor%20Object%20Reference))
  (bind _self self)
  (Utilities|IsValid TargetActor
    (:Is%20Valid
      (bind _turntrack (Timeline|Timeline_1 PlayFromStart)
        (:Update
          (Utilities|IsValid TargetActor
            (:Is%20Valid
              (Transformation|SetActorRotation (Math|Rotator|Lerp(Rotator) (Transformation|GetActorRotation _self) (Math|Rotator|MakeRotator 0.0 0.0 (.yaw (Math|Rotator|FindLookatRotation (Transformation|GetActorLocation _self) (Transformation|GetActorLocation TargetActor)))) _turntrack true)))))))))

(event Custom|Walk
  (Variables|/Script/Engine.CharacterMovementComponent|SetMaxWalkSpeed (Variables|Character|GetCharacterMovement) 1e+02))

(event Custom|Run
  (Variables|/Script/Engine.CharacterMovementComponent|SetMaxWalkSpeed (Variables|Character|GetCharacterMovement) 6e+02))

(event Custom|HandleAttack)

(event Custom|Summoned
  (Animation|PlayAnimMontage "/Game/Characters/NPC/EnemyCharacter/Skeleton_Mage/Animations/Skeleton_Summoned_Rising_Montage.Skeleton_Summoned_Rising_Montage" 1.75 "None")
  (CallFunction|SpawnSummonCircle)
  (Utilities|FlowControl|Delay 3.0))

(event Custom|UpdateGainWidgetRotate
  (bind _gainwidget (Variables|Default|GetGainWidget))
  (Utilities|IsValid _gainwidget
    (:Is%20Valid
      (Transformation|SetWorldRotation _gainwidget (Math|Rotator|MakeRotator 0.0 45.0 (+ (.z (Variables|Default|GetHealthbarRotation)) 9e+01)) false false))))

(event EventBeginPlay
  (Utilities|FlowControl|Delay 0.2)
  (CallFunction|SetUpHealthBar)
  (Utilities|IsValid (Variables|Default|GetLinkedMage)
    (:Is%20Valid
      (bind _returnvalue (Utilities|Time|SetTimerbyEvent (delegate Custom|CheckMage'sBeing) 0.3 true))
      (Variables|Default|SetTimer_0 _returnvalue))
    (:Is%20Not%20Valid
      _))
  (Variables|/Script/Engine.CharacterMovementComponent|SetMaxWalkSpeed (Variables|Character|GetCharacterMovement) (Variables|Default|GetMovementSpeed))
  (CallFunction|CreateWeapon)
  (bind _outactors (Actor|GetAllActorsOfClass "/Game/Sound/Arena/ArenaSoundManager_BP.ArenaSoundManager_BP_C"))
  (Variables|Default|SetSoundManager (Utilities|Array|Get(acopy) _outactors))
  (bind _astop_down_game_mode (Utilities|Casting|CastToTopDownGameMode (Game|GetGameMode)))
  (Variables|Default|SetMapName (Variables|/Game/GameData/GameModes/TopDownGameMode.TopDownGameMode_C|GetcurrentMap _astop_down_game_mode))
  (CallFunction|Summoned)
  (CallFunction|SetUpHealthBar)
  (Rendering|SetVisibility (Variables|Default|GetGainWidget) false false))

(event Collision|EventActorBeginOverlap
  (params (OtherActor :type Actor%20Object%20Reference)))

(event EventToggleHealthBar
  (|CallParentFunction)
  (Rendering|SetVisibility (Variables|Default|GetPlane) (Variables|Default|GetHealthBarToggle) false))

(event EventMeleeAttack
  (params (TaregtActor :type Actor%20Object%20Reference))
  (CallFunction|FaceTarget TaregtActor)
  (switch int (Math|Random|RandomIntegerinRange 0 1)
    (:Default
      (CallFunction|HeavyAttack :!label _label))
    (:0
      (goto _label))
    (:1
      (CallFunction|StabAttack))))

(event EventTick
  (params (DeltaSeconds :type Float%20%28single-precision%29))
  (bind _healthbarrotation (Variables|Default|GetHealthbarRotation))
  (|CallParentFunction DeltaSeconds)
  (if (not (CallFunction|IsDead))
    (Utilities|FlowControl|Sequence
      (:then_0
        (if (not (CallFunction|IsDead))
          (Transformation|SetWorldLocationAndRotation (Variables|Default|GetPlane) (+ (Transformation|GetActorLocation) (Variables|Default|GetHealthbarLocation)) (Math|Rotator|MakeRotator (.x _healthbarrotation) (.y _healthbarrotation) (.z _healthbarrotation)) false false)))
      (:then_1
        (if (Variables|Default|GetNeedsAnimation)
          (CallFunction|AnimateDamageTaken (Variables|Default|GetM_HealthBar) DeltaSeconds))))))

(event EventAbilityE
  (CallFunction|HeavyAttack))

(event EventAbilityQ
  (CallFunction|StabAttack))

(event EventPlayDead
  (|CallParentFunction)
  (Variables|Default|SethasIndicated true)
  (CallFunction|PlayDeathSound)
  (Class|Pawn|DetachfromControllerPendingDestroy)
  (CallFunction|UpdateGameStats)
  (Components|DestroyComponent (Variables|Default|GetPlane)))

(event Game|Damage|EventAnyDamage
  (params (Damage :type Float%20%28single-precision%29) (DamageType :type Damage%20Type%20Object%20Reference) (InstigatedBy :type Controller%20Object%20Reference) (DamageCauser :type Actor%20Object%20Reference))
  (bind _xpgain (Variables|Default|GetXPGain))
  (bind _xpgain_2 (Variables|Default|GetXPGain))
  (bind _returnvalue (/ _xpgain_2 2))
  (if (not (CallFunction|IsDead))
    (CallFunction|SetAggroed DamageCauser)
    (|CallParentFunction Damage DamageType InstigatedBy DamageCauser)
    (CallFunction|UpdateHealth)
    (Variables|Default|SetNeedsAnimation true)
    (Animation|PlayAnimMontage "/Game/Characters/NPC/EnemyCharacter/Skeleton/Assets/Montages/Skeleton_Hit1_Montage.Skeleton_Hit1_Montage" 2.0 "None")
    (Utilities|IsValid InstigatedBy
      (:Is%20Valid
        (bind _ascustom_player_controller_bp (Utilities|Casting|CastToCustomPlayerController_BP InstigatedBy))
        (bind _asknight_bp (Utilities|Casting|CastToKnight_BP (Pawn|GetControlledPawn _ascustom_player_controller_bp)))
        (bind _ascast_abilities_bp (Utilities|Casting|CastToCastAbilities_BP DamageCauser)
          (:then
            (if (CallFunction|IsDead)
              (CallFunction|ShowPointGain)
              (Default|UpdateAbilitySlot _asknight_bp (Variables|/Game/Abilities/CastAbilities/CastAbilities_BP.CastAbilities_BP_C|GetAbilitySlotIndex _ascast_abilities_bp) (* (Math|Conversions|ToFloat(Integer) (Variables|Default|GetXPGain)) (Variables|/Game/Abilities/CastAbilities/CastAbilities_BP.CastAbilities_BP_C|GetXpModifier _ascast_abilities_bp)))
              ;[1 1 1] Give player points upon skeleton death
              (Default|UpdatePlayerPoints _asknight_bp _xpgain :!label _label)
              ;[1 1 1] Give Player XP upon skeleton death
              (CallFunction|UpdateGainWidget _xpgain (Variables|Default|GetXPGain))
              (Default|UpdatePlayerXP _asknight_bp (Math|Conversions|ToFloat(Integer) (Variables|Default|GetXPGain)) :!label _label_2)
              (Collision|SetCollisionEnabled (Variables|Default|GetCapsuleComponent) "NoCollision")
              (else
                (Default|UpdateAbilitySlot _asknight_bp (Variables|/Game/Abilities/CastAbilities/CastAbilities_BP.CastAbilities_BP_C|GetAbilitySlotIndex _ascast_abilities_bp) (Variables|/Game/Abilities/CastAbilities/CastAbilities_BP.CastAbilities_BP_C|GetXpGainAlternative _ascast_abilities_bp)))))
          (:CastFailed
            (Utilities|Casting|CastToActivateAbleProps DamageCauser
              (:then
                (if (CallFunction|IsDead)
                  (CallFunction|ShowPointGain)
                  (Default|UpdatePlayerPoints _asknight_bp _returnvalue)
                  (CallFunction|UpdateGainWidget _returnvalue (Variables|Default|GetXPGain))
                  (goto _label_2)))
              (:CastFailed
                (if (CallFunction|IsDead)
                  (CallFunction|ShowPointGain)
                  (goto _label)
                  (else
                    (Development|PrintString "PeanutsHello")))))))))))

(event EventDestroyed
  (bind _weapon (Variables|Default|GetWeapon))
  (Utilities|IsValid _weapon
    (:Is%20Valid
      (Actor|DestroyActor _weapon))))

(event EventAnimateDamageTaken
  (params (Material :type Material%20Instance%20Dynamic%20Object%20Reference) (DeltaSeconds :type Float%20%28single-precision%29))
  (if (<= (Variables|Default|GetHealth) (Variables|Default|GetAnimateHealth))
    (Rendering|Material|SetVectorParameterValue Material "DamagedHealthColor" "(R=0.960784,G=0.349020,B=0.000000,A=1.000000)" :!class /Script/Engine.MaterialInstanceDynamic)
    (Rendering|Material|SetScalarParameterValue Material "isDamage" 1.0 :!class /Script/Engine.MaterialInstanceDynamic)
    (Variables|Default|SetAnimateHealth (- (Variables|Default|GetAnimateHealth) (* DeltaSeconds 3e+01)))
    (Rendering|Material|SetScalarParameterValue Material "OldHealthPercentage" (* (/ (Variables|Default|GetAnimateHealth) (Variables|Default|GetMaxHealth)) 1e+02) :!class /Script/Engine.MaterialInstanceDynamic)
    (else
      (Variables|Default|SetNeedsAnimation false))))

(fn ConstructionScript
  ;[1 1 1] Initialize Character stats
  (bind _output_get (Variables|Default|SetHealth 5e+01))
  (Variables|Default|SetMaxHealth _output_get)
  (Variables|Default|SetDamage 5.0)
  (Variables|Default|SetPhysicalResist 0.0)
  (Variables|Default|SetMagicalResist -0.2)
  (Variables|Default|SetMovementSpeed 4.8e+02)
  (Variables|Default|SetXPGain 40)
  (Variables|Default|SetisLarge false)
  (Variables|Default|SetTeamNumber 2)
  (bind _returnvalue (Rendering|Material|CreateDynamicMaterialInstance (Variables|Default|GetPlane) 0 "/Game/Characters/NPC/HealthMaterials/M_Health.M_Health" "None" :!class /Script/Engine.PrimitiveComponent))
  (Variables|Default|SetM_HealthBar _returnvalue)
  (Transformation|SetWorldLocationAndRotation (Variables|Default|GetPlane) (+ (Transformation|GetActorLocation) (Variables|Default|GetHealthbarLocation)) (Math|Rotator|MakeRotator (.x (Variables|Default|GetHealthbarRotation)) (.y (Variables|Default|GetHealthbarRotation)) (.z (Variables|Default|GetHealthbarRotation))) false false)
  (Variables|Default|SetHealthbarRotation (Variables|Default|GetHealthbarRotation_Final))
  (Variables|Default|SetHealthbarLocation "0, 0,200.000000"))

(fn UpdateGainWidget
  (params (Gold :type Integer) (XP :type Integer))
  (bind _asenemy_gain_widget (Utilities|Casting|CastToEnemyGain_Widget (UserInterface|GetUserWidgetObject (Variables|Default|GetGainWidget))))
  (Default|UpdateDisplay _asenemy_gain_widget Gold XP))

(fn UpdateGameStats
  (if (not (Variables|Default|GetHasAdded))
    (Variables|Default|SetHasAdded true)
    (Utilities|IsValid (Variables|Default|GetLinkedMage)
      (:Is%20Valid
        (bind _astll_game_instance (Utilities|Casting|CastToTLL_GameInstance (Game|GetGameInstance)))
        (Default|UnitKill _astll_game_instance "SummonedSkeletons"))
      (:Is%20Not%20Valid
        (bind _astll_game_instance_2 (Utilities|Casting|CastToTLL_GameInstance (Game|GetGameInstance)))
        (Default|UnitKill _astll_game_instance_2 "Skeleton")))))

(fn BattleRage
  (params (DamageAdd :type Float%20%28single-precision%29) (PhyResistAdd :type Float%20%28single-precision%29))
  (bind _mesh (Variables|Character|GetMesh))
  (Variables|Default|SetPhysicalResist (+ (Variables|Default|GetPhysicalResist) PhyResistAdd))
  (Variables|Default|SetDamage (+ (Variables|Default|GetDamage) DamageAdd))
  (bind _returnvalue (Game|SpawnActorfromClass "/Game/Characters/NPC/EnemyCharacter/Skeleton_Warrior/GlowEyes_BP.GlowEyes_BP_C" (Transformation|GetActorTransform) "AlwaysSpawn" 0 0))
  (Transformation|AttachComponentToComponent _returnvalue (Variables|Character|GetMesh) "EyesSocket" "SnapToTarget" "SnapToTarget" "SnapToTarget" false)
  (Variables|Default|SetGlowEyes _returnvalue)
  (Rendering|Material|SetMaterialbyName _mesh (Utilities|Array|Get(acopy) (Class|MeshComponent|GetMaterialSlotNames _mesh)) "/Game/Characters/NPC/EnemyCharacter/Skeleton_Warrior/BattleRageGlow_Mat_Inst.BattleRageGlow_Mat_Inst"))

(fn RemoveBattleRage
  (params (DamageLose :type Float%20%28single-precision%29) (PhyResistLose :type Float%20%28single-precision%29))
  (bind _gloweyes (Variables|Default|GetGlowEyes))
  (bind _mesh (Variables|Character|GetMesh))
  (Variables|Default|SetPhysicalResist (- (Variables|Default|GetPhysicalResist) PhyResistLose))
  (Variables|Default|SetDamage (- (Variables|Default|GetDamage) DamageLose))
  (Rendering|Material|SetMaterialbyName _mesh (Utilities|Array|Get(acopy) (Class|MeshComponent|GetMaterialSlotNames _mesh)) "/Game/Characters/NPC/EnemyCharacter/Skeleton/Assets/Skeleton_Material.Skeleton_Material")
  (Utilities|IsValid _gloweyes
    (:Is%20Valid
      (Actor|DestroyActor _gloweyes))))