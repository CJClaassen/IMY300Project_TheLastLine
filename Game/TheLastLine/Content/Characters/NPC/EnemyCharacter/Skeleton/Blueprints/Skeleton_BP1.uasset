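; Skeleton enemy character for arena combat, with its base stats and team set in the construction script.
; On spawn it attaches a team-tagged sword, and a looping timer gradually raises its walk speed.
; Ability and melee events play heavy or stab montages; death detaches the controller and later destroys the sword.
; Damage plays a hit reaction, then rewards the Knight player by damage source (ability, prop, other) and cues crowd sound on kills.
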(event Custom|StabAttack
  (Animation|PlayAnimMontage "/Game/Characters/NPC/EnemyCharacter/Skeleton/Assets/Montages/Skeleton_StabAttack_Montage.Skeleton_StabAttack_Montage" 1.0 "None"))

(event Custom|HeavyAttack
  (Animation|PlayAnimMontage "/Game/Characters/NPC/EnemyCharacter/Skeleton/Assets/Montages/Skeleton_HeavyAttack_Montage.Skeleton_HeavyAttack_Montage" 1.0 "None"))

(event Custom|CreateSword
  (bind _returnvalue (Game|SpawnActorfromClass "/Game/Items/Sword/Sword1_BP.Sword1_BP_C" (Transformation|GetActorTransform) "Undefined" 0 self))
  (Variables|Default|SetWeapon _returnvalue)
  (Variables|/Game/Items/Sword/Sword1_BP.Sword1_BP_C|SetHolder _returnvalue self)
  (Variables|/Game/Items/Sword/Sword1_BP.Sword1_BP_C|SetHolderTeam _returnvalue (Variables|Default|GetTeamNumber))
  (Transformation|AttachComponentToComponent _returnvalue (Variables|Character|GetMesh) "WeaponSocket" "SnapToTarget" "SnapToTarget" "SnapToTarget" false))

(event Custom|UpdateSpeed
  (bind _charactermovement (Variables|Character|GetCharacterMovement))
  (Variables|/Script/Engine.CharacterMovementComponent|SetMaxWalkSpeed _charactermovement (+ (Class|MovementComponent|GetMaxSpeed _charactermovement) 5e+01)))

(event Custom|HandleAttack)

(event EventBeginPlay
  (CallFunction|CreateSword)
  (Utilities|Time|SetTimerbyEvent (delegate Custom|UpdateSpeed) 25.0 true)
  (bind _outactors (Actor|GetAllActorsOfClass "/Game/Sound/Arena/ArenaSoundManager_BP.ArenaSoundManager_BP_C"))
  (Variables|Default|SetSoundManager (Utilities|Array|Get(acopy) _outactors))
  (bind _astop_down_game_mode (Utilities|Casting|CastToTopDownGameMode (Game|GetGameMode)))
  (Variables|Default|SetMapName (Variables|/Game/GameData/GameModes/TopDownGameMode.TopDownGameMode_C|GetcurrentMap _astop_down_game_mode)))

(event Collision|EventActorBeginOverlap
  (params (OtherActor :type Actor%20Object%20Reference)))

(event EventAbilityE
  (CallFunction|HeavyAttack))

(event EventAbilityQ
  (CallFunction|StabAttack))

(event EventPlayDead
  (Class|Pawn|DetachfromControllerPendingDestroy)
  (Utilities|FlowControl|Delay 15.0)
  (Actor|DestroyActor (Variables|Default|GetWeapon)))

(event Game|Damage|EventAnyDamage
  (params (Damage :type Float%20%28single-precision%29) (DamageType :type Damage%20Type%20Object%20Reference) (InstigatedBy :type Controller%20Object%20Reference) (DamageCauser :type Actor%20Object%20Reference))
  (Development|PrintString (Utilities|String|ToString(Float) Damage) true true "(R=0.000000,G=0.660000,B=1.000000,A=1.000000)" 1e+01)
  (if (not (CallFunction|IsDead))
    (Animation|PlayAnimMontage "/Game/Characters/NPC/EnemyCharacter/Skeleton/Assets/Montages/Skeleton_Hit1_Montage.Skeleton_Hit1_Montage" 1.0 "None")
    (|CallParentFunction Damage DamageType InstigatedBy DamageCauser)
    (Utilities|IsValid InstigatedBy
      (:Is%20Valid
        (bind _ascustom_player_controller_bp (Utilities|Casting|CastToCustomPlayerController_BP InstigatedBy))
        (bind _asknight_bp (Utilities|Casting|CastToKnight_BP (Pawn|GetControlledPawn _ascustom_player_controller_bp)))
        (bind _ascast_abilities_bp (Utilities|Casting|CastToCastAbilities_BP DamageCauser)
          (:then
            (if (CallFunction|IsDead)
              (Default|UpdateAbilitySlot _asknight_bp (Variables|/Game/Abilities/CastAbilities/CastAbilities_BP.CastAbilities_BP_C|GetAbilitySlotIndex _ascast_abilities_bp) (* (Math|Conversions|ToFloat(Integer) (Variables|Default|GetXPGain)) (Variables|/Game/Abilities/CastAbilities/CastAbilities_BP.CastAbilities_BP_C|GetXpModifier _ascast_abilities_bp)))
              (Default|UpdatePlayerXP _asknight_bp (Math|Conversions|ToFloat(Integer) (Variables|Default|GetXPGain)))
              (Default|UpdatePlayerPoints _asknight_bp (Variables|Default|GetXPGain) :!label _label)
              (Collision|SetCollisionEnabled (Variables|Default|GetCapsuleComponent) "NoCollision")
              (Default|UpdateCrowd (Variables|Default|GetSoundManager) "Enemy_Death")
              (else
                (Default|UpdateAbilitySlot _asknight_bp (Variables|/Game/Abilities/CastAbilities/CastAbilities_BP.CastAbilities_BP_C|GetAbilitySlotIndex _ascast_abilities_bp) (Variables|/Game/Abilities/CastAbilities/CastAbilities_BP.CastAbilities_BP_C|GetXpGainAlternative _ascast_abilities_bp)))))
          (:CastFailed
            (Utilities|Casting|CastToActivateAbleProps DamageCauser
              (:then
                (if (CallFunction|IsDead)
                  (Default|UpdatePlayerXP _asknight_bp (* (Math|Conversions|ToFloat(Integer) (Variables|Default|GetXPGain)) 2.0))
                  (Default|UpdateCrowd (Variables|Default|GetSoundManager) "Enemy_Death")))
              (:CastFailed
                (if (CallFunction|IsDead)
                  (Default|UpdatePlayerXP _asknight_bp (Math|Conversions|ToFloat(Integer) (Variables|Default|GetXPGain)))
                  (goto _label)
                  (else
                    (Development|PrintString "PeanutsHello")))))))))))

(event EventMeleeAttack
  (CallFunction|HeavyAttack))

(fn ConstructionScript
  ;[1 1 1] Initialize Character stats
  (Variables|Default|SetHealth 5e+01)
  (Variables|Default|SetDamage 5.0)
  (Variables|Default|SetPhysicalResist 0.0)
  (Variables|Default|SetMagicalResist -0.2)
  (Variables|Default|SetMovementSpeed 2.5e+02)
  (Variables|Default|SetXPGain 40)
  (Variables|Default|SetisLarge false)
  (Variables|Default|SetTeamNumber 2))