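; Tutorial variant of the skeleton enemy whose AI behavior is switched by named actions.
; ExecuteAction branches on Do Nothing or Attack and calls Run Behavior Tree on the skeleton's AI controller in either case.
; Damage handling and construction defer to the parent class, and Tick has no logic.
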(event EventBeginPlay)

(event Collision|EventActorBeginOverlap
  (params (OtherActor :type Actor%20Object%20Reference)))

(event EventTick
  (params (DeltaSeconds :type Float%20%28single-precision%29)))

(event Game|Damage|EventAnyDamage
  (params (Damage :type Float%20%28single-precision%29) (DamageType :type Damage%20Type%20Object%20Reference) (InstigatedBy :type Controller%20Object%20Reference) (DamageCauser :type Actor%20Object%20Reference))
  (|CallParentFunction Damage DamageType InstigatedBy DamageCauser))

(fn ConstructionScript
  (|CallParentFunction))

(fn ExecuteAction
  (params (Action :type String) (TimesActionOfExecution :type Integer))
  (switch string Action
    (:Do%20Nothing
      (AI|RunBehaviorTree (AI|GetAIController self)))
    (:Attack
      (AI|RunBehaviorTree (AI|GetAIController self)))))