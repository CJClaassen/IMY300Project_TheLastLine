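; Skeleton mage enemy, a child NPC Blueprint that sets its own stats, carries a staff and plays a montage for basic attacks.
; Two timer-cooled abilities summon a pair of linked, no-XP skeleton minions nearby, which share its aggro, and cast a fireball.
; The fireball is a hand-attached actor swapped for a projectile on throw, and is destroyed if the mage takes damage or dies.
; Its kill is reported once to the GameInstance.
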(event Custom|BasicAttack
  (params (TargetActor :type Actor%20Object%20Reference))
  (CallFunction|FaceTarget TargetActor)
  (Animation|PlayAnimMontage "/Game/Characters/NPC/EnemyCharacter/Skeleton_Mage/Animations/Skeleton_Mage_Attack_Montage.Skeleton_Mage_Attack_Montage" 1.5 "None"))

(event Custom|SummonSkeletons
  (bind _returnvalue (Transformation|GetActorLocation))
  (bind (_x _y _z) (Math|Vector|BreakVector _returnvalue))
  (bind _randomlocation (Class|NavigationSystemV1|GetRandomPointinNavigableRadius _returnvalue 2e+02 0 0))
  (Animation|PlayAnimMontage "/Game/Characters/NPC/EnemyCharacter/Skeleton_Mage/Animations/Skeleton_Mage_Summon_Montage.Skeleton_Mage_Summon_Montage" 1.0 "None")
  (for _index (range 0 1)
    (bind _returnvalue_2 (Game|SpawnActorfromClass "/Game/Characters/NPC/EnemyCharacter/Skeleton/Blueprints/Skeleton_BP.Skeleton_BP_C" (Math|Transform|MakeTransform (Math|Vector|MakeVector (Math|Float|Clamp(Float) (.x _randomlocation) (- _x 2e+02) (+ _x 2e+02)) (Math|Float|Clamp(Float) (.y _randomlocation) (- (.y _randomlocation) 2e+02) (+ (.y _randomlocation) 2e+02)) _z)) "Undefined" 0 "0.000000,0.000000,0.000000" "120.000000,180.000000,90.000000" 0))
    (Utilities|IsValid _returnvalue_2
      (:Is%20Valid
        (Variables|/Game/Characters/NPC/EnemyCharacter/Skeleton/Blueprints/Skeleton_BP.Skeleton_BP_C|SetLinkedMage _returnvalue_2 self)
        (Variables|/Game/Characters/AbstractCharacter.AbstractCharacter_C|SetXPGain _returnvalue_2 0)
        (Variables|/Game/Characters/AbstractCharacter.AbstractCharacter_C|SethasSpawned _returnvalue_2 false)
        (Rendering|Material|SetMaterialbyName (Variables|/Script/Engine.Character|GetMesh _returnvalue_2) (Utilities|Array|Get(acopy) (Class|MeshComponent|GetMaterialSlotNames (Variables|/Script/Engine.Character|GetMesh _returnvalue_2))) "/Game/Characters/NPC/NeutralCharacter/Mercenary/Assets/Armour_Metal_Battered.Armour_Metal_Battered")
        (Utilities|Array|Add (Variables|Default|GetSkeletonMinions) _returnvalue_2)
        (if (Variables|Default|GetAggroed)
          (Default|SetAggroed _returnvalue_2)))))
  (Variables|Default|SetAbility1_IsOnCooldown true)
  (Development|PrintString "Ability on Cooldown" true true "(R=0.000000,G=0.660000,B=1.000000,A=1.000000)" 1e+01)
  (Utilities|Time|SetTimerbyEvent (delegate Custom|Ability1_Ready) 6e+01))

(event Custom|Ability1_Ready
  (Variables|Default|SetAbility1_IsOnCooldown false)
  (Development|PrintString "Ability 1 is Ready" true true "(R=0.000000,G=0.660000,B=1.000000,A=1.000000)" 1e+01))

(event Custom|ThrowFireball
  (bind _self self)
  (bind _fireball (Variables|Default|GetFireball))
  (bind _returnvalue (Game|SpawnActorfromClass "/Game/Items/Staff/Fireball_Projectile_BP.Fireball_Projectile_BP_C" (Transformation|GetActorTransform _fireball) "Undefined" 0 0))
  (Variables|/Game/Items/ItemBP.ItemBP_C|SetHolder _returnvalue _self)
  (Variables|/Game/Items/ItemBP.ItemBP_C|SetHolderTeam _returnvalue (Variables|Default|GetTeamNumber _self))
  (Actor|DestroyActor _fireball)
  (Development|PrintString "Throw Fireball" true true "(R=0.000000,G=0.660000,B=1.000000,A=1.000000)" 1e+01))

(event Custom|MakeFireball
  (bind _returnvalue (Game|SpawnActorfromClass "/Game/Items/Staff/Fireball_BP.Fireball_BP_C" (Transformation|GetActorTransform) "Undefined" 0 self))
  (bind _output_get (Variables|Default|SetFireball _returnvalue))
  (Transformation|AttachComponentToComponent _output_get (Variables|Character|GetMesh) "right_hand_FireballSocket" "SnapToTarget" "SnapToTarget" "SnapToTarget" false)
  (Development|PrintString "Fireball Spawned" true true "(R=0.000000,G=0.660000,B=1.000000,A=1.000000)" 1e+01))

(event Custom|Fireball_Cast
  (params (targetActor :type Actor%20Object%20Reference))
  (CallFunction|FaceTarget targetActor)
  (Animation|PlayAnimMontage "/Game/Characters/NPC/EnemyCharacter/Skeleton_Mage/Animations/Skeleton_Mage_Fireball_Montage.Skeleton_Mage_Fireball_Montage" 2.0 "None")
  (Variables|Default|SetAbility2_IsOnCooldown true)
  (Utilities|Time|SetTimerbyEvent (delegate Custom|Ability2_Ready) 6e+01))

(event Custom|Ability2_Ready
  (Variables|Default|SetAbility2_IsOnCooldown false)
  (Development|PrintString "Ability 2 is Ready" true true "(R=0.000000,G=0.660000,B=1.000000,A=1.000000)" 1e+01))

(event EventBeginPlay
  (|CallParentFunction)
  (Variables|/Script/Engine.CharacterMovementComponent|SetMaxWalkSpeed (Variables|Character|GetCharacterMovement) (Variables|Default|GetMovementSpeed))
  (Variables|Default|SetAbility1_IsOnCooldown true)
  (Utilities|Time|SetTimerbyEvent (delegate Custom|Ability1_Ready) (Math|Random|RandomFloatinRange 0.0 2.0))
  (Variables|Default|SetHasAdded false))

(event Collision|EventActorBeginOverlap
  (params (OtherActor :type Actor%20Object%20Reference))
  (|CallParentFunction OtherActor) ; This node is disabled and will not be called.\nDrag off pins to build functionality.
)

(event EventTick
  (params (DeltaSeconds :type Float%20%28single-precision%29))
  (|CallParentFunction DeltaSeconds) ; This node is disabled and will not be called.\nDrag off pins to build functionality.
)

(event EventCreateWeapon
  (bind _returnvalue (Game|SpawnActorfromClass "/Game/Items/Staff/Staff_BP.Staff_BP_C" (Transformation|GetActorTransform) "Undefined" 0 self))
  (Variables|Default|SetWeapon _returnvalue)
  (Variables|/Game/Items/ItemBP.ItemBP_C|SetHolder _returnvalue self)
  (Variables|/Game/Items/ItemBP.ItemBP_C|SetHolderTeam _returnvalue (Variables|Default|GetTeamNumber))
  (Transformation|AttachComponentToComponent _returnvalue (Variables|Character|GetMesh) "left_hand_StaffSocket" "SnapToTarget" "SnapToTarget" "SnapToTarget" false))

(event EventRangeAttack
  (params (TargetActor :type Actor%20Object%20Reference))
  (CallFunction|BasicAttack TargetActor))

(event EventUpdateMovementSpeed
  (params (Movement%20Speed :type Float%20%28single-precision%29)))

(event EventPlayDead
  (|CallParentFunction)
  (Utilities|IsValid (Variables|Default|GetFireball)
    (:Is%20Valid
      (Actor|DestroyActor (Variables|Default|GetFireball)))))

(event Game|Damage|EventAnyDamage
  (params (Damage :type Float%20%28single-precision%29) (DamageType :type Damage%20Type%20Object%20Reference) (InstigatedBy :type Controller%20Object%20Reference) (DamageCauser :type Actor%20Object%20Reference))
  (bind _fireball (Variables|Default|GetFireball))
  (|CallParentFunction Damage DamageType InstigatedBy DamageCauser)
  (Utilities|IsValid _fireball
    (:Is%20Valid
      (Actor|DestroyActor _fireball))))

(event EventUpdateGameStats
  (if (not (Variables|Default|GetHasAdded))
    (Variables|Default|SetHasAdded true)
    (bind _astll_game_instance (Utilities|Casting|CastToTLL_GameInstance (Game|GetGameInstance)))
    (Default|UnitKill _astll_game_instance "Mage")))

(event EventSetAggroed
  (params (TargetEnemy :type Actor%20Object%20Reference))
  (|CallParentFunction 0)
  (for _array_element (Variables|Default|GetSkeletonMinions)
    (Utilities|IsValid _array_element
      (:Is%20Valid
        (Default|SetAggroed _array_element)))))

(fn ConstructionScript
  (|CallParentFunction)
  (Utilities|FlowControl|Sequence
    (:then_0
      (bind _output_get (Variables|Default|SetHealth 3e+01))
      (Variables|Default|SetMaxHealth _output_get))
    (:then_1
      (Variables|Default|SetDamage 1e+01))
    (:then_2
      (Variables|Default|SetPhysicalResist -0.2))
    (:then_3
      (Variables|Default|SetMagicalResist 0.2))
    (:then_4
      (Variables|Default|SetMovementSpeed 1.5e+02))
    (:then_5
      (Variables|Default|SetXPGain 60))
    (:then_6
      (Variables|Default|SetisLarge false))
    (:then_7
      (Variables|Default|SetTeamNumber 2))))