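; Default skeleton enemy NPC Blueprint that configures a small enemy variant on top of its parent class.
; The construction script calls the parent, then sets health, damage, resistances (including negative magical resistance), movement and attack speed, XP gain and size flag.
; Stab and Slash ability events are declared but empty, and BeginPlay, overlap and Tick are disabled placeholders.
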(event EventBeginPlay
  (|CallParentFunction) ; This node is disabled and will not be called.\nDrag off pins to build functionality.
)

(event Collision|EventActorBeginOverlap
  (params (OtherActor :type Actor%20Object%20Reference))
  (|CallParentFunction OtherActor) ; This node is disabled and will not be called.\nDrag off pins to build functionality.
)

(event EventTick
  (params (DeltaSeconds :type Float%20%28single-precision%29))
  (|CallParentFunction DeltaSeconds) ; This node is disabled and will not be called.\nDrag off pins to build functionality.
)

(event EventAbilityQ
  ;[1 1 1] Abilities
  ;;[0.2384 1 0.9734] Stab Ability
)

(event EventAbilityE
  ;[1 1 1] Abilities
  ;;[0.2384 1 0.9734] Slash Ability
)

(fn ConstructionScript
  (|CallParentFunction)
  (Utilities|FlowControl|Sequence
    (:then_0
      (Variables|Default|SetHealth 35.0))
    (:then_1
      (Variables|Default|SetDamage 5.0))
    (:then_2
      (Variables|Default|SetMagicalResist -2e+01))
    (:then_3
      (Variables|Default|SetPhysicalResist 0.0))
    (:then_4
      (Variables|Default|SetMovementSpeed 1e+02))
    (:then_5
      (Variables|Default|SetAttackSpeed 0.7))
    (:then_6
      (Variables|Default|SetXPGain 40))
    (:then_7
      (Variables|Default|SetisLarge false))))