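; Skeleton archer enemy, a child character Blueprint that sets its stats and team in the construction script and fights with a bow.
; CreateWeapon attaches a bow and quiver to mesh sockets; RangeAttack faces the player and plays the attack montage.
; Separate events attach a prop arrow, animate the bow, and swap the arrow for a team-tagged projectile.
; The PlayerDistanceLimitBox overlap events are empty, leaving the PlayerTooClose blackboard logic disconnected.
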(event OnComponentBeginOverlap(PlayerDistanceLimitBox)
  (params (OverlappedComponent :type Primitive%20Component%20Object%20Reference) (OtherActor :type Actor%20Object%20Reference) (OtherComp :type Primitive%20Component%20Object%20Reference) (OtherBodyIndex :type Integer) (bFromSweep :type Boolean) (SweepResult :type Hit%20Result%20Structure%20%28by%20ref%29)))

(event OnComponentEndOverlap(PlayerDistanceLimitBox)
  (params (OverlappedComponent :type Primitive%20Component%20Object%20Reference) (OtherActor :type Actor%20Object%20Reference) (OtherComp :type Primitive%20Component%20Object%20Reference) (OtherBodyIndex :type Integer)))

(event Custom|SpawnArrow
  (bind _returnvalue (Game|SpawnActorfromClass "/Game/Items/Bow+Arrows/Arrow/Arrow_BP.Arrow_BP_C" (Transformation|GetActorTransform) "Undefined" 0 self))
  (bind _output_get (Variables|Default|SetArrow _returnvalue))
  (Transformation|AttachComponentToComponent _output_get (Variables|Character|GetMesh) "ArrowSocket" "SnapToTarget" "SnapToTarget" "SnapToTarget" false)
  (Development|PrintString "Arrow Spawned" true true "(R=0.000000,G=0.660000,B=1.000000,A=1.000000)" 1e+01))

(event Custom|ShootAttack
  (CallFunction|FacePlayer)
  (Animation|PlayAnimMontage "/Game/Characters/NPC/EnemyCharacter/Skeletom_Archer/Animations/Skeleton_Archer_Attack_Montage.Skeleton_Archer_Attack_Montage" 3.0 "None"))

(event Custom|PullBow
  (bind _asbow_bp (Utilities|Casting|CastToBow_BP (Variables|Default|GetWeapon)))
  (Animation|Montage|PlayMontage (Variables|/Game/Items/Bow+Arrows/Bow/Bow_BP.Bow_BP_C|GetBowMesh _asbow_bp) "/Game/Items/Bow+Arrows/Bow/Bow_Shoot_Montage.Bow_Shoot_Montage"
    (:then
      (Development|PrintString "Bow Shooting" true true "(R=0.000000,G=0.660000,B=1.000000,A=1.000000)" 1e+01))))

(event Custom|ShootBow
  (bind _self self)
  (bind _arrow (Variables|Default|GetArrow))
  (bind _returnvalue (Game|SpawnActorfromClass "/Game/Items/Bow+Arrows/Arrow/Arrow_Projectile_BP.Arrow_Projectile_BP_C" (Transformation|GetActorTransform _arrow) "Undefined" 0 0))
  (Variables|/Game/Items/ItemBP.ItemBP_C|SetInAttack _returnvalue true)
  (Variables|/Game/Items/Bow+Arrows/Arrow/Arrow_Projectile_BP.Arrow_Projectile_BP_C|SetHolder _returnvalue _self)
  (Variables|/Game/Items/Bow+Arrows/Arrow/Arrow_Projectile_BP.Arrow_Projectile_BP_C|SetHolderTeam _returnvalue (Variables|Default|GetTeamNumber _self))
  (Actor|DestroyActor _arrow)
  (Development|PrintString "Arrow Shoot" true true "(R=0.000000,G=0.660000,B=1.000000,A=1.000000)" 1e+01))

(event EventBeginPlay
  (|CallParentFunction))

(event Collision|EventActorBeginOverlap
  (params (OtherActor :type Actor%20Object%20Reference))
  (|CallParentFunction OtherActor) ; This node is disabled and will not be called.\nDrag off pins to build functionality.
)

(event EventTick
  (params (DeltaSeconds :type Float%20%28single-precision%29))
  (|CallParentFunction DeltaSeconds) ; This node is disabled and will not be called.\nDrag off pins to build functionality.
)

(event EventCreateWeapon
  (Utilities|FlowControl|Sequence
    (:then_0
      (bind _returnvalue (Game|SpawnActorfromClass "/Game/Items/Bow+Arrows/Bow/Bow_BP.Bow_BP_C" (Transformation|GetActorTransform) "Undefined" 0 self))
      (Variables|Default|SetWeapon _returnvalue)
      (Variables|/Game/Items/Bow+Arrows/Bow/Bow_BP.Bow_BP_C|SetHolder _returnvalue self)
      (Variables|/Game/Items/Bow+Arrows/Bow/Bow_BP.Bow_BP_C|SetHolderTeam _returnvalue (Variables|Default|GetTeamNumber))
      (Transformation|AttachComponentToComponent _returnvalue (Variables|Character|GetMesh) "left_handWeaponSocket" "SnapToTarget" "SnapToTarget" "SnapToTarget" false))
    (:then_1
      (bind _returnvalue_2 (Game|SpawnActorfromClass "/Game/Items/Bow+Arrows/Quiver/Quiver_BP.Quiver_BP_C" (Transformation|GetActorTransform) "Undefined" 0 self))
      (Transformation|AttachComponentToComponent _returnvalue_2 (Variables|Character|GetMesh) "higher_backSocket" "SnapToTarget" "SnapToTarget" "SnapToTarget" false))))

(event EventRangeAttack
  (CallFunction|ShootAttack))

(fn ConstructionScript
  (|CallParentFunction)
  (Utilities|FlowControl|Sequence
    (:then_0
      (Variables|Default|SetHealth 3e+01))
    (:then_1
      (Variables|Default|SetDamage 8.0))
    (:then_2
      (Variables|Default|SetPhysicalResist -0.1))
    (:then_3
      (Variables|Default|SetMagicalResist -0.2))
    (:then_4
      (Variables|Default|SetMovementSpeed 2e+02))
    (:then_5
      (Variables|Default|SetXPGain 45))
    (:then_6
      (Variables|Default|SetisLarge false))
    (:then_7
      (Variables|Default|SetTeamNumber 2))))