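; Skeleton warrior enemy that spawns with a sword, shield and random helmet, and can randomly block physical hits, except from traps, with a floating "blocked" widget.
; At half health, or when CounterBox counts enough nearby skeletons, it pauses its AI for a battle cry and enters Battle Rage.
; The rage expands AuraBox, which buffs damage and physical resistance of overlapping skeletons until they leave, while a looping timer pulses a ping wave.
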(event OnComponentBeginOverlap(AuraBox)
  (params (OverlappedComponent :type Primitive%20Component%20Object%20Reference) (OtherActor :type Actor%20Object%20Reference) (OtherComp :type Primitive%20Component%20Object%20Reference) (OtherBodyIndex :type Integer) (bFromSweep :type Boolean) (SweepResult :type Hit%20Result%20Structure%20%28by%20ref%29))
  (bind _percentincrease (Variables|Default|GetPercentIncrease))
  (if (not (CallFunction|IsDead))
    (if (Variables|Default|GetAbilityActive)
      (bind _asskeleton_bp (Utilities|Casting|CastToSkeleton_BP OtherActor))
      (Variables|Default|SetDamageAdd (* (Variables|/Game/Characters/AbstractCharacter.AbstractCharacter_C|GetDamage _asskeleton_bp) _percentincrease))
      (Variables|Default|SetPhyResistAdd (* _percentincrease (Variables|/Game/Characters/AbstractCharacter.AbstractCharacter_C|GetPhysicalResist _asskeleton_bp)))
      (Default|BattleRage _asskeleton_bp (Variables|Default|GetDamageAdd) (Variables|Default|GetPhyResistAdd)))))

(event OnComponentEndOverlap(AuraBox)
  (params (OverlappedComponent :type Primitive%20Component%20Object%20Reference) (OtherActor :type Actor%20Object%20Reference) (OtherComp :type Primitive%20Component%20Object%20Reference) (OtherBodyIndex :type Integer))
  (if (Variables|Default|GetAbilityActive)
    (bind _asskeleton_bp (Utilities|Casting|CastToSkeleton_BP OtherActor))
    (Default|RemoveBattleRage _asskeleton_bp (Variables|Default|GetDamageAdd) (Variables|Default|GetPhyResistAdd))))

(event OnComponentBeginOverlap(AuraSphere)
  (params (OverlappedComponent :type Primitive%20Component%20Object%20Reference) (OtherActor :type Actor%20Object%20Reference) (OtherComp :type Primitive%20Component%20Object%20Reference) (OtherBodyIndex :type Integer) (bFromSweep :type Boolean) (SweepResult :type Hit%20Result%20Structure%20%28by%20ref%29)))

(event OnComponentEndOverlap(AuraSphere)
  (params (OverlappedComponent :type Primitive%20Component%20Object%20Reference) (OtherActor :type Actor%20Object%20Reference) (OtherComp :type Primitive%20Component%20Object%20Reference) (OtherBodyIndex :type Integer)))

(event OnComponentBeginOverlap(CounterBox)
  (params (OverlappedComponent :type Primitive%20Component%20Object%20Reference) (OtherActor :type Actor%20Object%20Reference) (OtherComp :type Primitive%20Component%20Object%20Reference) (OtherBodyIndex :type Integer) (bFromSweep :type Boolean) (SweepResult :type Hit%20Result%20Structure%20%28by%20ref%29))
  (if (not (CallFunction|IsDead))
    (if (not (Variables|Default|GetAbilityActive))
      (Utilities|Casting|CastToSkeleton_BP OtherActor)
      (Math|Integer|IncrementInt (Variables|Default|GetCloseSkeletons)))))

(event OnComponentEndOverlap(CounterBox)
  (params (OverlappedComponent :type Primitive%20Component%20Object%20Reference) (OtherActor :type Actor%20Object%20Reference) (OtherComp :type Primitive%20Component%20Object%20Reference) (OtherBodyIndex :type Integer))
  (if (not (CallFunction|IsDead))
    (if (not (Variables|Default|GetAbilityActive))
      (Utilities|Casting|CastToSkeleton_BP OtherActor)
      (Math|Integer|DecrementInt (Variables|Default|GetCloseSkeletons)))))

(event Custom|ActivateAbility
  (bind _self self)
  (bind _percentincrease (Variables|Default|GetPercentIncrease))
  (bind _returnvalue (AI|GetAIController _self))
  (bind _braincomponent (Variables|/Script/AIModule.AIController|GetBrainComponent _returnvalue))
  (Variables|Default|SetAbilityActive true)
  (Variables|/Script/Engine.CharacterMovementComponent|SetMaxWalkSpeed (Variables|Character|GetCharacterMovement) 0.0)
  (AI|Logic|StopLogic _braincomponent "")
  (Animation|PlayAnimMontage "/Game/Characters/NPC/EnemyCharacter/Skeleton_Warrior/Skeleton_Warrior_BattleCry_Montage.Skeleton_Warrior_BattleCry_Montage" 2.0 "None")
  (Utilities|FlowControl|Delay 1.8)
  (Class|BrainComponent|RestartLogic _braincomponent)
  (Variables|/Script/Engine.CharacterMovementComponent|SetMaxWalkSpeed (Variables|Character|GetCharacterMovement) 3.5e+02)
  (CallFunction|BattleRage (* (Variables|Default|GetDamage) _percentincrease) (* _percentincrease (Variables|Default|GetPhysicalResist)))
  (Components|Box|SetBoxExtent (Variables|Default|GetAuraBox) "500.000000,500.000000,10.000000" true)
  (if (not (CallFunction|IsDead))
    (Utilities|Time|SetTimerbyEvent (delegate Custom|BattlePing) 1.0 true)))

(event Custom|BattlePing
  (bind _battleping1 (Variables|Default|GetBattlePing1))
  (bind _battleping1_2 (Variables|Default|GetBattlePing1))
  (bind _battleping1_3 (Variables|Default|GetBattlePing1))
  (bind _aurabox (Variables|Default|GetAuraBox))
  (if (CallFunction|IsDead)
    (Timeline|ShrinkDelete PlayFromStart
      (:Update
        (Utilities|IsValid _aurabox
          (:Is%20Valid
            (Transformation|SetRelativeScale3D _aurabox "0, 0, 0"))))
      (:Finished
        (Utilities|IsValid _aurabox
          (:Is%20Valid
            (Components|DestroyComponent _aurabox)))))
    (else
      (Transformation|SetRelativeScale3D _battleping1 "1.000000,1.000000,1.000000")
      (Rendering|SetVisibility _battleping1 true false)
      (bind (_direction _wavegrow _opacityfade) (Timeline|Timeline_PingWave PlayFromStart)
        (:Update
          (Transformation|SetRelativeScale3D _battleping1_2 (Math|Vector|MakeVector (* _wavegrow 12.0) (* _wavegrow 12.0) (* _wavegrow 12.0)))
          (Rendering|Material|SetScalarParameterValueonMaterials _battleping1_2 "Opacity" _opacityfade))
        (:Finished
          (Rendering|SetVisibility _battleping1_3 false false)
          (Rendering|Material|SetScalarParameterValueonMaterials _battleping1_3 "Opacity" 1.0))))))

(event EventBeginPlay
  (|CallParentFunction)
  (CallFunction|CreateWeapon)
  (Rendering|SetVisibility (Variables|Default|GetBlockedWidget) false false)
  (Rendering|SetVisibility (Variables|Default|GetBattlePing1) false false))

(event Collision|EventActorBeginOverlap
  (params (OtherActor :type Actor%20Object%20Reference))
  (|CallParentFunction OtherActor) ; This node is disabled and will not be called.\nDrag off pins to build functionality.
)

(event EventTick
  (params (DeltaSeconds :type Float%20%28single-precision%29))
  (|CallParentFunction DeltaSeconds)
  (if (not (Variables|Default|GetAbilityActive))
    (if (<= (Variables|Default|GetHealth) (/ (Variables|Default|GetMaxHealth) 2.0))
      (CallFunction|ActivateAbility :!label _label)
      (elif (>= (Variables|Default|GetCloseSkeletons) 6)
        (goto _label)))))

(event EventCreateWeapon
  (bind _returnvalue (Math|Random|RandomIntegerinRange 0 100))
  (Utilities|FlowControl|Sequence
    (:then_0
      (bind _returnvalue_2 (Game|SpawnActorfromClass "/Game/Items/Sword/Sword1_BP.Sword1_BP_C" (Transformation|GetActorTransform) "Undefined" 0 self))
      (Variables|Default|SetWeapon _returnvalue_2)
      (Variables|/Game/Items/ItemBP.ItemBP_C|SetHolder _returnvalue_2 self)
      (Variables|/Game/Items/ItemBP.ItemBP_C|SetHolderTeam _returnvalue_2 (Variables|Default|GetTeamNumber))
      (Transformation|AttachComponentToComponent _returnvalue_2 (Variables|Character|GetMesh) "WeaponSocket" "SnapToTarget" "SnapToTarget" "SnapToTarget" false)
      (Utilities|Array|Add (Variables|Default|GetItemsArr) _returnvalue_2))
    (:then_1
      (bind _returnvalue_3 (Game|SpawnActorfromClass "/Game/Items/Shield/RoundShield_BP.RoundShield_BP_C" (Transformation|GetActorTransform) "Undefined" 0 self))
      (Utilities|Array|Add (Variables|Default|GetItemsArr) _returnvalue_3)
      (Transformation|AttachComponentToComponent _returnvalue_3 (Variables|Character|GetMesh) "ShieldSocket" "SnapToTarget" "SnapToTarget" "SnapToTarget" false))
    (:then_2
      (if (== (Math|Integer|%(Integer) _returnvalue 10) 0)
        (bind _returnvalue_4 (Game|SpawnActorfromClass "/Game/Items/Helmet/Skeleton_Helmet_BP.Skeleton_Helmet_BP_C" (Transformation|GetActorTransform) "Undefined" 0 self :!label _label))
        (Transformation|AttachComponentToComponent _returnvalue_4 (Variables|Character|GetMesh) "HelmetSocket" "SnapToTarget" "SnapToTarget" "SnapToTarget" false)
        (Utilities|Array|Add (Variables|Default|GetItemsArr) _returnvalue_4)
        (elif (>= _returnvalue 80)
          (goto _label)
          (elif (<= _returnvalue 20)
            (goto _label)))))))

(event EventPlayDead
  (for _array_element (Variables|Default|GetItemsArr)
    (Actor|DestroyActor _array_element))
  (|CallParentFunction))

(event Game|Damage|EventAnyDamage
  (params (Damage :type Float%20%28single-precision%29) (DamageType :type Damage%20Type%20Object%20Reference) (InstigatedBy :type Controller%20Object%20Reference) (DamageCauser :type Actor%20Object%20Reference))
  (bind _blockedwidget (Variables|Default|GetBlockedWidget))
  (if (not (CallFunction|IsDead))
    (Utilities|Casting|CastToActivateAbleProps DamageCauser ; Prevent blicking traps
      (:then
        (|CallParentFunction Damage DamageType InstigatedBy DamageCauser :!label _label))
      (:CastFailed
        (Utilities|Casting|CastToDamageType_Physical DamageType
          (:then
            (bind _block (CallFunction|BlockChance))
            (if _block
              (Animation|PlayAnimMontage "/Game/Characters/NPC/EnemyCharacter/Skeleton_Warrior/Skeleton_Warrior_Block_Hit_Montage.Skeleton_Warrior_Block_Hit_Montage" 3.0 "None")
              (Rendering|SetVisibility _blockedwidget true false)
              (bind _textlift (Timeline|Timeline_BlockedText PlayFromStart)
                (:Update
                  (Transformation|SetRelativeLocation _blockedwidget (Math|Vector|MakeVector 0.0 0.0 (+ (* _textlift 1e+02) 2e+02)) false false)
                  (Transformation|SetWorldRotation _blockedwidget "45.000000,-180.000000, 0" false false)
                  (Transformation|SetRelativeScale3D _blockedwidget (Math|Vector|MakeVector (+ _textlift 1.2) (+ _textlift 1.2) (+ _textlift 1.2))))
                (:Finished
                  (Rendering|SetVisibility _blockedwidget false false)))
              (else
                (goto _label))))
          (:CastFailed
            (goto _label)))))))

(fn ConstructionScript
  (|CallParentFunction)
  (Utilities|FlowControl|Sequence
    (:then_0
      (bind _output_get (Variables|Default|SetHealth 1e+02))
      (Variables|Default|SetMaxHealth _output_get))
    (:then_1
      (Variables|Default|SetDamage 12.0))
    (:then_2
      (Variables|Default|SetPhysicalResist 0.2))
    (:then_3
      (Variables|Default|SetMagicalResist 0.0))
    (:then_4
      (Variables|Default|SetMovementSpeed 3.5e+02))
    (:then_5
      (Variables|Default|SetXPGain 80))
    (:then_6
      (Variables|Default|SetisLarge false))
    (:then_7
      (Variables|Default|SetTeamNumber 2))))

(fn BlockChance
  (return (== (Math|Integer|%(Integer) (Math|Random|RandomIntegerinRange 0 100) 5) 0)))