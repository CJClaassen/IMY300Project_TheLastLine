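; Wave spawner that fills an enemy or unit wave up to a total health budget, through a SpawnWave function called from outside.
; It repeatedly loops over unit types, filtering by a seeded-stream probability roll and each type's minimum wave level.
; Candidates spawn with their behavior trees at a fixed location, then either deduct their Health from the budget or are destroyed if too costly.
; It returns the spawned unit count once the budget is exhausted.
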(event EventBeginPlay)

(event Collision|EventActorBeginOverlap
  (params (OtherActor :type Actor%20Object%20Reference)))

(event EventTick
  (params (DeltaSeconds :type Float%20%28single-precision%29)))

(fn ConstructionScript)

(fn SpawnWave
  (params (typeOfUnits :type Array%20of%20Abstract%20Character%20Class%20References) (ProbabilityOfUnits :type Array%20of%20Floats%20%28single-precision%29) (MaximumHealth :type Float%20%28single-precision%29) (CurrentWave :type Integer) (UnitBehaviourtree :type Array%20of%20Behavior%20Tree%20Object%20References))
  (LocalVariables|Set_TypeOfUnits typeOfUnits)
  (LocalVariables|Set_ProbabilityOfUnits ProbabilityOfUnits)
  (LocalVariables|Set_CurrentWave CurrentWave)
  (LocalVariables|SetMaxHealth MaximumHealth)
  (LocalVariables|SetBehaviourTrees UnitBehaviourtree)
  (while (> (LocalVariables|GetMaxHealth) 0.0)
    (for (_array_element _array_index) (Variables|Default|GetUnitLevel)
      (if (>= (Utilities|Array|Get(acopy) (LocalVariables|Get_ProbabilityOfUnits) _array_index) (Math|Random|RandomFloatinRangefromStream 0.0 1e+02 (Math|Random|MakeRandomStream 0)))
        (if (<= _array_element (LocalVariables|Get_CurrentWave))
          (bind _returnvalue (AI|SpawnAIFromClass (Utilities|Array|Get(acopy) (LocalVariables|Get_TypeOfUnits) _array_index) (Utilities|Array|Get(acopy) (LocalVariables|GetBehaviourTrees) _array_index) "0, 0,500.000000" "0.000000, 0, 0" false))
          (bind _asabstract_character (Utilities|Casting|CastToAbstractCharacter _returnvalue))
          (if (>= (LocalVariables|GetMaxHealth) (Variables|/Game/Characters/AbstractCharacter.AbstractCharacter_C|GetHealth _asabstract_character))
            (Math|Integer|IncrementInt (LocalVariables|GetNumberOfUnitsSpawned)
              (:%20%20
                (LocalVariables|SetMaxHealth (- (LocalVariables|GetMaxHealth) (Variables|/Game/Characters/AbstractCharacter.AbstractCharacter_C|GetHealth _asabstract_character)))))
            (else
              (Actor|DestroyActor _asabstract_character)))))))
  (return (LocalVariables|GetNumberOfUnitsSpawned)))