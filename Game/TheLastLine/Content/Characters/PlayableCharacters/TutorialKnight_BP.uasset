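; Tutorial variant of the playable knight that reports player actions to a TutorialHandler to drive tutorial progression.
; Overrides gate abilities, attack and block behind disable flags, with combat also requiring picked-up sword and shield, before calling the parent.
; Ability use, damage, blocks, ability readiness and timer-polled prop proximity notify the handler.
; BeginPlay skips the parent's, doing its own setup and helmet spawn; death before wave 2 refills health.
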(event Custom|SetHandler
  (params (Handler :type Tutorial%20Map%20Handler%20Object%20Reference))
  (Variables|Default|SetTutorialHandler Handler))

(event Custom|CreateTriggerSphere
  (bind _returnvalue (Utilities|Time|SetTimerbyEvent (delegate Custom|CheckDistance) 0.1 true))
  (Variables|Default|SetTimer _returnvalue))

(event Custom|CheckDistance
  (bind _outactors (Actor|GetAllActorsOfClass "/Game/Traps/ActivateAbleProps.ActivateAbleProps_C"))
  (if (<= (Transformation|GetDistanceTo (Utilities|Array|Get(acopy) _outactors)) 3e+02)
    (Utilities|Time|ClearandInvalidateTimerbyHandle (Variables|Default|GetTimer))
    (Default|UpdateNextWave (Variables|Default|GetTutorialHandler) 1e+01)))

(event EventPlayDead
  (bind _astop_down_game_mode (Utilities|Casting|CastToTopDownGameMode (Game|GetGameMode)))
  (if (< (Variables|/Game/Maps/MapHandler_BP.MapHandler_BP_C|GetCurrentWave (Variables|/Game/GameData/GameModes/TopDownGameMode.TopDownGameMode_C|GetMapHandler _astop_down_game_mode)) 2)
    (Variables|Default|SetHealth (Variables|Default|GetMaxHealth))
    (else
      (bind _ascustom_player_controller_bp (Utilities|Casting|CastToCustomPlayerController_BP (Pawn|GetController)))
      (Input|SetInputModeUIOnly _ascustom_player_controller_bp 0 "DoNotLock"))))

(event EventAbilityE
  ;[1 1 1] Ability E
  (if (not (Utilities|Array|Get(acopy) (Variables|Default|GetAbilityCastingDisabled) 1))
    (if (Utilities|Array|Get(acopy) (Variables|Default|GetAbilityTutorialUpdate) 1)
      (Default|UpdateNextWave (Variables|Default|GetTutorialHandler) 1e+01))
    (|CallParentFunction)))

(event Game|Damage|EventAnyDamage
  (params (Damage :type Float%20%28single-precision%29) (DamageType :type Damage%20Type%20Object%20Reference) (InstigatedBy :type Controller%20Object%20Reference) (DamageCauser :type Actor%20Object%20Reference))
  (bind _tutorialhandler (Variables|Default|GetTutorialHandler))
  (|CallParentFunction Damage DamageType InstigatedBy DamageCauser)
  (if (Variables|Default|GetisBlocking)
    (Default|UpdateonBlock _tutorialhandler)
    (else
      (Development|PrintString "Received Damage")
      (Default|OnReceiveDamage _tutorialhandler))))

(event EventTick
  (params (DeltaSeconds :type Float%20%28single-precision%29))
  (bind _abilityslots (Variables|Default|GetAbilitySlots))
  (bind _abilityslots_2 (Variables|Default|GetAbilitySlots))
  (bind _abilityslots_3 (Variables|Default|GetAbilitySlots))
  (bind _output (Utilities|Array|Get(acopy) _abilityslots_2))
  (bind _output_2 (Utilities|Array|Get(acopy) _abilityslots 2))
  (bind _output_3 (Utilities|Array|Get(acopy) _abilityslots_3 1))
  (|CallParentFunction DeltaSeconds)
  (Utilities|IsValid _output
    (:Is%20Valid
      (if (and (Utilities|Array|Get(acopy) (Variables|Default|GetNotifyOnAbilityReady)) (Default|IsReady _output))
        (Default|NotifyonAbilityonReady (Variables|Default|GetTutorialHandler))
        (Utilities|Array|SetArrayElem (Variables|Default|GetNotifyOnAbilityReady) 0 false)
        (else
          (Utilities|IsValid _output_3 :!label _label
            (:Is%20Valid
              (if (and (Utilities|Array|Get(acopy) (Variables|Default|GetNotifyOnAbilityReady) 1) (Default|IsReady _output_3))
                (Default|NotifyonAbilityonReady (Variables|Default|GetTutorialHandler) 1)
                (Utilities|Array|SetArrayElem (Variables|Default|GetNotifyOnAbilityReady) 1 false)
                (else
                  (Utilities|IsValid _output_2 :!label _label_2
                    (:Is%20Valid
                      (if (and (Utilities|Array|Get(acopy) (Variables|Default|GetNotifyOnAbilityReady) 2) (Default|IsReady _output_2))
                        (Default|NotifyonAbilityonReady (Variables|Default|GetTutorialHandler) 2)
                        (Utilities|Array|SetArrayElem (Variables|Default|GetNotifyOnAbilityReady) 2 false)))))))
            (:Is%20Not%20Valid
              (goto _label_2))))))
    (:Is%20Not%20Valid
      (goto _label))))

(event EventUpdateSkillMenuTutorial
  (|CallParentFunction)
  (Default|UpdateNextWave (Variables|Default|GetTutorialHandler) 1e+01))

(event EventTryBasicAttack
  (if (and (Variables|Default|GetItemsPickupUp) (not (Variables|Default|GetAttackDisabled)))
    (|CallParentFunction)
    (else
      (Default|TrytoAttack (Variables|Default|GetTutorialHandler)))))

(event EventAbilityQ
  ;[1 1 1] Ability Q
  (if (not (Utilities|Array|Get(acopy) (Variables|Default|GetAbilityCastingDisabled)))
    (if (Utilities|Array|Get(acopy) (Variables|Default|GetAbilityTutorialUpdate))
      (Default|UpdateNextWave (Variables|Default|GetTutorialHandler) 1e+01))
    (|CallParentFunction)))

(event EventUpdateDisplay
  (params (PlayerController :type Custom%20Player%20Controller%20BP%20Object%20Reference))
  (|CallParentFunction PlayerController))

(event EventAbilityR
  ;[1 1 1] Ability R
  (if (not (Utilities|Array|Get(acopy) (Variables|Default|GetAbilityCastingDisabled) 2))
    (if (Utilities|Array|Get(acopy) (Variables|Default|GetAbilityTutorialUpdate) 2)
      (Default|UpdateNextWave (Variables|Default|GetTutorialHandler) 1e+01))
    (|CallParentFunction)))

(event EventReleaseBlock
  (if (and (Variables|Default|GetItemsPickupUp) (not (Variables|Default|GetBlockDisabled)))
    (|CallParentFunction)))

(event EventTryBlock
  (if (and (Variables|Default|GetItemsPickupUp) (not (Variables|Default|GetBlockDisabled)))
    (|CallParentFunction)))

(event EventUpdateHealthBarDisplay
  (|CallParentFunction))

(event EventBeginPlay
  (for (_ _array_index) (Variables|Default|GetSlotLevels)
    (Utilities|Array|SetArrayElem (Variables|Default|GetSlotLevels) _array_index 1))
  (CallFunction|AddPlayerHelmet)
  (Variables|Default|SetPoints 0)
  (CallFunction|InitializePlayerStartingAttributes)
  (bind _outactors (Actor|GetAllActorsOfClass "/Game/Items/Helmet/HelmetItem.HelmetItem_C"))
  (for _array_element _outactors
    (if (not (== _array_element (Variables|Default|GetHelmet)))
      (Actor|DestroyActor _array_element))))

(fn ConstructionScript
  (|CallParentFunction)
  (for (_ _array_index) (Variables|Default|GetSlotLevels)
    (Utilities|Array|SetArrayElem (Variables|Default|GetSlotLevels) _array_index 0)
    (CallFunction|UpdateAbilitySlot _array_index 0.0)))

(fn SetAbility
  (params (AbilityType :type Cast%20Abilities%20BP%20Class%20Reference))
  (bind _objectivestruct (Utilities|Struct|MakeObjectiveStruct "None"))
  (bind _tutorialhandler (Variables|Default|GetTutorialHandler))
  (bind _indexassigned (|CallParentFunction AbilityType))
  (if (!= _indexassigned -1)
    (if (not (Variables|Default|GetHasPromptedSwap))
      (bind _loaded (CallFunction|CountLoadedAbilities))
      (if (== _loaded 2)
        (Default|UpdateObjective _tutorialhandler false _objectivestruct)
        (Variables|Default|SetHasPromptedSwap true)
        (else
          (Default|UpdateObjective _tutorialhandler false _objectivestruct :!label _label)))
      (else
        (goto _label)))
    (else
      (Default|UpdateObjective (Variables|Default|GetTutorialHandler) false _objectivestruct)))
  (return _indexassigned))

(fn GetAbilitybyName
  (params (AbilityName :type String))
  (bind (_array_element _array_index) (Utilities|Array|ForEachLoopwithBreak (Variables|Default|GetAbilitySlots) :!label _label)
    (:LoopBody
      (if (Utilities|Enum|Equal(Enum) (Variables|/Game/Abilities/CastAbilities/CastAbilities_BP.CastAbilities_BP_C|GetAbilityName _array_element) AbilityName)
        (LocalVariables|SetIndex _array_index)
        (goto _label Break)))
    (:Completed
      (return (LocalVariables|GetIndex)))))

(fn CountLoadedAbilities
  (for _array_element (Variables|Default|GetAbilitySlots)
    (Utilities|IsValid _array_element
      (:Is%20Valid
        (Math|Integer|IncrementInt (LocalVariables|GetAbilities)))))
  (return (LocalVariables|GetAbilities)))

(fn AddPlayerHelmet
  (bind _returnvalue (Transformation|GetActorTransform))
  (bind _returnvalue_2 (Game|SpawnActorfromClass "/Game/Items/Helmet/HelmetItem.HelmetItem_C" (Math|Transform|MakeTransform (.location _returnvalue) (.rotation _returnvalue) (.scale _returnvalue)) "Undefined" 0 0))
  (Variables|Default|SetHelmet _returnvalue_2)
  (Utilities|IsValid _returnvalue_2
    (:Is%20Valid
      (Transformation|AttachComponentToComponent _returnvalue_2 (Variables|Character|GetMesh) "HeadSocket" "SnapToTarget" "SnapToTarget" "KeepWorld" false))))

(fn PickUpItems
  (params (Items :type Array%20of%20Item%20BP%20Object%20References) (addToList :type Boolean))
  (Variables|Default|SetItemsPickupUp true)
  (if addToList
    (for _array_element Items
      (bind _astower_shield_bp (Utilities|Casting|CastToTowerShield_BP _array_element)
        (:then
          (bind _output_get (Variables|Default|SetShield _astower_shield_bp))
          (Transformation|AttachComponentToComponent _output_get (Variables|Character|GetMesh) "ShieldSocket" "SnapToTarget" "SnapToTarget" "KeepWorld" false)
          (Development|PrintString "Set Shield"))
        (:CastFailed
          (bind _assword_1_bp (Utilities|Casting|CastToSword1_BP _array_element))
          (bind _output_get_2 (Variables|Default|SetSword _assword_1_bp))
          (Variables|/Game/Items/Sword/Sword1_BP.Sword1_BP_C|SetHolder _output_get_2 self)
          (Transformation|AttachComponentToComponent _output_get_2 (Variables|Character|GetMesh) "WeaponSocket" "SnapToTarget" "SnapToTarget" "KeepWorld" false)
          (Development|PrintString "Set Sword")))))
  (Variables|Default|SetItemsPickupUp true))

(fn IndicateRange
  (params (range :type Float%20%28single-precision%29))
  (bind _sphere (Variables|Default|GetSphere))
  (bind _staticmesh (Variables|Default|GetStaticMesh))
  (bind _returnvalue (Transformation|GetWorldScale _staticmesh))
  (bind _sphereradius (Variables|/Script/Engine.SphereComponent|GetSphereRadius _sphere))
  (bind _returnvalue_2 (/ range _sphereradius))
  (Transformation|SetWorldScale3D _staticmesh (Math|Vector|MakeVector (* (.x _returnvalue) _returnvalue_2) (* (.y _returnvalue) _returnvalue_2) (* (.z _returnvalue) _returnvalue_2)))
  (Components|Sphere|SetSphereRadius (Variables|Default|GetSphere) range false)
  (Rendering|Material|SetMaterial (Variables|Default|GetStaticMesh) 0 "/Game/GameData/VisualProps/RadiusIndicator/MInstance_DamageIndicator.MInstance_DamageIndicator"))

(fn HideRadius
  (Rendering|Material|SetMaterial (Variables|Default|GetStaticMesh) 0 "/Game/UI/Gameplay/M_Invisible.M_Invisible"))