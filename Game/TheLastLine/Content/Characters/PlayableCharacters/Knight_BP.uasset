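; Playable Knight character for a top-down game, spawning a sword, tower shield and helmet onto mesh sockets.
; Combat uses a section-chained combo montage and a block that negates frontal hits via a facing dot product.
; Three ability slots (Q/E/R) hold spawned ability actors that can be swapped, discarded and leveled by slot XP.
; Health, player XP, points and ability events are pushed to the gameplay HUD and player controller.
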(event Custom|CreateWeapons
  (bind _returnvalue (Transformation|GetActorTransform))
  (bind _returnvalue_2 (Transformation|GetActorTransform))
  (bind _returnvalue_3 (Transformation|GetActorTransform))
  (Utilities|FlowControl|Sequence
    (:then_0
      (bind _returnvalue_4 (Game|SpawnActorfromClass "/Game/Items/Sword/Sword1_BP.Sword1_BP_C" (Math|Transform|MakeTransform (.location _returnvalue_2) (.rotation _returnvalue_2) (* "1.000000,1.000000,1.000000" "0.200000,0.200000,0.200000")) "Undefined" 0 0))
      (Utilities|IsValid _returnvalue_4
        (:Is%20Valid
          (bind _output_get (Variables|Default|SetSword _returnvalue_4))
          (Variables|/Game/Items/Sword/Sword1_BP.Sword1_BP_C|SetHolder _output_get self)
          (Transformation|AttachComponentToComponent _returnvalue_4 (Variables|Character|GetMesh) "WeaponSocket" "SnapToTarget" "SnapToTarget" "KeepWorld" false))))
    (:then_1
      (bind _returnvalue_5 (Game|SpawnActorfromClass "/Game/Items/Shield/TowerShield_BP.TowerShield_BP_C" (Math|Transform|MakeTransform (.location _returnvalue_3) (.rotation _returnvalue_3) (* "1.000000,1.000000,1.000000" "0.200000,0.200000,0.200000")) "AlwaysSpawn" 0 0))
      (Utilities|IsValid _returnvalue_5
        (:Is%20Valid
          (bind _output_get_2 (Variables|Default|SetShield _returnvalue_5))
          (Transformation|AttachComponentToComponent _output_get_2 (Variables|Character|GetMesh) "ShieldSocket" "SnapToTarget" "SnapToTarget" "KeepWorld" false))))
    (:then_2
      (bind _returnvalue_6 (Game|SpawnActorfromClass "/Game/Items/Helmet/HelmetItem.HelmetItem_C" (Math|Transform|MakeTransform (.location _returnvalue) (.rotation _returnvalue) (.scale _returnvalue)) "Undefined" 0 0))
      (Utilities|IsValid _returnvalue_6
        (:Is%20Valid
          (Transformation|AttachComponentToComponent _returnvalue_6 (Variables|Character|GetMesh) "HeadSocket" "SnapToTarget" "SnapToTarget" "KeepWorld" false))))))

(event Custom|ReleaseBlock
  (bind _returnvalue (Actor|GetGameTimeSinceCreation))
  (Variables|Default|SetisBlocking false)
  (if (>= (- _returnvalue (Variables|Default|GettimeDeactivatedBlock)) 0.4)
    (Variables|Default|SettimeDeactivatedBlock _returnvalue)
    (Audio|PlaySoundatLocation "/Game/HumanVocalizations/HumanMaleB/Cues/voice_male_b_effort_quick_action_02_Cue.voice_male_b_effort_quick_action_02_Cue" (Transformation|GetActorLocation) "0, 0, 0" 0.6 1.0 0.0 0 "/Game/Characters/PlayableCharacters/Sound/PlayerDamageSound.PlayerDamageSound" 0)))

(event EventBeginPlay
  (|CallParentFunction)
  (CallFunction|CreateWeapons)
  (CallFunction|InitializePlayerStartingAttributes))

(event Collision|EventActorBeginOverlap
  (params (OtherActor :type Actor%20Object%20Reference))
  (|CallParentFunction OtherActor) ; This node is disabled and will not be called.\nDrag off pins to build functionality.
)

(event EventTick
  (params (DeltaSeconds :type Float%20%28single-precision%29))
  (bind _returnvalue (Game|GetPlayerController 0))
  (bind _hitresult (Game|Player|GetHitResultUnderCursorbyChannel _returnvalue "TraceTypeQuery1" true))
  (bind (_bblockinghit _binitialoverlap _time _distance _location _impactpoint _normal _impactnormal) (Collision|BreakHitResult _hitresult))
  (Transformation|SetWorldLocationAndRotation (Variables|Default|GetCursorToWorld) _location (Math|Rotator|MakeRotationfromAxes _impactnormal "0, 0, 0" "0, 0, 0") false false)
  (if (CallFunction|IsDead)
    ;[1 1 1] Handling Character Death
    (CallFunction|DisableCharacterInput)
    (Animation|PlayAnimMontage 0 1.0 "None")
    (else
      (CallFunction|GetCalculatedDamage))))

(event EventPossessed
  (params (NewController :type Controller%20Object%20Reference))
  (bind _ascustom_player_controller_bp (Utilities|Casting|CastToCustomPlayerController_BP NewController))
  (CallFunction|UpdateDisplay _ascustom_player_controller_bp))

(event EventAbilityE
  (bind _abilityslots (Variables|Default|GetAbilitySlots))
  (bind _output (Utilities|Array|Get(acopy) _abilityslots 1))
  ;[1 1 1] Ability Trigger
  ;;[1 1 1] Check if slot Q is occupied
  (if (Utilities|Array|Get(acopy) (Variables|Default|GetAbilityOccupationSlots) 1)
    ;;[1 1 1] Activating the ability E
    (if (Default|IsReady (Utilities|Array|Get(acopy) (Variables|Default|GetAbilitySlots) 1))
      (Default|Activate _output (Transformation|GetActorLocation) (Variables|Default|GetActorRotation) (Variables|Default|GetplayerIndex) (Utilities|Array|Get(acopy) (Variables|Default|GetSlotLevels) 1))
      (bind _ascustom_player_controller_bp (Utilities|Casting|CastToCustomPlayerController_BP (Pawn|GetController)))
      (Default|NotifyonAbilityCast _ascustom_player_controller_bp _output 1)
      (else
        (Development|PrintString "Still in cooldown")))))

(event EventAbilityR
  (bind _abilityslots (Variables|Default|GetAbilitySlots))
  (bind _output (Utilities|Array|Get(acopy) _abilityslots 2))
  ;[1 1 1] Ability Trigger
  ;;[1 1 1] Check if slot Q is occupied
  (if (Utilities|Array|Get(acopy) (Variables|Default|GetAbilityOccupationSlots) 2)
    ;;[1 1 1] Activating the ability E
    (if (Default|IsReady (Utilities|Array|Get(acopy) (Variables|Default|GetAbilitySlots) 2))
      (Default|Activate _output (Transformation|GetActorLocation) (Variables|Default|GetActorRotation) (Variables|Default|GetplayerIndex) (Utilities|Array|Get(acopy) (Variables|Default|GetSlotLevels) 2))
      (bind _ascustom_player_controller_bp (Utilities|Casting|CastToCustomPlayerController_BP (Pawn|GetController)))
      (Default|NotifyonAbilityCast _ascustom_player_controller_bp _output 2)
      (else
        (Development|PrintString "Still in cooldown")))))

(event EventAbilityQ
  (bind _abilityslots (Variables|Default|GetAbilitySlots))
  (bind _output (Utilities|Array|Get(acopy) _abilityslots))
  ;[1 1 1] Ability Trigger
  ;;[1 1 1] Check if slot Q is occupied
  (if (Utilities|Array|Get(acopy) (Variables|Default|GetAbilityOccupationSlots))
    ;;[1 1 1] Activating the ability Q
    (if (Default|IsReady (Utilities|Array|Get(acopy) (Variables|Default|GetAbilitySlots)))
      (Default|Activate _output (Transformation|GetActorLocation) (Variables|Default|GetActorRotation) (Variables|Default|GetplayerIndex) (Utilities|Array|Get(acopy) (Variables|Default|GetSlotLevels)))
      (bind _ascustom_player_controller_bp (Utilities|Casting|CastToCustomPlayerController_BP (Pawn|GetController)))
      (Default|NotifyonAbilityCast _ascustom_player_controller_bp _output))))

(event Game|Damage|EventAnyDamage
  (params (Damage :type Float%20%28single-precision%29) (DamageType :type Damage%20Type%20Object%20Reference) (InstigatedBy :type Controller%20Object%20Reference) (DamageCauser :type Actor%20Object%20Reference))
  (if (and (Variables|Default|GetisBlocking) (CallFunction|CanDoDamage (Transformation|GetActorForwardVector (Pawn|GetControlledPawn InstigatedBy))))
    (Audio|PlaySound2D "/Game/Characters/PlayableCharacters/Sound/Knight_shield_hit.Knight_shield_hit" (Variables|/Game/GameData/GameModes/TopDownGameMode.TopDownGameMode_C|GetVolumeMultiplier (Variables|Default|GetGameMode)) 1.0 0.0 "/Game/Characters/PlayableCharacters/Sound/PlayerItemSound.PlayerItemSound" 0)
    (Animation|PlayAnimMontage "/Game/Characters/PlayableCharacters/NewAssets/Animations/Impact/ImpactWBlocking_Montage.ImpactWBlocking_Montage" 1.0 "None")
    (else
      (|CallParentFunction Damage DamageType InstigatedBy DamageCauser)
      (CallFunction|UpdateHealthBarDisplay)
      (if (CallFunction|IsDead)
        (if (not (Variables|Default|Getbranch%20hasplayed))
          (Audio|PlaySoundatLocation 0 "0, 0, 0" "0, 0, 0" 1.0 1.0 0.0 0 0 0))
        (else
          (Animation|PlayAnimMontage "/Game/Characters/PlayableCharacters/NewAssets/Animations/Impact/ImpactNoBlocking_Montage.ImpactNoBlocking_Montage" 1.0 "None")
          (switch int (Math|Random|RandomIntegerinRange 0 5)
            (:0
              (Audio|PlaySoundatLocation "/Game/HumanVocalizations/HumanMaleC/Cues/voice_male_c_hurt_pain_03_Cue.voice_male_c_hurt_pain_03_Cue" (Transformation|GetActorLocation) "0, 0, 0" (Variables|/Game/GameData/GameModes/TopDownGameMode.TopDownGameMode_C|GetVolumeMultiplier (Variables|Default|GetGameMode)) 1.0 0.0 0 "/Game/Characters/PlayableCharacters/Sound/PlayerDamageSound.PlayerDamageSound" 0))
            (:1
              (Audio|PlaySoundatLocation "/Game/HumanVocalizations/HumanMaleC/Cues/voice_male_c_hurt_pain_04_Cue.voice_male_c_hurt_pain_04_Cue" (Transformation|GetActorLocation) "0, 0, 0" (Variables|/Game/GameData/GameModes/TopDownGameMode.TopDownGameMode_C|GetVolumeMultiplier (Variables|Default|GetGameMode)) 1.0 0.0 0 "/Game/Characters/PlayableCharacters/Sound/PlayerDamageSound.PlayerDamageSound" 0))
            (:2
              (Audio|PlaySoundatLocation "/Game/HumanVocalizations/HumanMaleC/Cues/voice_male_c_hurt_pain_05_Cue.voice_male_c_hurt_pain_05_Cue" (Transformation|GetActorLocation) "0, 0, 0" (Variables|/Game/GameData/GameModes/TopDownGameMode.TopDownGameMode_C|GetVolumeMultiplier (Variables|Default|GetGameMode)) 1.0 0.0 0 "/Game/Characters/PlayableCharacters/Sound/PlayerDamageSound.PlayerDamageSound" 0))
            (:3
              (Audio|PlaySoundatLocation "/Game/HumanVocalizations/HumanMaleC/Cues/voice_male_c_hurt_pain_06_Cue.voice_male_c_hurt_pain_06_Cue" (Transformation|GetActorLocation) "0, 0, 0" (Variables|/Game/GameData/GameModes/TopDownGameMode.TopDownGameMode_C|GetVolumeMultiplier (Variables|Default|GetGameMode)) 1.0 0.0 0 "/Game/Characters/PlayableCharacters/Sound/PlayerDamageSound.PlayerDamageSound" 0))
            (:4
              (Audio|PlaySoundatLocation "/Game/HumanVocalizations/HumanMaleC/Cues/voice_male_c_hurt_pain_07_Cue.voice_male_c_hurt_pain_07_Cue" (Transformation|GetActorLocation) "0, 0, 0" (Variables|/Game/GameData/GameModes/TopDownGameMode.TopDownGameMode_C|GetVolumeMultiplier (Variables|Default|GetGameMode)) 1.0 0.0 0 "/Game/Characters/PlayableCharacters/Sound/PlayerDamageSound.PlayerDamageSound" 0))
            (:5
              (Audio|PlaySoundatLocation "/Game/HumanVocalizations/HumanMaleC/Cues/voice_male_c_hurt_pain_08_Cue.voice_male_c_hurt_pain_08_Cue" (Transformation|GetActorLocation) "0, 0, 0" (Variables|/Game/GameData/GameModes/TopDownGameMode.TopDownGameMode_C|GetVolumeMultiplier (Variables|Default|GetGameMode)) 1.0 0.0 0 "/Game/Characters/PlayableCharacters/Sound/PlayerDamageSound.PlayerDamageSound" 0))))))))

(event EventTryBlock
  (bind _returnvalue (Transformation|GetActorLocation))
  (bind _returnvalue_2 (Actor|GetGameTimeSinceCreation))
  (Variables|Default|SetisBlocking true)
  (if (>= (- _returnvalue_2 (Variables|Default|GettimeActivatedBlock)) 0.4)
    (Variables|Default|SettimeActivatedBlock _returnvalue_2)
    (switch int (Math|Float|Truncate (Math|Float|%(Float) (* _returnvalue_2 1e+01) 2.0))
      (:0
        (Audio|PlaySoundatLocation "/Game/HumanVocalizations/HumanMaleB/Cues/voice_male_b_effort_jump_04_Cue.voice_male_b_effort_jump_04_Cue" _returnvalue "0, 0, 0" 0.6 1.0 0.0 0 "/Game/Characters/PlayableCharacters/Sound/PlayerDamageSound.PlayerDamageSound" 0))
      (:1
        (Audio|PlaySoundatLocation "/Game/HumanVocalizations/HumanMaleB/Cues/voice_male_b_effort_jump_05_Cue.voice_male_b_effort_jump_05_Cue" _returnvalue "0, 0, 0" 0.6 1.0 0.0 0 "/Game/Characters/PlayableCharacters/Sound/PlayerDamageSound.PlayerDamageSound" 0)))))

(event EventTryBasicAttack
  (bind _mesh (Variables|Character|GetMesh))
  (bind _returnvalue (Components|SkeletalMesh|GetAnimInstance _mesh))
  (bind _returnvalue_2 (Animation|Montage|MontageGetCurrentSection _returnvalue "/Game/Characters/PlayableCharacters/NewAssets/Animations/Attack/AttackCombo.AttackCombo"))
  (if (not (Variables|Default|GetisBlocking))
    (if (Class|AnimInstance|MontageIsActive _returnvalue "/Game/Characters/PlayableCharacters/NewAssets/Animations/Attack/AttackCombo.AttackCombo")
      (switch name _returnvalue_2
        (:Attack1End
          (Class|AnimInstance|MontageSetNextSection _returnvalue _returnvalue_2 "Attack2" "/Game/Characters/PlayableCharacters/NewAssets/Animations/Attack/AttackCombo.AttackCombo")))
      (else
        (Animation|PlayAnimMontage "/Game/Characters/PlayableCharacters/NewAssets/Animations/Attack/AttackCombo.AttackCombo" 1.5 "Attack1")))))

(fn ConstructionScript
  (bind _output_get (Variables|Default|SetHealth 1e+02))
  (Variables|Default|SetMaxHealth _output_get)
  (Variables|Default|SetDamage 2e+01)
  (Variables|Default|SetMagicalResist 0.1)
  (Variables|Default|SetPhysicalResist 0.1)
  (Variables|Default|SetMovementSpeed 5e+02)
  (Variables|Default|SetAttackSpeed 1.0)
  (Variables|Default|SetXPGain 0)
  (Variables|Default|SetisLarge false)
  (Variables|Default|SetTeamNumber 0)
  (CallFunction|ShiftCameratoDefault))

(fn SetAbility
  (params (AbilityType :type Cast%20Abilities%20BP%20Class%20Reference))
  (bind _openslot (CallFunction|GetFirstOpenAbilitySlot))
  (bind _output_get (LocalVariables|SetOpenSlot _openslot))
  (if (!= _output_get -1)
    (bind _output_get_2 (LocalVariables|SetAbility AbilityType))
    (bind _returnvalue (Game|SpawnActorfromClass _output_get_2 (Math|Transform|MakeTransform "0, 0, 0" "0, 0, 0" "1,1,1") "Undefined" 0 0))
    (Utilities|Array|SetArrayElem (Variables|Default|GetAbilitySlots) (LocalVariables|GetOpenSlot) _returnvalue)
    (Utilities|Array|SetArrayElem (Variables|Default|GetAbilityOccupationSlots) (LocalVariables|GetOpenSlot) true true)
    (Variables|/Game/Abilities/CastAbilities/CastAbilities_BP.CastAbilities_BP_C|SetAbilitySlotIndex _returnvalue (LocalVariables|GetOpenSlot))
    (if (>= (LocalVariables|GetOpenSlot) 0)
      (bind _astop_down_game_mode (Utilities|Casting|CastToTopDownGameMode (Game|GetGameMode)))
      (Audio|PlaySound2D "/Game/Sound/Knight/pickup/pickup.pickup" (Variables|/Game/GameData/GameModes/TopDownGameMode.TopDownGameMode_C|GetVolumeMultiplier _astop_down_game_mode) 1.0 0.0 0 0))
    (return (LocalVariables|GetOpenSlot))
    (else
      (return -1))))

(fn GetFirstOpenAbilitySlot
  (bind (_array_element _array_index) (Utilities|Array|ForEachLoopwithBreak (Variables|Default|GetAbilityOccupationSlots) :!label _label)
    (:LoopBody
      (if (not _array_element)
        (LocalVariables|SetopenIndex _array_index)
        (goto _label Break)))
    (:Completed
      (return (LocalVariables|GetopenIndex)))))

(fn SwapAbilities
  (params (Ability%20X :type Integer) (Ability%20Y :type Integer))
  (bind _abilityslots (Variables|Default|GetAbilitySlots))
  (bind _abilityslots_2 (Variables|Default|GetAbilitySlots))
  (bind _abilityslots_3 (Variables|Default|GetAbilitySlots))
  (bind _abilityslots_4 (Variables|Default|GetAbilitySlots))
  (bind _output (Utilities|Array|Get(acopy) _abilityslots_4 Ability%20Y))
  (bind _output_2 (Utilities|Array|Get(acopy) _abilityslots_2 Ability%20X))
  (bind _output_3 (Utilities|Array|Get(acopy) _abilityslots Ability%20Y))
  (bind _output_4 (Utilities|Array|Get(acopy) _abilityslots_3 Ability%20X))
  (Utilities|IsValid _output_4
    (:Is%20Valid
      (Utilities|IsValid _output_3
        (:Is%20Valid
          (if (and (Default|IsReady _output_4) (Default|IsReady _output_3))
            _
            (else
              (return false))))
        (:Is%20Not%20Valid
          (if (Default|IsReady _output_4)
            _
            (else
              (return false))))))
    (:Is%20Not%20Valid
      (Utilities|IsValid _output_3
        (:Is%20Valid
          (if (Default|IsReady _output_3)
            _
            (else
              (return false))))
        (:Is%20Not%20Valid
          (return false)))))
  (Utilities|Array|Swap (Variables|Default|GetAbilityOccupationSlots) Ability%20X Ability%20Y)
  (Utilities|Array|Swap (Variables|Default|GetAbilitySlots) Ability%20X Ability%20Y)
  ;[1 1 1] Handle avility X
  (Utilities|IsValid _output_2
    (:Is%20Valid
      (if (== (Variables|/Game/Abilities/CastAbilities/CastAbilities_BP.CastAbilities_BP_C|GetAbilitySlotIndex _output_2) Ability%20X)
        (Variables|/Game/Abilities/CastAbilities/CastAbilities_BP.CastAbilities_BP_C|SetAbilitySlotIndex _output_2 Ability%20Y)
        (else
          (Variables|/Game/Abilities/CastAbilities/CastAbilities_BP.CastAbilities_BP_C|SetAbilitySlotIndex _output_2 Ability%20X))))
    (:Is%20Not%20Valid
      _))
  ;[1 1 1] Handle ability Y
  (Utilities|IsValid _output
    (:Is%20Valid
      (if (== (Variables|/Game/Abilities/CastAbilities/CastAbilities_BP.CastAbilities_BP_C|GetAbilitySlotIndex _output) Ability%20Y)
        (Variables|/Game/Abilities/CastAbilities/CastAbilities_BP.CastAbilities_BP_C|SetAbilitySlotIndex _output Ability%20X)
        (else
          (Variables|/Game/Abilities/CastAbilities/CastAbilities_BP.CastAbilities_BP_C|SetAbilitySlotIndex _output Ability%20Y)
          (return true))))))

(fn DiscardAbility
  (params (AbilitySlotIndex :type Integer))
  (if (Utilities|Array|Get(acopy) (Variables|Default|GetAbilityOccupationSlots) AbilitySlotIndex)
    (Default|DestroySelf (Utilities|Array|Get(acopy) (Variables|Default|GetAbilitySlots) AbilitySlotIndex))
    (Utilities|Array|SetArrayElem (Variables|Default|GetAbilitySlots) AbilitySlotIndex 0)
    (Utilities|Array|SetArrayElem (Variables|Default|GetAbilityOccupationSlots) AbilitySlotIndex false)
    (else
      (bind _output_get (LocalVariables|Setdiscarded false))))
  (return _output_get))

(fn ShiftCameratoThirdPerson
  (bind _springarm (Variables|Default|GetSpringArm))
  (Variables|/Script/Engine.SpringArmComponent|SetTargetArmLength _springarm 3e+02)
  (Transformation|SetWorldLocationAndRotation _springarm (+ (Transformation|GetActorLocation) "1.500000,40.000000,50.000000") (Math|Rotator|MakeRotator 0.0 363.514435 0.0) false false))

(fn ShiftCameratoDefault
  (Variables|/Script/Engine.SpringArmComponent|SetTargetArmLength (Variables|Default|GetSpringArm) 1.2e+03)
  (Transformation|SetWorldRotation (Variables|Default|GetSpringArm) (Math|Rotator|MakeRotator 0.0 2.9e+02 0.0) false false)
  (Transformation|SetWorldLocation (Variables|Default|GetSpringArm) (Transformation|GetActorLocation) false false))

(fn UpdateAbilitySlot
  (params (SlotIndex :type Integer) (XpAmount :type Float%20%28single-precision%29))
  (bind _slotxp (Variables|Default|GetSlotXp))
  (bind _maxxp (Variables|Default|GetMaxXP))
  (bind _slotlevels (Variables|Default|GetSlotLevels))
  (bind _slotxp_2 (Variables|Default|GetSlotXp))
  (bind _output (Utilities|Array|Get(acopy) _slotlevels SlotIndex))
  (bind _output_2 (Utilities|Array|Get(acopy) _slotxp_2 SlotIndex))
  (Utilities|Array|SetArrayElem _slotxp SlotIndex (+ XpAmount (Utilities|Array|Get(acopy) _slotxp SlotIndex)))
  (if (>= _output_2 _maxxp)
    (Utilities|Array|SetArrayElem (Variables|Default|GetSlotXp) SlotIndex (- _output_2 _maxxp))
    (if (< _output (Variables|Default|GetMaxSlotLevel))
      (Math|Integer|IncrementInt _output
        (:%20%20
          (bind _ascustom_player_controller_bp (Utilities|Casting|CastToCustomPlayerController_BP (Pawn|GetController)))
          (Default|NotifyonAbilityLevelUp _ascustom_player_controller_bp SlotIndex (Utilities|Array|Get(acopy) (Variables|Default|GetSlotLevels) SlotIndex)))))))

(fn GetAbilitySlotDetails
  (params (SlotIndex :type Integer))
  (return (Utilities|Array|Get(acopy) (Variables|Default|GetAbilityOccupationSlots) SlotIndex) (Utilities|Array|Get(acopy) (Variables|Default|GetAbilitySlots) SlotIndex) (Utilities|Array|Get(acopy) (Variables|Default|GetSlotLevels) SlotIndex) (Utilities|Array|Get(acopy) (Variables|Default|GetSlotXp) SlotIndex)))

(fn OnCameraChange
  (params (VerticalArrowAction :type Integer) (HorizontalArrowAction :type Integer))
  (return true))

(fn UpdateDamage
  (params (PercentageDamageChange :type Float%20%28single-precision%29) (Duration :type Float%20%28single-precision%29))
  (if (== Duration 0.0)
    (Variables|Default|SetDamage (* (Variables|Default|GetDamage) PercentageDamageChange))
    (else
      (Variables|Default|SetDamageBoostDuration Duration)
      (Variables|Default|SetDamageBoost (* (Variables|Default|GetDamage) PercentageDamageChange))
      (Variables|Default|SetisBoosted true))))

(fn UpdateHealth
  (params (HealthIncrease :type Float%20%28single-precision%29) (IsPermanent :type Boolean))
  (if IsPermanent
    (Variables|Default|SetHealth (+ (Variables|Default|GetHealth) HealthIncrease))
    (Variables|Default|SetMaxHealth (+ (Variables|Default|GetMaxHealth) HealthIncrease))
    (else
      (bind _output_get (Variables|Default|SetHealth (+ (Variables|Default|GetHealth) HealthIncrease)))
      (if (> _output_get (Variables|Default|GetMaxHealth))
        (Variables|Default|SetHealth (Variables|Default|GetMaxHealth)))))
  (CallFunction|UpdateHealthBarDisplay))

(fn UpdatePlayerXP
  (params (XP%20Gain :type Float%20%28single-precision%29))
  (bind _output_get (Variables|Default|SetPlayerCurrent%20XP (+ XP%20Gain (Variables|Default|GetPlayerCurrent%20XP))))
  (if (< _output_get (Variables|Default|GetPlayer%20Max%20XP))
    _
    (else
      ;[1 1 1] Player leveled up
      (while (>= (Variables|Default|GetPlayerCurrent%20XP) (Variables|Default|GetPlayer%20Max%20XP))
        (Math|Integer|IncrementInt (Variables|Default|GetPlayerLevel)
          (:%20%20
            (Variables|Default|SetPlayerCurrent%20XP (- (Variables|Default|GetPlayerCurrent%20XP) (Variables|Default|GetPlayer%20Max%20XP)))
            (Variables|Default|SetPlayer%20Max%20XP (+ (Variables|Default|GetPlayer%20Max%20XP) 1e+02))
            (CallFunction|UpdateXPDisplay false))))))
  (CallFunction|UpdateXPDisplay false))

(fn GetCalculatedDamage
  (bind _damage (|CallParentFunction))
  (return _damage))

(fn UpdateDisplay
  (params (PlayerController :type Custom%20Player%20Controller%20BP%20Object%20Reference))
  (bind _asuser_interface_hud (Utilities|Casting|CastToUserInterfaceHud (HUD|GetHUD PlayerController)))
  (Default|LoadUI _asuser_interface_hud "Gameplay")
  (Default|NotifyonAbilityLevelUp PlayerController 0 1)
  (Default|NotifyonAbilityLevelUp PlayerController 1 1)
  (Default|NotifyonAbilityLevelUp PlayerController 2 1))

(fn UpdateHealthBarDisplay
  (bind _asuser_interface_hud (Utilities|Casting|CastToUserInterfaceHud (HUD|GetHUD (Game|GetPlayerController (Variables|Default|GetplayerIndex)))))
  (Utilities|IsValid (Variables|/Game/UI/UserInterfaceHud.UserInterfaceHud_C|GetGameplayWidget _asuser_interface_hud)
    (:Is%20Valid
      _)
    (:Is%20Not%20Valid
      (Default|LoadUI _asuser_interface_hud "Gameplay")))
  (Default|UpdateHealth (Variables|/Game/UI/UserInterfaceHud.UserInterfaceHud_C|GetGameplayWidget _asuser_interface_hud) (Variables|Default|GetHealth) (Variables|Default|GetMaxHealth)))

(fn UpdateXPDisplay
  (params (IncreasedLevel :type Boolean))
  (bind _ascustom_player_controller_bp (Utilities|Casting|CastToCustomPlayerController_BP (Game|GetPlayerController (Variables|Default|GetplayerIndex))))
  (bind _asuser_interface_hud (Utilities|Casting|CastToUserInterfaceHud (HUD|GetHUD _ascustom_player_controller_bp)))
  (Default|UpdatePlayerXP (Variables|/Game/UI/UserInterfaceHud.UserInterfaceHud_C|GetGameplayWidget _asuser_interface_hud) (Variables|Default|GetPlayerCurrent%20XP) (Variables|Default|GetPlayer%20Max%20XP) IncreasedLevel))

(fn BlockRelease
  (Animation|PlayAnimMontage "/Game/Characters/PlayableCharacters/NewAssets/Animations/Blocking/BlockEnd_AnimMontage.BlockEnd_AnimMontage" 1.0 "None"))

(fn UpdatePlayerPoints
  (params (AddedPoints :type Integer))
  (Variables|Default|SetPoints (+ AddedPoints (Variables|Default|GetPoints)))
  (bind _ascustom_player_controller_bp (Utilities|Casting|CastToCustomPlayerController_BP (Pawn|GetController)))
  (bind _asuser_interface_hud (Utilities|Casting|CastToUserInterfaceHud (HUD|GetHUD _ascustom_player_controller_bp)))
  (Default|UpdatePoints (Variables|/Game/UI/UserInterfaceHud.UserInterfaceHud_C|GetGameplayWidget _asuser_interface_hud) (Variables|Default|GetPoints)))

(fn CanDoDamage
  (params (AttackerForwardVector :type Vector))
  (bind _output_get (LocalVariables|SetForwardVector AttackerForwardVector))
  (return (> -0.75 (Math|Vector|DotProduct _output_get (Transformation|GetActorForwardVector)))))

(fn InitializePlayerStartingAttributes
  (for _index (range 0 2)
    (Utilities|Array|SetArrayElem (Variables|Default|GetAbilityOccupationSlots) _index false true)
    (Utilities|Array|Add (Variables|Default|GetAbilitySlots) 0))
  (CallFunction|UpdateHealthBarDisplay)
  (CallFunction|UpdateXPDisplay false)
  (bind _astop_down_game_mode (Utilities|Casting|CastToTopDownGameMode (Game|GetGameMode)))
  (Variables|Default|SetGameMode _astop_down_game_mode))