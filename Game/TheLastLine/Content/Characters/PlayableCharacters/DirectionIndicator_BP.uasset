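; Arrow indicator actor that shows the direction from a linked actor to a destination.
; Each tick it places the arrow 100 units from the linked actor toward the destination, lowered slightly and rotated in yaw only to match that direction.
; Within 400 units of the destination it hides the arrow by swapping to an invisible material.
; DestinationReached destroys the indicator.
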(event EventBeginPlay)

(event Collision|EventActorBeginOverlap
  (params (OtherActor :type Actor%20Object%20Reference)))

(event EventTick
  (params (DeltaSeconds :type Float%20%28single-precision%29))
  (bind _linkedactor (Variables|Default|GetLinkedActor))
  (bind _linkedactor_2 (Variables|Default|GetLinkedActor))
  (bind _destination (Variables|Default|GetDestination))
  (bind _returnvalue (Transformation|GetActorLocation _linkedactor))
  (bind _returnvalue_2 (Transformation|GetActorLocation _linkedactor_2))
  (bind _returnvalue_3 (Math|Vector|GetUnitDirection(Vector) _destination _returnvalue))
  (bind _returnvalue_4 (* _returnvalue_3 -1e+02))
  (bind _returnvalue_5 (+ _returnvalue_4 _returnvalue_2))
  (Utilities|IsValid (Variables|Default|GetLinkedActor)
    (:Is%20Valid
      (if (>= (Math|Vector|VectorLength (- (Variables|Default|GetDestination) (Transformation|GetActorLocation (Variables|Default|GetLinkedActor)))) 4e+02)
        (Rendering|Material|SetMaterial (Variables|Default|GetArrowDirection) 0 "/Game/Controllers/PlayerControllers/Direction.Direction")
        (Transformation|SetWorldLocation (Variables|Default|GetArrowDirection) _returnvalue false false)
        (Transformation|SetWorldRotation (Variables|Default|GetArrowDirection) (Math|Rotator|MakeRotator 0.0 0.0 (- (.yaw (Math|Rotator|MakeRotfromX _returnvalue_3)) 9e+01)) false false)
        (Transformation|SetWorldLocation (Variables|Default|GetArrowDirection) (Math|Vector|MakeVector (.x _returnvalue_5) (.y _returnvalue_5) (- (.z _returnvalue_5) 5e+01)) false false)
        (else
          (Rendering|Material|SetMaterial (Variables|Default|GetArrowDirection) 0 "/Game/GameData/GlobalMaterials/M_InvisibleMaterial.M_InvisibleMaterial"))))))

(fn ConstructionScript)

(fn DestinationReached
  (Actor|DestroyActor))