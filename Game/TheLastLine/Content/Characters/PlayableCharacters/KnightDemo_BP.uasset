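; KnightDemo_BP is a playable knight character that equips itself with gear and sets its own combat stats.
; After the parent BeginPlay, CreateWeapons spawns a scaled-down sword and tower shield plus a helmet, snapping each to its skeletal mesh socket.
; The sword is stored and given the knight as its Holder.
; The construction script fills in health, damage, resistances, speeds, XP gain, size and team defaults.
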(event Custom|CreateWeapons
  (bind _returnvalue (Transformation|GetActorTransform))
  (bind _returnvalue_2 (Transformation|GetActorTransform))
  (bind _returnvalue_3 (Transformation|GetActorTransform))
  (Utilities|FlowControl|Sequence
    (:then_0
      (bind _returnvalue_4 (Game|SpawnActorfromClass "/Game/Items/Sword/Sword1_BP.Sword1_BP_C" (Math|Transform|MakeTransform (.location _returnvalue_2) (.rotation _returnvalue_2) (* "1.000000,1.000000,1.000000" "0.200000,0.200000,0.200000")) "Undefined" 0 0))
      (Utilities|IsValid _returnvalue_4
        (:Is%20Valid
          (bind _output_get (Variables|Default|SetSword _returnvalue_4))
          (Variables|/Game/Items/Sword/Sword1_BP.Sword1_BP_C|SetHolder _output_get self)
          (Transformation|AttachComponentToComponent _returnvalue_4 (Variables|Character|GetMesh) "WeaponSocket" "SnapToTarget" "SnapToTarget" "KeepWorld" false))))
    (:then_1
      (bind _returnvalue_5 (Game|SpawnActorfromClass "/Game/Items/Shield/TowerShield_BP.TowerShield_BP_C" (Math|Transform|MakeTransform (.location _returnvalue_3) (.rotation _returnvalue_3) (* "1.000000,1.000000,1.000000" "0.200000,0.200000,0.200000")) "Undefined" 0 0))
      (Utilities|IsValid _returnvalue_5
        (:Is%20Valid
          (Transformation|AttachComponentToComponent _returnvalue_5 (Variables|Character|GetMesh) "ShieldSocket" "SnapToTarget" "SnapToTarget" "KeepWorld" false))))
    (:then_2
      (bind _returnvalue_6 (Game|SpawnActorfromClass "/Game/Items/Helmet/HelmetItem.HelmetItem_C" (Math|Transform|MakeTransform (.location _returnvalue) (.rotation _returnvalue) (.scale _returnvalue)) "Undefined" 0 0))
      (Utilities|IsValid _returnvalue_6
        (:Is%20Valid
          (Transformation|AttachComponentToComponent _returnvalue_6 (Variables|Character|GetMesh) "HeadSocket" "SnapToTarget" "SnapToTarget" "KeepWorld" false))))))

(event EventBeginPlay
  (|CallParentFunction)
  (CallFunction|CreateWeapons))

(event Collision|EventActorBeginOverlap
  (params (OtherActor :type Actor%20Object%20Reference))
  (|CallParentFunction OtherActor) ; This node is disabled and will not be called.\nDrag off pins to build functionality.
)

(fn ConstructionScript
  (bind _output_get (Variables|Default|SetHealth 1e+02))
  (Variables|Default|SetMaxHealth _output_get)
  (Variables|Default|SetDamage 2e+01)
  (Variables|Default|SetMagicalResist 0.1)
  (Variables|Default|SetPhysicalResist 0.1)
  (Variables|Default|SetMovementSpeed 5e+02)
  (Variables|Default|SetAttackSpeed 1.0)
  (Variables|Default|SetXPGain 0)
  (Variables|Default|SetisLarge false)
  (Variables|Default|SetTeamNumber 0))