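; Arena map handler that advances enemy waves, extending a parent handler that triggers UpdateNextWave.
; It starts at wave zero with a single objective already marked completed.
; Each update notifies every player's gameplay HUD widget of the new wave, increments the counter, calls SpawnWave, then displays the wave's unit total.
; An older WaveSpawner path with calculated health scaling remains but never runs.
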(event EventBeginPlay
  (|CallParentFunction)
  (Variables|Default|SetCurrentWave 0)
  (Variables|Default|SetObjectiveList (Utilities|Array|MakeArray (Utilities|Struct|MakeObjectiveStruct "None" "" "" 0.0 0.0 true))))

(event EventUpdateNextWave
  (params (TimeBeforeSpawnWave :type Float%20%28single-precision%29))
  ;[1 1 1] Parent will call this function
  (Development|PrintString "Updating all player controllers" true true "(R=0.000000,G=0.660000,B=1.000000,A=1.000000)" 5.0)
  ;[1 1 1] Update all players gameplay interface with new wave indication
  (bind _astop_down_game_mode (Utilities|Casting|CastToTopDownGameMode (Game|GetGameMode))
    (:then
      (for _index (range 0 (Variables|/Game/GameData/GameModes/TopDownGameMode.TopDownGameMode_C|GetNumberOfPlayers _astop_down_game_mode))
        (bind _asuser_interface_hud (Utilities|Casting|CastToUserInterfaceHud (HUD|GetHUD (Game|GetPlayerController _index)))
          (:then
            (Utilities|IsValid (Variables|/Game/UI/UserInterfaceHud.UserInterfaceHud_C|GetGameplayWidget _asuser_interface_hud)
              (:Is%20Valid
                (Default|NotifyNewWave (Variables|/Game/UI/UserInterfaceHud.UserInterfaceHud_C|GetGameplayWidget _asuser_interface_hud) (+ (Variables|Default|GetCurrentWave) 1)))
              (:Is%20Not%20Valid
                (Development|PrintString "gameplay Widget is not working"))))
          (:CastFailed
            (Development|PrintString "Faied casting widget"))))
      (Math|Integer|IncrementInt (Variables|Default|GetCurrentWave)
        (:%20%20
          (CallFunction|SpawnWave)
          (Development|PrintText (Utilities|Text|FormatText "Wave spawn with {N} units" (Variables|Default|GetTotalWaveUnits)))
          (bind _astop_down_game_mode_2 (Utilities|Casting|CastToTopDownGameMode (Game|GetGameMode)))
          (for _index_2 (range 0 (Variables|/Game/GameData/GameModes/TopDownGameMode.TopDownGameMode_C|GetNumberOfPlayers _astop_down_game_mode_2))
            (bind _asuser_interface_hud_2 (Utilities|Casting|CastToUserInterfaceHud (HUD|GetHUD (Game|GetPlayerController _index_2))))
            (Utilities|IsValid (Variables|/Game/UI/UserInterfaceHud.UserInterfaceHud_C|GetGameplayWidget _asuser_interface_hud_2)
              (:Is%20Valid
                (Default|UpdateWaveDisplay (Variables|/Game/UI/UserInterfaceHud.UserInterfaceHud_C|GetGameplayWidget _asuser_interface_hud_2) (Utilities|Text|ToText(Integer) (Variables|Default|GetTotalWaveUnits)))))))))
    (:CastFailed
      (Development|PrintString "top down Casting failed"))))

(fn ConstructionScript
  (|CallParentFunction))