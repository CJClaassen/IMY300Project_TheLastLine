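; Spawner actor that places ability pickups at every AbilitySpawnLocation in the level, on BeginPlay and again on a three-minute looping timer.
; Each update hides the location marker cubes with an invisible material and spawns pickups typed from a generated ability list, without removing earlier ones.
; GenerateAbilitiesToSpawn draws from Abilities with a random stream, attempting to skip duplicates without rerolling.
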(event Custom|UpdateAbilities
  (for _array_element (Variables|Default|GetAbilitySpawnLocations)
    ;[1 1 1] Spawn a random ability at the spawn location
    (Rendering|Material|SetMaterial (Variables|/Game/Abilities/AbilitySpawner/AbilitySpawnLocation.AbilitySpawnLocation_C|GetCube _array_element) 0 "/Game/GameData/GlobalMaterials/M_InvisibleMaterial.M_InvisibleMaterial"))
  (bind _abilities_chosen (CallFunction|GenerateAbilitiestoSpawn (Utilities|Array|Length (Variables|Default|GetAbilitySpawnLocations))))
  (for (_array_element_2 _array_index) _abilities_chosen
    (bind _returnvalue (Game|SpawnActorfromClass "/Game/Abilities/Pickup/PickUpAbility_BP.PickUpAbility_BP_C" (Math|Transform|MakeTransform (Transformation|GetActorLocation (Utilities|Array|Get(acopy) (Variables|Default|GetAbilitySpawnLocations) _array_index)) "0, 0, 0" "1,1,1") "AlwaysSpawn" 0 0))
    (Variables|/Game/Abilities/Pickup/PickUpAbility_BP.PickUpAbility_BP_C|SetAbilityType _returnvalue _array_element_2)
    (Default|ClasstoName _returnvalue _array_element_2)))

(event EventBeginPlay
  (bind _outactors (Actor|GetAllActorsOfClass "/Game/Abilities/AbilitySpawner/AbilitySpawnLocation.AbilitySpawnLocation_C"))
  (Variables|Default|SetAbilitySpawnLocations _outactors)
  (CallFunction|UpdateAbilities)
  (Utilities|Time|SetTimerbyEvent (delegate Custom|UpdateAbilities) 1.8e+02 true))

(event Collision|EventActorBeginOverlap
  (params (OtherActor :type Actor%20Object%20Reference)))

(event EventTick
  (params (DeltaSeconds :type Float%20%28single-precision%29)))

(fn ConstructionScript)

(fn GenerateAbilitiestoSpawn
  (params (NumberOfSpawnPoints :type Integer))
  (bind _result (Math|Integer|DecrementInt NumberOfSpawnPoints)
    (:%20%20
      (for _index (range 0 _result)
        (bind _output_get (LocalVariables|SetRandom (Math|Random|RandomIntegerinRangefromStream 1 (Utilities|Array|Length (Variables|Default|GetAbilities)) (Variables|Default|GetRandomStream))))
        (bind _result_2 (Math|Integer|DecrementInt _output_get)
          (:%20%20
            (bind _array_element (Utilities|Array|ForEachLoopwithBreak (LocalVariables|GetSelectedAbilties) :!label _label)
              (:LoopBody
                (if (== _array_element (Utilities|Array|Get(acopy) (Variables|Default|GetAbilities) _result_2))
                  (LocalVariables|SetisAlreadyAdded true)
                  (goto _label Break)))
              (:Completed
                (if (not (LocalVariables|GetisAlreadyAdded))
                  (Utilities|Array|SetArrayElem (LocalVariables|GetSelectedAbilties) _index (Utilities|Array|Get(acopy) (Variables|Default|GetAbilities) (LocalVariables|GetRandom)) true)))))))
      (return (LocalVariables|GetSelectedAbilties)))))