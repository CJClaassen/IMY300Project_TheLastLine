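; StoneWall cast ability for the Knight that raises a temporary Wall_BP in front of the casting player.
; Action spawns the wall with health from knight MaxHealth times slot level, enables box collision and raises it by timeline with rock sounds.
; Slot XP is granted when the raise ends and when non-player damage meets or exceeds wall health.
; BreakDown destroys the wall and disables collision after its lifespan.
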(event OnTakeAnyDamage(Wall)
  (params (DamagedActor :type Actor%20Object%20Reference) (Damage :type Float%20%28single-precision%29) (DamageType :type Damage%20Type%20Object%20Reference) (InstigatedBy :type Controller%20Object%20Reference) (DamageCauser :type Actor%20Object%20Reference))
  ;[1 1 1] If damage wasn't caused by player
  (Utilities|Casting|CastToPlayerController InstigatedBy
    (:CastFailed
      (if (>= Damage (Variables|/Game/Abilities/CastAbilities/WallRaise/Wall_BP.Wall_BP_C|GetHealth (Variables|Default|GetWall)))
        ;[1 1 1] Reward the player for using it effectively
        (bind _asknight_bp (Utilities|Casting|CastToKnight_BP (Pawn|GetControlledPawn (Game|GetPlayerController (Variables|Default|GetPlayerIndex)))))
        (Default|UpdateAbilitySlot _asknight_bp (Variables|Default|GetAbilitySlotIndex) (/ (Variables|Default|GetXpGainAlternative) 2.0))
        (else
          (Variables|/Game/Abilities/CastAbilities/WallRaise/Wall_BP.Wall_BP_C|SetHealth (Variables|Default|GetWall) (- (Variables|/Game/Abilities/CastAbilities/WallRaise/Wall_BP.Wall_BP_C|GetHealth (Variables|Default|GetWall)) Damage)))))))

(event Custom|PlayMainSound
  ;[1 1 1] Plays the main sounds
  (Audio|PlaySoundatLocation "/Game/Sound/StoneWallAbility/groundfalling.groundfalling" (Transformation|GetActorLocation) "0, 0, 0" 1.0 1.0 0.0 0 "/Game/Sound/StoneWallAbility/StoneWall_Sound_Concurrency.StoneWall_Sound_Concurrency" 0)
  (Audio|PlaySoundatLocation "/Game/Sound/StoneWallAbility/fallingRocks.fallingRocks" (Transformation|GetActorLocation) "0, 0, 0" 1.0 1.0 0.1 0 "/Game/Sound/StoneWallAbility/StoneWall_Sound_Concurrency.StoneWall_Sound_Concurrency" 0))

(event Custom|RandomRockfall
  ;[1 1 1] Plays the single indivual rocks at each at a different timestamp of the ability
  (if (not (Variables|Default|GetisDoneAnimating))
    (switch int (Math|Random|RandomIntegerinRange 0 3)
      (:0
        (Variables|Default|SetselectedRockSound "/Game/Sound/StoneWallAbility/SingleRockHit1.SingleRockHit1"))
      (:1
        (Variables|Default|SetselectedRockSound "/Game/Sound/StoneWallAbility/SingleRockHit2.SingleRockHit2"))
      (:2
        (Variables|Default|SetselectedRockSound "/Game/Sound/StoneWallAbility/SingleRockHit3.SingleRockHit3"))
      (:3
        (Variables|Default|SetselectedRockSound "/Game/Sound/StoneWallAbility/SingleRockHit4.SingleRockHit4")))
    (Audio|PlaySoundatLocation (Variables|Default|GetselectedRockSound) (Transformation|GetActorLocation) "0, 0, 0" (Math|Random|RandomFloatinRange 0.1 0.4) 1.0 0.0 0 "/Game/Sound/StoneWallAbility/StoneWall_Sound_Concurrency.StoneWall_Sound_Concurrency" 0)))

(event Custom|Set%20isDoneAnim
  (Variables|Default|SetisDoneAnimating true))

(event EventBeginPlay)

(event Collision|EventActorBeginOverlap
  (params (OtherActor :type Actor%20Object%20Reference)))

(event EventTick
  (params (DeltaSeconds :type Float%20%28single-precision%29)))

(event EventAction
  (params (Location :type Vector :default "0, 0, 0") (Rotation :type Rotator :default "0, 0, 0") (PlayerIndex :type Integer) (Slot%20Level :type Integer) (SlotIndex :type Integer))
  (bind _returnvalue (Game|GetPlayerController PlayerIndex))
  (bind _returnvalue_2 (Pawn|GetControlledPawn _returnvalue))
  (bind _returnvalue_3 (Transformation|GetActorRotation _returnvalue_2))
  (bind _returnvalue_4 (Transformation|GetActorRotation _returnvalue_2))
  (bind _returnvalue_5 (- (.yaw _returnvalue_3) 9e+01))
  ;[1 1 1] Casting the wall ability
  ;;[1 1 1] Spawn and initialize the wall
  (Variables|Default|SetearlyActivation false)
  (Variables|Default|SetPlayerIndex PlayerIndex)
  (Variables|Default|SetSlotLevel Slot%20Level)
  (Variables|Default|SetisDestroyed false)
  (bind _output_get (Variables|Default|SetcastedLocation Location))
  (Variables|Default|SetForwardVector (Transformation|GetActorForwardVector _returnvalue_2))
  (Transformation|SetWorldLocationAndRotation (Variables|Default|GetBox) _output_get (Math|Rotator|MakeRotator (.roll _returnvalue_3) (.pitch _returnvalue_3) _returnvalue_5) false false)
  (bind _returnvalue_6 (Game|SpawnActorfromClass "/Game/Abilities/CastAbilities/WallRaise/Wall_BP.Wall_BP_C" (Math|Transform|MakeTransform _output_get (Math|Rotator|MakeRotator (.roll _returnvalue_3) (.pitch _returnvalue_3) _returnvalue_5) "0.500000,0.500000,0.500000") "AlwaysSpawn" 0 0))
  (bind _output_get_2 (Variables|Default|SetWall _returnvalue_6))
  (bind _wall_health (CallFunction|CalculateHealth))
  (Variables|/Game/Abilities/CastAbilities/WallRaise/Wall_BP.Wall_BP_C|SetHealth _output_get_2 _wall_health)
  (Collision|SetCollisionEnabled (Variables|Default|GetBox) "QueryAndPhysics")
  (CallFunction|PlayMainSound)
  (Utilities|Time|SetTimerbyEvent (delegate Custom|RandomRockfall) 0.3 true)
  (Variables|Default|SetisDoneAnimating false)
  (Utilities|Time|SetTimerbyEvent (delegate Custom|Set%20isDoneAnim) 2.5 true)
  (Transformation|SetWorldLocationAndRotation (Variables|Default|GetBox) (+ (Variables|Default|GetcastedLocation) (* (Variables|Default|GetForwardVector) 2.5e+02)) (Math|Rotator|MakeRotator (.roll _returnvalue_4) (.pitch _returnvalue_4) (+ (.yaw _returnvalue_4) 9e+01)) false false)
  ;;[1 1 1] Raise the wall at the casted location
  (bind _raise (Timeline|WallRaise PlayFromStart)
    (:Update
      (Transformation|SetActorLocation (Variables|Default|GetWall) (Math|Vector|MakeVector (+ (.x (Variables|Default|GetcastedLocation)) (.x (* (Variables|Default|GetForwardVector) 2.5e+02))) (+ (.y (Variables|Default|GetcastedLocation)) (.y (* (Variables|Default|GetForwardVector) 2.5e+02))) (- (+ (.z (Variables|Default|GetcastedLocation)) _raise) 1e+02)) false false))
    (:Finished
      (Variables|Default|SetisDoneAnimating true)
      (bind _asknight_bp (Utilities|Casting|CastToKnight_BP (Pawn|GetControlledPawn (Game|GetPlayerController (Variables|Default|GetPlayerIndex)))))
      (Default|UpdateAbilitySlot _asknight_bp (Variables|Default|GetAbilitySlotIndex) (/ (Variables|Default|GetXpGainAlternative) 2.0))
      ;[1 1 1] Check if the wall is still standing
      (Utilities|FlowControl|Delay (Variables|Default|GetWallLifeSpan))
      (if (not (Variables|Default|GetisDestroyed))
        (Variables|Default|SetisDestroyed true)
        (CallFunction|BreakDown)))))

(fn ConstructionScript
  (Variables|Default|SetCooldown 45.0)
  (Variables|Default|SetXpGainAlternative 15.0)
  (Variables|Default|SetWallLifeSpan 2e+01)
  (Variables|Default|SetAbilityName "StoneWall"))

(fn BreakDown
  (Actor|DestroyActor (Variables|Default|GetWall))
  (Collision|SetCollisionEnabled (Variables|Default|GetBox) "NoCollision"))

(fn CreateCube)

(fn CalculateHealth
  (bind _asknight_bp (Utilities|Casting|CastToKnight_BP (Game|Player|GetPlayerPawn (Variables|Default|GetPlayerIndex))))
  (return (* (Variables|/Game/Characters/AbstractCharacter.AbstractCharacter_C|GetMaxHealth _asknight_bp) (Math|Conversions|ToFloat(Integer) (Variables|Default|GetSlotLevel)))))