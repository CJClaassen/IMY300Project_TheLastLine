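; Knight cast ability Blade Rain, which drops swords around a target location and deals magic damage to other-team characters in a circle.
; Action spawns randomly placed, angled Sword_BP actors; timelines accelerate them down to the cast height and animate opacity before destroying them.
; Damage hits the sphere's overlaps immediately on cast, scaled by Knight damage, player level, slot level and power boost.
; Tutorial mode shortens the cooldown.
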(event EventBeginPlay
  ;[1 1 1] Adding all the friendly type of characters to the whitelist
  (Utilities|Array|Add (Variables|Default|GetObjectTypes) "ObjectTypeQuery3")
  (bind _outactors (Actor|GetAllActorsOfClass "/Game/Characters/AbstractCharacter.AbstractCharacter_C"))
  (for _array_element _outactors
    (if (!= (Variables|/Game/Characters/AbstractCharacter.AbstractCharacter_C|GetTeamNumber _array_element) (Variables|Default|GetEnemyType))
      (Utilities|Array|Add (Variables|Default|GetIgnoreActors) _array_element)))
  (bind _astop_down_game_mode (Utilities|Casting|CastToTopDownGameMode (Game|GetGameMode)))
  (if (Variables|/Game/GameData/GameModes/TopDownGameMode.TopDownGameMode_C|GetisTutorial _astop_down_game_mode)
    (Variables|Default|SetCooldown 5.0)))

(event Collision|EventActorBeginOverlap
  (params (OtherActor :type Actor%20Object%20Reference))
  (|CallParentFunction OtherActor) ; This node is disabled and will not be called.\nDrag off pins to build functionality.
)

(event EventAction
  (params (Location :type Vector :default "0, 0, 0") (Rotation :type Rotator :default "0, 0, 0") (PlayerIndex :type Integer) (Slot%20Level :type Integer) (SlotIndex :type Integer))
  (bind _sphere (Variables|Default|GetSphere))
  (bind _spawnradius (Variables|AbilityCasting|GetSpawnRadius))
  (bind _spawnradius_2 (Variables|AbilityCasting|GetSpawnRadius))
  ;[1 1 1] Upon activating the ability for BladeRain
  (Variables|Default|SetisActivated true)
  (Variables|Default|SetearlyActivation false)
  (Components|Sphere|SetSphereRadius (Variables|Default|GetSphere) (Variables|AbilityCasting|GetDamageRadius) true)
  (Variables|Default|SetSlotLevel Slot%20Level)
  (Variables|Default|SetPlayerIndex PlayerIndex)
  (bind _output_get (Variables|Default|SetCastedLocation (Math|Vector|MakeVector (.x Location) (.y Location) (.z Location))))
  ;;[1 1 1] Generating new location and rotations for the sword
  (for _index (range 0 (Variables|AbilityCasting|GetnumberOfSwords))
    (Variables|Default|SetNewSwordsLocation (Math|Vector|MakeVector (+ (.x _output_get) (Math|Random|RandomFloatinRange (* _spawnradius_2 -1.0) _spawnradius_2)) (+ (.y _output_get) (Math|Random|RandomFloatinRange (* _spawnradius -1.0) _spawnradius)) (+ (.z _output_get) (- (Variables|AbilityCasting|GetBaseHeight) (Math|Random|RandomFloatinRange -5e+02 2e+02)))))
    (Variables|Default|SetNewSwordRotation (Math|Rotator|MakeRotator (Math|Random|RandomFloatinRange 0.0 3.6e+02) (Math|Random|RandomFloatinRange -115.0 -75.0) (Math|Random|RandomFloatinRange -2e+01 2e+01)))
    (bind _ascustom_player_controller_bp (Utilities|Casting|CastToCustomPlayerController_BP (Game|GetPlayerController 0)))
    ;;[1 1 1] Creating the swords at their generated location and rotation
    (bind _returnvalue (Game|SpawnActorfromClass "/Game/Abilities/CastAbilities/BladeRain/Sword_BP.Sword_BP_C" (Math|Transform|MakeTransform (Variables|Default|GetNewSwordsLocation) (Variables|Default|GetNewSwordRotation) (Math|Vector|MakeVector 0.2 0.2 0.2)) "AlwaysSpawn" self (Variables|/Game/Controllers/PlayerControllers/CustomPlayerController_BP.CustomPlayerController_BP_C|GetPlayerCharacter _ascustom_player_controller_bp)))
    (Utilities|Array|Add (Variables|Default|GetSwordsList) _returnvalue))
  (bind _astop_down_game_mode (Utilities|Casting|CastToTopDownGameMode (Game|GetGameMode)))
  (Audio|PlaySoundatLocation "/Game/Abilities/CastAbilities/BladeRain/Assets/swordability1.swordability1" (Variables|Default|GetCastedLocation) "0, 0, 0" (Default|GetSoundEffectVolume _astop_down_game_mode) 1.0 0.0 0 0 0)
  (Utilities|FlowControl|Sequence
    (:then_0
      ;;[1 1 1] Animating the falling swords
      (bind _aceleration (Timeline|FallingAcceleration PlayFromStart)
        (:Update
          (for _array_element (Variables|Default|GetSwordsList)
            (if (> (.z (Transformation|GetWorldLocation (Variables|/Script/Engine.Actor|GetRootComponent _array_element))) (.z (Variables|Default|GetCastedLocation)))
              (Transformation|SetWorldLocation (Variables|/Script/Engine.Actor|GetRootComponent _array_element) (+ (Transformation|GetWorldLocation (Variables|/Script/Engine.Actor|GetRootComponent _array_element)) (* (Math|Vector|GetForwardVector (Variables|/Script/Engine.Actor|GetRootComponent _array_element)) _aceleration)) false false))))))
    (:then_1
      ;;;[0.2826 0.5885 0.2027] Apply damage and fade out
      (bind _damage (CallFunction|CalculateDamage (Variables|Default|GetSlotLevel) (Variables|Default|GetPlayerIndex)))
      (Variables|Default|Setdamage _damage)
      (Transformation|SetWorldLocation _sphere (Variables|Default|GetCastedLocation) false false)
      (bind _output_get_2 (Variables|Default|SetOverlappingActors (Collision|GetOverlappingActors _sphere "/Game/Characters/AbstractCharacter.AbstractCharacter_C" :!class /Script/Engine.PrimitiveComponent)))
      (bind _output_get_3 (Variables|Default|Setindex (- (Utilities|Array|Length _output_get_2) 1)))
      (for _index_2 (range 0 _output_get_3)
        (bind _asabstract_character (Utilities|Casting|CastToAbstractCharacter (Utilities|Array|Get(acopy) (Variables|Default|GetOverlappingActors) _index_2)))
        (Utilities|IsValid _asabstract_character
          (:Is%20Valid
            (bind _asabstract_character_2 (Utilities|Casting|CastToAbstractCharacter (Game|Player|GetPlayerPawn (Variables|Default|GetPlayerIndex))))
            (if (!= (Variables|/Game/Characters/AbstractCharacter.AbstractCharacter_C|GetTeamNumber _asabstract_character_2) (Variables|/Game/Characters/AbstractCharacter.AbstractCharacter_C|GetTeamNumber _asabstract_character))
              (Game|Damage|ApplyDamage _asabstract_character (Variables|Default|Getdamage) (Game|GetPlayerController (Variables|Default|GetPlayerIndex)) self "/Game/GameData/Damages/DamageType_Magic.DamageType_Magic_C")))))
      (bind _opacity (Timeline|Opacity PlayFromStart)
        (:Update
          (for _array_element_2 (Variables|Default|GetSwordsList)
            (Rendering|Material|SetScalarParameterValue (Variables|/Game/Abilities/CastAbilities/BladeRain/Sword_BP.Sword_BP_C|GetSwordMaterial _array_element_2) "Opacity" _opacity :!class /Script/Engine.MaterialInstanceDynamic)))
        (:Finished
          (for _array_element_3 (Variables|Default|GetSwordsList)
            (Actor|DestroyActor _array_element_3))
          (Utilities|Array|Clear (Variables|Default|GetSwordsList)))))))

(fn ConstructionScript
  (Variables|Default|SetCooldown 25.0)
  (Variables|Default|SetXpModifier 0.45)
  (Variables|Default|SetXpGainAlternative 1e+01)
  (Variables|Default|SetAbilityName "Blade Rain")
  (Variables|Default|SetRadius (Variables|AbilityCasting|GetDamageRadius)))

(fn CalculateDamage
  (params (SlotLevel :type Integer) (PlayerIndex :type Integer))
  (bind _asknight_bp (Utilities|Casting|CastToKnight_BP (Game|Player|GetPlayerPawn PlayerIndex)))
  (bind _damage (Default|GetCalculatedDamage _asknight_bp))
  (return (+ (+ (+ (* _damage 0.5) (* (* SlotLevel _damage) 0.2)) (Math|Conversions|ToFloat(Integer) (Variables|/Game/Characters/PlayableCharacters/Knight_BP.Knight_BP_C|GetPlayerLevel _asknight_bp))) (* (+ (+ (* _damage 0.5) (* (* SlotLevel _damage) 0.2)) (Math|Conversions|ToFloat(Integer) (Variables|/Game/Characters/PlayableCharacters/Knight_BP.Knight_BP_C|GetPlayerLevel _asknight_bp))) (Variables|/Game/Characters/Components/PlayerSkillSet.PlayerSkillSet_C|GetAbilityPowerBoost (Variables|Default|GetAbilityComponent)))) (+ (+ (+ (* _damage 0.5) (* (* SlotLevel _damage) 0.2)) (Math|Conversions|ToFloat(Integer) (Variables|/Game/Characters/PlayableCharacters/Knight_BP.Knight_BP_C|GetPlayerLevel _asknight_bp))) (* (+ (+ (* _damage 0.5) (* (* SlotLevel _damage) 0.2)) (Math|Conversions|ToFloat(Integer) (Variables|/Game/Characters/PlayableCharacters/Knight_BP.Knight_BP_C|GetPlayerLevel _asknight_bp))) (Variables|/Game/Characters/Components/PlayerSkillSet.PlayerSkillSet_C|GetAbilityPowerBoost (Variables|Default|GetAbilityComponent))))))

(fn GetAbilityDescription
  (bind _damage (CallFunction|CalculateDamage (Variables|Default|GetSlotLevel) (Variables|Default|GetPlayerIndex)))
  (LocalVariables|Setdmg _damage)
  (if (CallFunction|IsReady)
    (LocalVariables|SetreadyState "Can activate")
    (else
      (LocalVariables|SetreadyState "On cooldown")))
  (return (Utilities|Text|FormatText "Damage: {dmg} 
Radius: {radius} 
AoE type: Circle 
Damage Type: magic 
Cooldown: {cooldown}s 
Ready: {readiness} 
 
Description: 
This ability allows the knight to call upon the heavens. With the heavens throwing down the Blades of Light." (LocalVariables|Getdmg) (Variables|AbilityCasting|GetDamageRadius) (CallFunction|GetCooldown) (LocalVariables|GetreadyState))))