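; Impalement ("Spears of Dagon") is a Knight line-AoE ability that thrusts spears out of the ground ahead of the caster.
; Activate spawns randomly angled spears below ground along a slot-level-scaled length, fits a damage box to it and raises them with a timeline.
; When the timeline ends, enemies in the box take physical damage from Knight stats and slot level, usually distance-scaled, and spears despawn after a delay.
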(event EventBeginPlay
  ;[1 1 1] Init cooldown for tutorial
  (bind _astop_down_game_mode (Utilities|Casting|CastToTopDownGameMode (Game|GetGameMode)))
  (if (Variables|/Game/GameData/GameModes/TopDownGameMode.TopDownGameMode_C|GetisTutorial _astop_down_game_mode)
    (Variables|Default|SetCooldown 5.0)))

(event Collision|EventActorBeginOverlap
  (params (OtherActor :type Actor%20Object%20Reference))
  (|CallParentFunction OtherActor) ; This node is disabled and will not be called.\nDrag off pins to build functionality.
)

(event EventTick
  (params (DeltaSeconds :type Float%20%28single-precision%29))
  (|CallParentFunction DeltaSeconds) ; This node is disabled and will not be called.\nDrag off pins to build functionality.
)

(event EventActivate
  (params (Location :type Vector :default "0, 0, 0") (Rotator :type Rotator :default "0, 0, 0") (PlayerIndex :type Integer) (Slot%20level :type Integer) (SlotIndex :type Integer))
  (bind _spears (Variables|Default|GetSpears))
  (bind _box (Variables|Default|GetBox))
  (bind _box_2 (Variables|Default|GetBox))
  (bind _returnvalue (Transformation|GetWorldRotation _box_2))
  (bind _boxextent (Variables|/Script/Engine.BoxComponent|GetBoxExtent _box))
  ;[1 1 1] Upon ability activate
  (|CallParentFunction Location Rotator PlayerIndex Slot%20level SlotIndex)
  (Variables|Default|SetPlayerIndex PlayerIndex)
  (Variables|Default|SetSlotLevel Slot%20level)
  (Variables|Default|SetSlotIndex SlotIndex)
  (Variables|Default|SetearlyActivation false)
  (Variables|Default|SetMaxLength (+ 3e+02 (* 3e+02 (/ (Math|Conversions|ToFloat(Integer) (Variables|Default|GetSlotLevel)) 1e+01))))
  (Transformation|SetActorLocationAndRotation Location Rotator)
  (Variables|Default|SetActivationTime (Utilities|Time|GetGameTimeinSeconds))
  ;;[1 1 1] Clear the previous casted impalement spell first
  (for _array_element (Variables|Default|GetSpears)
    (Actor|DestroyActor _array_element))
  (Utilities|Array|Clear (Variables|Default|GetSpears))
  ;;[1 1 1] Setting variable
  (Variables|Default|SetCasterLocation Location)
  (bind _output_get (Variables|Default|Setpawn (Pawn|GetControlledPawn (Game|GetPlayerController (Variables|Default|GetPlayerIndex)))))
  (Variables|Default|SetForwardDirectionvector (Transformation|GetActorForwardVector _output_get))
  ;;[1 1 1] Calculate the location and direction the spears will face when casted
  (for _index (range 1 (Variables|Default|GetNumberofSpears))
    (bind _output_get_2 (Variables|Default|SetLength (Math|Random|RandomFloatinRange 35.0 (Variables|Default|GetMaxLength))))
    (bind _returnvalue_2 (Game|SpawnActorfromClass "/Game/Traps/SpearTrap/Spear_BP.Spear_BP_C" (Math|Transform|MakeTransform (+ (* (Variables|Default|GetForwardDirectionvector) _output_get_2) (Math|Vector|MakeVector (.x (Variables|Default|GetCasterLocation)) (.y (Variables|Default|GetCasterLocation)) (- (.z (Variables|Default|GetCasterLocation)) (Math|Random|RandomFloatinRange 4.5e+02 5.2e+02)))) (Math|Rotator|MakeRotator (+ (.roll (Math|Rotator|MakeRotfromZ (Variables|Default|GetForwardDirectionvector))) (Math|Random|RandomFloatinRange 3e+01 85.0)) (+ (.pitch (Math|Rotator|MakeRotfromZ (Variables|Default|GetForwardDirectionvector))) (Math|Random|RandomFloatinRange -1e+01 1e+01)) (.yaw (Math|Rotator|MakeRotfromZ (Variables|Default|GetForwardDirectionvector)))) "1.500000,1.500000,1.500000") "Undefined" 0 0))
    (Utilities|Array|Add (Variables|Default|GetSpears) _returnvalue_2))
  ;;[1 1 1] Rotate the Damage box according to the player's casted rotation and adjust the size of it dependend on the max length of farthest spear
  (Transformation|SetWorldRotation (Variables|Default|GetBox) (Math|Rotator|MakeRotator (.roll (Transformation|GetActorRotation (Variables|Default|Getpawn))) (.pitch (Transformation|GetActorRotation (Variables|Default|Getpawn))) (.yaw (Transformation|GetActorRotation (Variables|Default|Getpawn)))) false false)
  (Transformation|SetWorldLocation (Variables|Default|GetBox) (+ (Transformation|GetActorLocation) (* (Math|Vector|GetForwardVector (Variables|Default|GetBox)) (Variables|Default|GetMaxLength))) false false)
  (Transformation|SetWorldRotation _box_2 (Math|Rotator|MakeRotator (.roll _returnvalue) (.pitch _returnvalue) (.yaw (Math|Rotator|MakeRotfromZ (Variables|Default|GetForwardDirectionvector)))) false false)
  (Components|Box|SetBoxExtent (Variables|Default|GetBox) (Math|Vector|MakeVector (.x _boxextent) (Variables|Default|GetMaxLength) (.z _boxextent)) true)
  ;;[1 1 1] Animating spears
  (bind _accelaration (Timeline|SpearAcceleration PlayFromStart)
    (:Update
      (for _array_element_2 (Variables|Default|GetSpears)
        (Transformation|SetActorLocation _array_element_2 (+ (Transformation|GetActorLocation _array_element_2) (* (Transformation|GetActorUpVector _array_element_2) _accelaration)) false false)))
    (:Finished
      ;;[1 1 1] Apply the damage amount
      (bind (_damagegradient _startingheight) (CallFunction|CalculateDamageOperations))
      (Variables|Default|SetDamageGradient _damagegradient)
      (Variables|Default|SetDamageStartingHeight _startingheight)
      (bind _output_get_3 (Variables|Default|SetOverlappedActors (Collision|GetOverlappingActors (Variables|Default|GetBox) "/Game/Characters/AbstractCharacter.AbstractCharacter_C" :!class /Script/Engine.PrimitiveComponent)))
      (Variables|Default|Setindex (- (Utilities|Array|Length _output_get_3) 1))
      (for _index_2 (range 0 (Variables|Default|Getindex))
        (bind _asabstract_character (Utilities|Casting|CastToAbstractCharacter (Utilities|Array|Get(acopy) _output_get_3 _index_2)))
        (if (== (Variables|/Game/Characters/AbstractCharacter.AbstractCharacter_C|GetTeamNumber _asabstract_character) (Variables|Default|GetEnemyType))
          (if (not (== (Variables|Default|GetDamageGradient) 0.0))
            ;;;[1 1 1] Calculate damage [ (Y-C)/M=X ]
            (bind (_damage _minimum_damage) (CallFunction|CalculateDamage (Variables|Default|GetSlotLevel) (Variables|Default|GetPlayerIndex)))
            (bind _returnvalue_3 (Game|Damage|ApplyDamage _asabstract_character (Math|Float|Clamp(Float) (* _damage (Math|Float|Clamp(Float) (/ (Variables|Default|GetMaxLength) (Math|Vector|VectorLength (- (Transformation|GetActorLocation _asabstract_character) (Transformation|GetActorLocation)))) 0.0)) _minimum_damage _damage) (Game|GetPlayerController (Variables|Default|GetPlayerIndex)) self "/Game/GameData/Damages/DamageType_Physical.DamageType_Physical_C"))
            (Development|PrintString (Utilities|String|ToString(Float) _returnvalue_3))
            (else
              (bind _damage_2 (CallFunction|CalculateDamage (Variables|Default|GetSlotLevel) (Variables|Default|GetPlayerIndex)))
              (Game|Damage|ApplyDamage _asabstract_character _damage_2 (Game|GetPlayerController (Variables|Default|GetPlayerIndex)) self "/Game/GameData/Damages/DamageType_Physical.DamageType_Physical_C")))))
      ;;;[1 1 1] Clear the created spears
      (Utilities|FlowControl|Delay 3.0)
      (for _array_element_3 _spears
        (Actor|DestroyActor _array_element_3))
      (Utilities|Array|Clear _spears))))

(fn ConstructionScript
  (Variables|Default|SetCooldown 2e+01)
  (Variables|Default|SetXpGainAlternative 8.0)
  (Variables|Default|SetXpModifier 0.35)
  (Variables|Default|SetAbilityName "Spears of Dagon"))

(fn CalculateDamage
  (params (SlotLevel :type Integer) (PlayerIndex :type Integer))
  (bind _asknight_bp (Utilities|Casting|CastToKnight_BP (Game|Player|GetPlayerPawn PlayerIndex)))
  (bind _damage (Default|GetCalculatedDamage _asknight_bp))
  (return (Math|Float|Clamp(Float) (+ (+ _damage (* _damage (* SlotLevel 0.2))) (Math|Conversions|ToFloat(Integer) (Variables|/Game/Characters/PlayableCharacters/Knight_BP.Knight_BP_C|GetPlayerLevel _asknight_bp))) _damage 6e+01) (+ _damage (Math|Conversions|ToFloat(Integer) (Variables|/Game/Characters/PlayableCharacters/Knight_BP.Knight_BP_C|GetPlayerLevel _asknight_bp)))))

(fn CalculateDamageGradient
  (params (maxDamage :type Float%20%28single-precision%29) (Min%20Damage :type Float%20%28single-precision%29))
  (return (/ (- 0.0 (Variables|Default|GetMaxLength)) (- maxDamage Min%20Damage))))

(fn CalculateDamageFunctionHeight
  (params (DamageGradient :type Float%20%28single-precision%29))
  (return 0.0))

(fn CalculateDamageOperations
  (bind (_damage _minimum_damage) (CallFunction|CalculateDamage (Variables|Default|GetSlotLevel) (Variables|Default|GetPlayerIndex)))
  (bind _damagegradient (CallFunction|CalculateDamageGradient _damage _minimum_damage))
  (return _damagegradient (Math|Float|Absolute(Float) (* _damagegradient 0.0))))

(fn GetAbilityDescription
  (bind (_damage _minimum_damage) (CallFunction|CalculateDamage (Variables|Default|GetSlotLevel) (Variables|Default|GetPlayerIndex)))
  (LocalVariables|Setdmg _damage)
  (LocalVariables|SetMinDmg _minimum_damage)
  (if (CallFunction|IsReady)
    (LocalVariables|SetreadyState "Can activate")
    (else
      (LocalVariables|SetreadyState "On cooldown")))
  (return (Utilities|Text|FormatText "This ability has been tought by the Royal knight, Dagon. The spears comes straight from the ground in a straight towards the target, destroying everything in it's path.")))

(fn GetAbilityStatistics
  (bind (_damage _minimum_damage) (CallFunction|CalculateDamage (Variables|Default|GetSlotLevel) (Variables|Default|GetPlayerIndex)))
  (LocalVariables|Setdmg _damage)
  (LocalVariables|SetMinDmg _minimum_damage)
  (if (CallFunction|IsReady)
    (LocalVariables|SetreadyState "Can activate")
    (else
      (LocalVariables|SetreadyState "On cooldown")))
  (return (Utilities|Text|FormatText "Damage: {min} - {max} 
Radius: {radius} 
AoE type: Line 
Damage Type: Physical 
Cooldown: {ctime}s 
Cooldown upon acitivation: {cooldown}s 
Ready: {readiness}" (LocalVariables|GetMinDmg) (LocalVariables|Getdmg) (Variables|Default|GetMaxLength) (CallFunction|GetRemainingCooldownTime) (CallFunction|GetCooldown) (LocalVariables|GetreadyState))))