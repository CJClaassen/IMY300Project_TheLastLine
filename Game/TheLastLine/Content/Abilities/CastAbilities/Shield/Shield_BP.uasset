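; Shield cast ability that grants the Knight extra health and shows a shield sphere that follows the player.
; Activation, when ready, sets the Knight's ExtraHealthAmount from CalculateShield (currently a fixed value) and applies a dynamic material.
; A timer using the cooldown duration cancels the shield, clearing the health and hiding the sphere, as does DestroySelf.
; ShieldHit plays a timeline that drives the material's DamageTrigger parameter for hit feedback.
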(event Custom|CancelShield
  (bind _asknight_bp (Utilities|Casting|CastToKnight_BP (Game|Player|GetPlayerPawn (Variables|Default|GetPlayerIndex))))
  (Variables|/Game/Characters/PlayableCharacters/Knight_BP.Knight_BP_C|SetExtraHealthAmount _asknight_bp 0.0)
  (Default|UpdateonShieldDestroy _asknight_bp false)
  (Rendering|Material|SetMaterial (Variables|Default|GetSphere) 0 "/Game/UI/Gameplay/M_Invisible.M_Invisible")
  (Utilities|Time|ClearandInvalidateTimerbyHandle (Variables|Default|GetTimerByEvent)))

(event Custom|ShieldHit
  (if (not (Variables|Default|GetisPlaying))
    (Variables|Default|SetisPlaying true)
    (bind _shieldopacity (Timeline|ShieldTriger PlayFromStart)
      (:Update
        (Rendering|Material|SetScalarParameterValue (Variables|Default|GetDynamicShield) "DamageTrigger" _shieldopacity :!class /Script/Engine.MaterialInstanceDynamic))
      (:Finished
        (Variables|Default|SetisPlaying false)))))

(event EventBeginPlay
  (Variables|Default|SetCooldown 5e+01))

(event Collision|EventActorBeginOverlap
  (params (OtherActor :type Actor%20Object%20Reference))
  (|CallParentFunction OtherActor) ; This node is disabled and will not be called.\nDrag off pins to build functionality.
)

(event EventTick
  (params (DeltaSeconds :type Float%20%28single-precision%29))
  (if (Variables|Default|Getactivated)
    (Transformation|SetActorLocation (Transformation|GetActorLocation (Game|Player|GetPlayerPawn (Variables|Default|GetPlayerIndex))) false false)))

(event EventActivate
  (params (Location :type Vector :default "0, 0, 0") (Rotator :type Rotator :default "0, 0, 0") (PlayerIndex :type Integer) (Slot%20level :type Integer) (SlotIndex :type Integer))
  (|CallParentFunction Location Rotator PlayerIndex Slot%20level SlotIndex)
  (if (CallFunction|IsReady)
    (Variables|Default|Setactivated true)
    (Variables|Default|SetearlyActivation false)
    (bind _asknight_bp (Utilities|Casting|CastToKnight_BP (Game|Player|GetPlayerPawn PlayerIndex)))
    (bind _shieldamount (CallFunction|CalculateShield Slot%20level PlayerIndex))
    (Variables|/Game/Characters/PlayableCharacters/Knight_BP.Knight_BP_C|SetExtraHealthAmount _asknight_bp _shieldamount)
    (bind _returnvalue (Utilities|Time|SetTimerbyEvent (delegate Custom|CancelShield) (Variables|Default|GetCooldown)))
    (Variables|Default|SetTimerByEvent _returnvalue)
    (bind _returnvalue_2 (Rendering|Material|CreateDynamicMaterialInstance (Variables|Default|GetSphere) 0 "/Game/Abilities/CastAbilities/Shield/M_ShieldAbility.M_ShieldAbility" "None" :!class /Script/Engine.PrimitiveComponent))
    (Variables|Default|SetDynamicShield _returnvalue_2)))

(event EventDestroySelf
  (bind _asknight_bp (Utilities|Casting|CastToKnight_BP (Game|Player|GetPlayerPawn (Variables|Default|GetPlayerIndex))))
  (Variables|/Game/Characters/PlayableCharacters/Knight_BP.Knight_BP_C|SetExtraHealthAmount _asknight_bp 0.0)
  (Default|UpdateonShieldDestroy _asknight_bp false)
  (Rendering|Material|SetMaterial (Variables|Default|GetSphere) 0 "/Game/UI/Gameplay/M_Invisible.M_Invisible"))

(fn ConstructionScript
  (|CallParentFunction)
  (Variables|Default|SetAbilityName "Shield"))

(fn GetAbilityDescription
  (bind _shieldamount (CallFunction|CalculateShield (Variables|Default|GetSlotLevel) (Variables|Default|GetPlayerIndex)))
  (LocalVariables|Setdmg _shieldamount)
  (if (CallFunction|IsReady)
    (LocalVariables|SetreadyState "Can activate")
    (else
      (LocalVariables|SetreadyState "On cooldown")))
  (return (Utilities|Text|FormatText "Shield Amount: {dmg} 
Radius: N/A 
AoE type: Single unit 
Cooldown: {cooldown} s 
Ready: {readiness} 
 
Description: 
This is power of the Eagle. The Eagle was the name of the commanding force of which the knight wast part of before they were destroyed, except for one. " (LocalVariables|Getdmg) (Variables|Default|GetCooldown) (LocalVariables|GetreadyState))))

(fn CalculateShield
  (params (SlotLevel :type Integer) (PlayerIndex :type Integer))
  (return 25.0))