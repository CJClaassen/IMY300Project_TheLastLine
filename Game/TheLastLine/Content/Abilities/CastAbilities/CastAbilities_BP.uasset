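; Base actor for cast abilities, with empty Action, damage, initialization and description functions for children to override.
; Activate gates on IsReady (cooldown reduced by the component's CDR, or EarlyActivation), stamps the time, moves the actor, runs Action and reports to the game instance.
; A one-shot timer set for the remaining cooldown calls Validate, which notifies the player's controller of the slot's ability once ready.
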(event Custom|Validate
  (bind _playerindex (Variables|Default|GetPlayerIndex))
  (bind _returnvalue (Game|GetPlayerController _playerindex))
  (if (CallFunction|IsReady)
    (Utilities|IsValid _returnvalue
      (:Is%20Valid
        (bind _ascustom_player_controller_bp (Utilities|Casting|CastToCustomPlayerController_BP _returnvalue))
        (Default|NotifyonAbilityChange _ascustom_player_controller_bp (Variables|Default|GetSlotIndex) (Utilities|GetClass self))
        (Utilities|Time|ClearandInvalidateTimerbyHandle (Variables|Default|GetAbilityValidator))))))

(event Custom|NotifyOnGameplayUpdate
  (CallFunction|AbilityReadyCheck))

(event Custom|AbilityReadyCheck
  (bind _returnvalue (Utilities|Time|SetTimerbyEvent (delegate Custom|Validate) (- (CallFunction|GetCooldown) (- (Utilities|Time|GetGameTimeinSeconds) (Variables|Default|GetActivationTime)))))
  (Variables|Default|SetAbilityValidator _returnvalue)
  (CallFunction|Validate))

(event EventBeginPlay
  (bind _astop_down_game_mode (Utilities|Casting|CastToTopDownGameMode (Game|GetGameMode)))
  (Variables|Default|SetVolumeMultiplier (Variables|/Game/GameData/GameModes/TopDownGameMode.TopDownGameMode_C|GetSoundEffectVolumeMultiplier _astop_down_game_mode)))

(event Collision|EventActorBeginOverlap
  (params (OtherActor :type Actor%20Object%20Reference)))

(event EventTick
  (params (DeltaSeconds :type Float%20%28single-precision%29)))

(fn ConstructionScript)

(fn Activate
  (params (Location :type Vector) (Rotator :type Rotator) (PlayerIndex :type Integer) (Slot%20level :type Integer) (SlotIndex :type Integer))
  (if (CallFunction|IsReady)
    (Variables|Default|SetActivationTime (Utilities|Time|GetGameTimeinSeconds))
    (Transformation|SetActorLocationAndRotation Location Rotator)
    (CallFunction|Action Location Rotator PlayerIndex Slot%20level SlotIndex)
    (Variables|Default|SetSlotIndex SlotIndex)
    (Variables|Default|SetSlotLevel Slot%20level)
    (CallFunction|AbilityReadyCheck)
    (bind _astll_game_instance (Utilities|Casting|CastToTLL_GameInstance (Game|GetGameInstance)))
    (Default|AbilityActivated _astll_game_instance (Variables|Default|GetAbilityName))))

(fn IsReady
  (return (or (<= (CallFunction|GetCooldown) (- (Utilities|Time|GetGameTimeinSeconds) (Variables|Default|GetActivationTime))) (Variables|Default|GetearlyActivation))))

(fn Action
  (params (Location :type Vector) (Rotation :type Rotator) (PlayerIndex :type Integer) (Slot%20Level :type Integer) (SlotIndex :type Integer)))

(fn DestroySelf
  (Actor|DestroyActor))

(fn CalculateDamage
  (params (SlotLevel :type Integer) (PlayerIndex :type Integer))
  (return 0.0 0.0))

(fn InitializeProperties
  (params (Slot%20level :type Integer) (Holder :type Knight%20BP%20Object%20Reference)))

(fn GetAbilityDescription
  (return ""))

(fn GetCooldown
  (return (* (Variables|Default|GetCooldown) (- 1.0 (Variables|/Game/Characters/Components/PlayerSkillSet.PlayerSkillSet_C|GetAbilityCDR (Variables|Default|GetAbilityComponent))))))