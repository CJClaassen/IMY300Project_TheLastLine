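; Fireball ability projectile that detonates on overlapping items, characters, static meshes, props or objectives, with filters for its holder and golem trigger areas.
; PerformDamage applies radial falloff damage ignoring friendlies when upgraded, otherwise damages enemies inside DamageArea, doubled against objectives.
; Only the non-radial path totals character XP and feeds it, clamped and scaled, to the caster's ability slot.
; Explode then plays sound and particles, removes flight components and destroys the actor after a delay.
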(event OnComponentBeginOverlap(ProjectileSphere)
  (params (OverlappedComponent :type Primitive%20Component%20Object%20Reference) (OtherActor :type Actor%20Object%20Reference) (OtherComp :type Primitive%20Component%20Object%20Reference) (OtherBodyIndex :type Integer) (bFromSweep :type Boolean) (SweepResult :type Hit%20Result%20Structure%20%28by%20ref%29))
  (Utilities|IsValid (Variables|Default|GetHolder)
    (:Is%20Valid
      (bind _asitem_bp (Utilities|Casting|CastToItemBP OtherActor)
        (:then
          (Variables|Default|SetAttackedActor (Variables|/Game/Items/ItemBP.ItemBP_C|GetHolder _asitem_bp))
          (Utilities|IsValid (Variables|Default|GetAttackedActor) :!label _label
            (:Is%20Valid
              (if (not (== (Variables|Default|GetAttackedActor) (Variables|Default|GetHolder)))
                (CallFunction|PerformDamage)))))
        (:CastFailed
          (bind _asabstract_character (Utilities|Casting|CastToAbstractCharacter OtherActor)
            (:then
              (bind _asstone_golem_bp (Utilities|Casting|CastToStone_Golem_BP _asabstract_character)
                (:then
                  (Variables|Default|SetAttackedActor _asstone_golem_bp)
                  (if (not (or (== (Variables|/Game/Characters/NPC/NeutralCharacter/Stone_Golem/Stone_Golem_BP.Stone_Golem_BP_C|GetStompArea _asstone_golem_bp) OtherComp) (== OtherComp (Variables|/Game/Traps/ActivateAbleProps.ActivateAbleProps_C|GetActivationRadius (Variables|/Game/Characters/NPC/NeutralCharacter/Stone_Golem/Stone_Golem_BP.Stone_Golem_BP_C|GetGolemnActivator _asstone_golem_bp)))))
                    (goto _label)))
                (:CastFailed
                  (Variables|Default|SetAttackedActor _asabstract_character)
                  (goto _label))))
            (:CastFailed
              (Utilities|Casting|CastToStaticMeshActor OtherActor
                (:then
                  (CallFunction|PerformDamage))
                (:CastFailed
                  (bind _asactivate_able_props (Utilities|Casting|CastToActivateAbleProps OtherActor)
                    (:then
                      (Utilities|Casting|CastToGolemnActivator_BP _asactivate_able_props
                        (:CastFailed
                          (if (or (== OtherComp (Variables|/Game/Traps/ActivateAbleProps.ActivateAbleProps_C|GetActivationRadius _asactivate_able_props)) (== OtherComp (Variables|/Game/Traps/ActivateAbleProps.ActivateAbleProps_C|GetDamageRadius _asactivate_able_props)))
                            (CallFunction|PerformDamage)))))
                    (:CastFailed
                      (Utilities|Casting|CastToObjectiveActor_Copy OtherActor)
                      (CallFunction|PerformDamage))))))))))))

(event Custom|Explode
  (bind _fireparticlesystem (Variables|Default|GetFireParticleSystem))
  (bind _projectilesphere (Variables|Default|GetProjectileSphere))
  (CallFunction|PlaySound)
  (Utilities|IsValid _projectilesphere
    (:Is%20Valid
      (Components|DestroyComponent _projectilesphere))
    (:Is%20Not%20Valid
      _))
  (Utilities|IsValid _fireparticlesystem
    (:Is%20Valid
      (Components|DestroyComponent _fireparticlesystem))
    (:Is%20Not%20Valid
      _))
  (Utilities|IsValid (Variables|Default|GetSphere)
    (:Is%20Valid
      (Components|DestroyComponent (Variables|Default|GetSphere)))
    (:Is%20Not%20Valid
      _))
  (Components|Activation|Activate (Variables|Default|GetExplosionParticleSystem) false)
  (Components|Movement|StopMovementImmediately (Variables|Default|GetProjectileMovement))
  (Utilities|FlowControl|Delay 1.0)
  (Actor|DestroyActor))

(event Custom|PerformDamage
  (bind _self self)
  (bind _holder (Variables|Default|GetHolder))
  (bind _fireballdata (Variables|Default|GetFireBallData))
  (bind _fireballdata_2 (Variables|Default|GetFireBallData))
  (bind (_radialupgraded _basedamage _mindamage _innerradius _outerradius) (Utilities|Struct|BreakFireBallData _fireballdata))
  (bind (_radialupgraded_2 _basedamage_2 _mindamage_2 _innerradius_2 _outerradius_2 _xpmodifier _caster _slotindex) (Utilities|Struct|BreakFireBallData _fireballdata_2))
  (bind _returnvalue (Pawn|GetController _holder))
  (bind _teamnumber (Variables|/Game/Characters/AbstractCharacter.AbstractCharacter_C|GetTeamNumber _caster))
  (if _radialupgraded_2
    (Class|GameplayStatics|ApplyRadialDamagewithFalloff _basedamage _mindamage (Transformation|GetActorLocation) _innerradius _outerradius 1.0 "/Game/GameData/Damages/DamageType_Magic.DamageType_Magic_C" (CallFunction|GetAllFriendlies) self (Pawn|GetController (Variables|Default|GetHolder)) "ECC_GameTraceChannel1")
    (else
      (bind _output_get (Variables|Default|SetOverlappingActors (Collision|GetOverlappingActors (Variables|Default|GetDamageArea) "/Game/Characters/AbstractCharacter.AbstractCharacter_C" :!class /Script/Engine.PrimitiveComponent)))
      (for _array_element _output_get
        (bind _asabstract_character (Utilities|Casting|CastToAbstractCharacter _array_element))
        (if (!= _teamnumber (Variables|/Game/Characters/AbstractCharacter.AbstractCharacter_C|GetTeamNumber _asabstract_character))
          (Variables|Default|SetxpTotal (+ (Variables|/Game/Characters/AbstractCharacter.AbstractCharacter_C|GetXPGain _asabstract_character) (Variables|Default|GetxpTotal)))
          (Game|Damage|ApplyDamage _asabstract_character _basedamage_2 _returnvalue _self "/Game/GameData/Damages/DamageType_Magic.DamageType_Magic_C")))
      (bind _output_get_2 (Variables|Default|SetOverlappingActors (Collision|GetOverlappingActors (Variables|Default|GetDamageArea) "/Game/GameData/System/ObjectiveSystem/ObjectiveTarget/ObjectiveActor_Copy.ObjectiveActor_Copy_C" :!class /Script/Engine.PrimitiveComponent)))
      (for _array_element_2 _output_get_2
        (bind _asobjective_actor_copy (Utilities|Casting|CastToObjectiveActor_Copy _array_element_2))
        (if (!= _teamnumber (Variables|/Game/GameData/System/ObjectiveSystem/ObjectiveTarget/ObjectiveActor_Copy.ObjectiveActor_Copy_C|GetTeamNumber _asobjective_actor_copy))
          (Game|Damage|ApplyDamage _asobjective_actor_copy (* _basedamage_2 2.0) _returnvalue _self "/Game/GameData/Damages/DamageType_Magic.DamageType_Magic_C")))
      (Default|UpdateAbilitySlot _caster _slotindex (* _xpmodifier (Math|Conversions|ToFloat(Integer) (Math|Integer|Clamp(Integer) (Variables|Default|GetxpTotal) 0 50))))))
  (CallFunction|Explode))

(event Custom|PlaySound
  (Audio|PlaySoundatLocation (CallFunction|ChooseSound) (Transformation|GetActorLocation) "0, 0, 0" (* (Default|GetSoundEffectVolume (CallFunction|GetGameMode)) 2.0) 1.0 0.0 "/Game/Items/Staff/FireBallProjectile_Auttenation.FireBallProjectile_Auttenation" "/Game/Items/Sword/SwordHitConcurrency.SwordHitConcurrency" 0))

(event Custom|PerformDamageToComponent
  (params (Component :type Primitive%20Component%20Object%20Reference)))

(event EventBeginPlay
  (Variables|Default|SetCurrentTag 99999)
  (Variables|/Script/Engine.ProjectileMovementComponent|SetInitialSpeed (Variables|Default|GetProjectileMovement) 2e+03)
  (Utilities|FlowControl|Delay 0.5)
  (Development|PrintString "Hello"))

(event Collision|EventActorBeginOverlap
  (params (OtherActor :type Actor%20Object%20Reference)))

(event EventTick
  (params (DeltaSeconds :type Float%20%28single-precision%29)))

(fn ConstructionScript)

(fn GetDamage
  (bind _output_get (Variables|Default|SetDamage (Variables|/Game/Characters/AbstractCharacter.AbstractCharacter_C|GetDamage (Variables|Default|GetHolder))))
  (Development|PrintString (Utilities|String|Append (Utilities|String|MakeLiteralString "Damage : ") (Utilities|String|ToString(Float) _output_get)) true true "(R=1.000000,G=0.000000,B=0.000000,A=1.000000)" 1e+01))

(fn ChooseSound
  (return "/Game/Sound/Mage/Spells/Fireball_Explode_hit_Cue.Fireball_Explode_hit_Cue"))

(fn GetAllFriendlies
  (bind _outactors (Actor|GetAllActorsOfClass "/Game/Characters/AbstractCharacter.AbstractCharacter_C"))
  (for _array_element _outactors
    (if (== (Variables|Default|GetHolderTeam) (Variables|/Game/Characters/AbstractCharacter.AbstractCharacter_C|GetTeamNumber _array_element))
      (Utilities|Array|Add (LocalVariables|GetFriendlies) _array_element)))
  (return (LocalVariables|GetFriendlies)))