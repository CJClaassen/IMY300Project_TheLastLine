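; FireBall is a castable knight ability that launches a single-target magic fireball projectile along the player's forward vector.
; On activation it runs the parent logic and, if ready, spawns the projectile, assigns the knight as holder and passes it the damage.
; Damage scales the knight's calculated damage by slot level and ability power boost, though activation always passes slot level zero.
; It also builds description text showing damage, cooldown and readiness.
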(event EventBeginPlay
  (Variables|Default|SetCooldown 3e+01)
  (Variables|Default|SetAbilityName "FireBall"))

(event Collision|EventActorBeginOverlap
  (params (OtherActor :type Actor%20Object%20Reference)))

(event EventTick
  (params (DeltaSeconds :type Float%20%28single-precision%29)))

(event EventActivate
  (params (Location :type Vector :default "0, 0, 0") (Rotator :type Rotator :default "0, 0, 0") (PlayerIndex :type Integer) (Slot%20level :type Integer) (SlotIndex :type Integer))
  (bind _returnvalue (Game|Player|GetPlayerPawn PlayerIndex))
  ;[1 1 1] Creating the fireball
  (|CallParentFunction Location Rotator PlayerIndex Slot%20level SlotIndex)
  (Variables|Default|SetActivationTime (Utilities|Time|GetGameTimeinSeconds))
  (if (CallFunction|IsReady)
    (Variables|Default|SetearlyActivation false)
    (bind _returnvalue_2 (Game|SpawnActorfromClass "/Game/Abilities/CastAbilities/FireBall/FireballAbilityProjectile_BP.FireballAbilityProjectile_BP_C" (Math|Transform|MakeTransform Location (Math|Rotator|MakeRotfromZ (Transformation|GetActorForwardVector _returnvalue)) "0.300000,0.300000,0.300000") "AdjustIfPossibleButAlwaysSpawn" 0 0))
    (Utilities|IsValid _returnvalue_2
      (:Is%20Valid
        (bind _asknight_bp (Utilities|Casting|CastToKnight_BP _returnvalue))
        (bind _output_get (Variables|/Game/Items/ItemBP.ItemBP_C|SetHolder _returnvalue_2 _asknight_bp))
        (bind _damage (CallFunction|CalculateDamage 0 (Variables|/Game/Characters/AbstractCharacter.AbstractCharacter_C|GetplayerIndex _output_get)))
        (Variables|/Game/Abilities/CastAbilities/FireBall/FireballAbilityProjectile_BP.FireballAbilityProjectile_BP_C|SetFireBallData _returnvalue_2 (Utilities|Struct|MakeFireBallData false _damage)))
      (:Is%20Not%20Valid
        (Development|PrintString "Failed" true true "(R=1.000000,G=0.024638,B=0.000000,A=1.000000)" 15.0)))))

(fn ConstructionScript
  (Variables|Default|SetCooldown 5.0))

(fn CalculateDamage
  (params (SlotLevel :type Integer) (PlayerIndex :type Integer))
  (bind _asknight_bp (Utilities|Casting|CastToKnight_BP (Pawn|GetControlledPawn (Game|GetPlayerController PlayerIndex))))
  (bind _damage (Default|GetCalculatedDamage _asknight_bp))
  (return (+ (+ _damage (* _damage (* SlotLevel 0.1))) (* (+ _damage (* _damage (* SlotLevel 0.1))) (Variables|/Game/Characters/Components/PlayerSkillSet.PlayerSkillSet_C|GetAbilityPowerBoost (Variables|Default|GetAbilityComponent)))) 0.0))

(fn CalculateDamageRadius
  (bind _baseradius (Variables|Default|GetBaseRadius))
  (return _baseradius _baseradius))

(fn GetAbilityDescription
  (bind _damage (CallFunction|CalculateDamage (Variables|Default|GetSlotLevel) (Variables|Default|GetPlayerIndex)))
  (LocalVariables|Setdmg _damage)
  (if (CallFunction|IsReady)
    (LocalVariables|SetreadyState "Can activate")
    (else
      (LocalVariables|SetreadyState "On cooldown")))
  (return (Utilities|Text|FormatText "Damage: {dmg} 
Radius: N/A 
AoE type: Single unit 
Damage Type: magic 
Cooldown: {cooldown}s 
Ready: {readiness} 
 
Description: 
This is a deadly ability that thrown by knight upon to those that oppose him." (LocalVariables|Getdmg) (CallFunction|GetCooldown) (LocalVariables|GetreadyState))))