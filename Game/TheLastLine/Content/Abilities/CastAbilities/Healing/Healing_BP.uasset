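; Healing cast ability that restores the player Knight's health by a base amount plus slot level times player level.
; Activate applies the heal, then updates the ability slot with XP scaled by remaining missing health relative to the heal amount.
; It also enables a FollowPlayer flag that gates per-tick transform updates.
; A separate fadeOut event fades the mesh's opacity by timeline, then clears that flag.
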(event Custom|fadeOut
  (bind _opacity (Timeline|Fading PlayFromStart)
    (:Update
      (Rendering|Material|SetScalarParameterValueonMaterials (Variables|Default|GetStaticMesh) "Opacity" _opacity))
    (:Finished
      (Variables|Default|SetFollowPlayer false))))

(event EventBeginPlay
  (|CallParentFunction) ; This node is disabled and will not be called.\nDrag off pins to build functionality.
)

(event Collision|EventActorBeginOverlap
  (params (OtherActor :type Actor%20Object%20Reference))
  (|CallParentFunction OtherActor) ; This node is disabled and will not be called.\nDrag off pins to build functionality.
)

(event EventTick
  (params (DeltaSeconds :type Float%20%28single-precision%29))
  (bind _returnvalue (Transformation|GetActorTransform))
  (if (Variables|Default|GetFollowPlayer)
    (Transformation|SetActorTransform (Math|Transform|MakeTransform (Math|Vector|MakeVector (.x (.location _returnvalue)) (.y (.location _returnvalue)) (- (.z (.location _returnvalue)) 5e+01)) (.rotation _returnvalue) "1,1,1"))))

(event EventActivate
  (params (Location :type Vector :default "0, 0, 0") (Rotator :type Rotator :default "0, 0, 0") (PlayerIndex :type Integer) (Slot%20level :type Integer) (SlotIndex :type Integer))
  (Variables|Default|SetearlyActivation false)
  (Variables|Default|SetActivationTime (Utilities|Time|GetGameTimeinSeconds))
  (bind _asknight_bp (Utilities|Casting|CastToKnight_BP (Game|Player|GetPlayerPawn PlayerIndex)))
  (bind _added_health (CallFunction|CalculateHealth Slot%20level (Variables|/Game/Characters/PlayableCharacters/Knight_BP.Knight_BP_C|GetPlayerLevel _asknight_bp)))
  (Default|UpdateHealth _asknight_bp _added_health false)
  (Default|UpdateAbilitySlot _asknight_bp SlotIndex (* (/ (- (Variables|/Game/Characters/AbstractCharacter.AbstractCharacter_C|GetMaxHealth _asknight_bp) (Variables|/Game/Characters/AbstractCharacter.AbstractCharacter_C|GetHealth _asknight_bp)) _added_health) (Variables|Default|GetXpGainAlternative)))
  (Variables|Default|SetFollowPlayer true))

(fn ConstructionScript
  (Variables|Default|SetCooldown 6e+01)
  (Variables|Default|SetXpGainAlternative 8.0))

(fn CalculateHealth
  (params (SlotLevel :type Integer) (PlayerLevel :type Integer))
  (return (+ (Variables|Default|GetBaseHealth) (Math|Conversions|ToFloat(Integer) (* SlotLevel PlayerLevel)))))