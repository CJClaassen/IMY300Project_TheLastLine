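; Blade Rain sword ability actor that drops randomly scattered swords and deals magic damage to the enemy team.
; BeginPlay casts it at a hard-coded location, spawning tilted swords above that point.
; A timeline slides them along their forward vectors, then damages enemies overlapping the Sphere component.
; Only a hit starts the opacity fade that destroys everything; the whitelist feeds just an unconnected overlap-damage branch.
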(event EventBeginPlay
  ;[1 1 1] Adding all the friendly type of characters to the whitelist
  (Utilities|Array|Add (Variables|Default|GetObjectTypes) "ObjectTypeQuery3")
  (bind _outactors (Actor|GetAllActorsOfClass "/Game/Characters/AbstractCharacter.AbstractCharacter_C"))
  (for _array_element _outactors
    (if (!= (Variables|/Game/Characters/AbstractCharacter.AbstractCharacter_C|GetTeamNumber _array_element) (Variables|Default|GetEnemyType))
      (Utilities|Array|Add (Variables|Default|GetIgnoreActors) _array_element)))
  (CallFunction|Action "-270.000000,-20.000000,275.000000" "0, 0, 0"))

(event Collision|EventActorBeginOverlap
  (params (OtherActor :type Actor%20Object%20Reference))
  (|CallParentFunction OtherActor) ; This node is disabled and will not be called.\nDrag off pins to build functionality.
)

(event EventAction
  (params (Location :type Vector :default "0, 0, 0") (Rotation :type Rotator :default "0, 0, 0"))
  (bind _spawnradius (Variables|AbilityCasting|GetSpawnRadius))
  (bind _spawnradius_2 (Variables|AbilityCasting|GetSpawnRadius))
  ;[1 1 1] Upon activating the ability for BladeRain
  (Variables|Default|SetisActivated true)
  (bind _output_get (Variables|Default|SetCastedLocation (Math|Vector|MakeVector (.x Location) (.y Location) (.z Location))))
  ;;[1 1 1] Generating new location and rotations for the sword
  (for _index (range 0 (Variables|AbilityCasting|GetnumberOfSwords))
    (Variables|Default|SetNewSwordsLocation (Math|Vector|MakeVector (+ (.x _output_get) (Math|Random|RandomFloatinRange (* _spawnradius_2 -1.0) _spawnradius_2)) (+ (.y _output_get) (Math|Random|RandomFloatinRange (* _spawnradius -1.0) _spawnradius)) (+ (.z _output_get) (- (Variables|AbilityCasting|GetBaseHeight) (Math|Random|RandomFloatinRange -5e+02 2e+02)))))
    (Variables|Default|SetNewSwordRotation (Math|Rotator|MakeRotator (Math|Random|RandomFloatinRange 0.0 3.6e+02) (Math|Random|RandomFloatinRange -115.0 -75.0) (Math|Random|RandomFloatinRange -2e+01 2e+01)))
    (bind _ascustom_player_controller (Utilities|Casting|CastToCustomPlayerController (Game|GetPlayerController 0)))
    ;;[1 1 1] Creating the swords at their generated location and rotation
    (bind _returnvalue (Game|SpawnActorfromClass "/Game/Abilities/Sword/Sword_BP.Sword_BP_C" (Math|Transform|MakeTransform (Variables|Default|GetNewSwordsLocation) (Variables|Default|GetNewSwordRotation) (Math|Vector|MakeVector 0.2 0.2 0.2)) "AlwaysSpawn" self (Variables|/Game/Characters/PlayableCharacters/CustomPlayerController.CustomPlayerController_C|GetPlayerCharacter _ascustom_player_controller)))
    (Utilities|Array|Add (Variables|Default|GetSwordsList) _returnvalue)
    ;;[1 1 1] Animating the falling swords
    (bind _aceleration (Timeline|FallingAcceleration PlayFromStart)
      (:Update
        (for _array_element (Variables|Default|GetSwordsList)
          (if (> (.z (Transformation|GetWorldLocation (Variables|/Script/Engine.Actor|GetRootComponent _array_element))) (.z (Variables|Default|GetCastedLocation)))
            (Transformation|SetWorldLocation (Variables|/Script/Engine.Actor|GetRootComponent _array_element) (+ (Transformation|GetWorldLocation (Variables|/Script/Engine.Actor|GetRootComponent _array_element)) (* (Math|Vector|GetForwardVector (Variables|/Script/Engine.Actor|GetRootComponent _array_element)) _aceleration)) false false))))
      (:Finished
        ;;;[0.2826 0.5885 0.2027] Apply damage and fade out
        (for _array_element_2 (Collision|GetOverlappingActors (Variables|Default|GetSphere) "/Game/Characters/AbstractCharacter.AbstractCharacter_C" :!class /Script/Engine.PrimitiveComponent)
          (bind _asabstract_character (Utilities|Casting|CastToAbstractCharacter _array_element_2))
          (if (== (Variables|/Game/Characters/AbstractCharacter.AbstractCharacter_C|GetTeamNumber _asabstract_character) (Variables|Default|GetEnemyType))
            (Development|PrintString "Hello")
            (Game|Damage|ApplyDamage _asabstract_character (Variables|AbilityCasting|GetBaseDamage) (Game|GetPlayerController 0) self "/Game/GameData/Damages/DamageType_Magic.DamageType_Magic_C")
            (bind _opacity (Timeline|Opacity PlayFromStart)
              (:Update
                (for _array_element_3 (Variables|Default|GetSwordsList)
                  (Rendering|Material|SetScalarParameterValue (Variables|/Game/Abilities/Sword/Sword_BP.Sword_BP_C|GetSwordMaterial _array_element_3) "Opacity" _opacity :!class /Script/Engine.MaterialInstanceDynamic)))
              (:Finished
                (for _array_element_4 (Variables|Default|GetSwordsList)
                  (Actor|DestroyActor _array_element_4))
                (Actor|DestroyActor)))))))))

(fn ConstructionScript
  (|CallParentFunction))