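; WallCast_BP is a wall-casting ability that spawns a temporary Wall_BP at a given location and rotation.
; Action spawns the half-scale wall, copies MaxHealth into its Health, then drives its height with the WallRaise timeline.
; After raising, it waits WallLifeSpan and calls BreakDown to destroy the wall unless IsDestroyed is already set.
; BeginPlay triggers one cast at a hardcoded location.
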(event EventBeginPlay
  (CallFunction|Action "40.000000,900.000000,170.000000" "0, 0, 0"))

(event Collision|EventActorBeginOverlap
  (params (OtherActor :type Actor%20Object%20Reference)))

(event EventTick
  (params (DeltaSeconds :type Float%20%28single-precision%29)))

(event EventAction
  (params (Location :type Vector :default "0, 0, 0") (Rotation :type Rotator :default "0, 0, 0"))
  ;[1 1 1] Casting the wall ability
  ;;[1 1 1] Spawn and initialize the wall
  (bind _output_get (Variables|Default|SetcastedLocation Location))
  (bind _returnvalue (Game|SpawnActorfromClass "/Game/Abilities/Wall/Wall_BP.Wall_BP_C" (Math|Transform|MakeTransform _output_get Rotation "0.500000,0.500000,0.500000") "Undefined" 0 0))
  (bind _output_get_2 (Variables|Default|SetWall _returnvalue))
  (Variables|/Game/Abilities/Wall/Wall_BP.Wall_BP_C|SetHealth _output_get_2 (Variables|Default|GetMaxHealth))
  ;;[1 1 1] Raise the wall at the casted location
  (bind _raise (Timeline|WallRaise PlayFromStart)
    (:Update
      (Transformation|SetActorLocation (Variables|Default|GetWall) (Math|Vector|MakeVector (.x (Variables|Default|GetcastedLocation)) (.y (Variables|Default|GetcastedLocation)) (+ (.z (Variables|Default|GetcastedLocation)) _raise)) false false))
    (:Finished
      ;;[1 1 1] Check if the wall is still standing
      (Utilities|FlowControl|Delay (Variables|Default|GetWallLifeSpan))
      (if (not (Variables|Default|GetisDestroyed))
        (Variables|Default|SetisDestroyed true)
        (CallFunction|BreakDown)))))

(fn ConstructionScript
  (|CallParentFunction))

(fn BreakDown
  (Actor|DestroyActor (Variables|Default|GetWall)))