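; World pickup card for an ability, which spins in place until a player collects it.
; A timeline driven from Tick loops the card's yaw rotation.
; Overlapping the activation sphere registers the card on the character's custom player controller and shows a "Pick up" notification with the ability name; leaving clears both.
; A helper function maps ability classes to display names.
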(event OnComponentBeginOverlap(ActivatableSphere)
  (params (OverlappedComponent :type Primitive%20Component%20Object%20Reference) (OtherActor :type Actor%20Object%20Reference) (OtherComp :type Primitive%20Component%20Object%20Reference) (OtherBodyIndex :type Integer) (bFromSweep :type Boolean) (SweepResult :type Hit%20Result%20Structure%20%28by%20ref%29))
  ;[1 1 1] When the player is in range
  (bind _asabstract_character (Utilities|Casting|CastToAbstractCharacter OtherActor))
  (Utilities|IsValid (Variables|/Game/Characters/AbstractCharacter.AbstractCharacter_C|GetCharacterController _asabstract_character)
    (:Is%20Valid
      ;;[1 1 1] Linking ability type to the player controller and notifies the controller
      (bind _ascustom_player_controller_bp (Utilities|Casting|CastToCustomPlayerController_BP (Variables|/Game/Characters/AbstractCharacter.AbstractCharacter_C|GetCharacterController _asabstract_character)))
      (Variables|/Game/Controllers/PlayerControllers/CustomPlayerController_BP.CustomPlayerController_BP_C|SetAbilityCard _ascustom_player_controller_bp self)
      (Default|NotifyOfInteraction _ascustom_player_controller_bp "Pick up " (Variables|Default|GetAbilityName)))))

(event OnComponentEndOverlap(ActivatableSphere)
  (params (OverlappedComponent :type Primitive%20Component%20Object%20Reference) (OtherActor :type Actor%20Object%20Reference) (OtherComp :type Primitive%20Component%20Object%20Reference) (OtherBodyIndex :type Integer))
  (bind _asabstract_character (Utilities|Casting|CastToAbstractCharacter OtherActor))
  (Utilities|IsValid (Variables|/Game/Characters/AbstractCharacter.AbstractCharacter_C|GetCharacterController _asabstract_character)
    (:Is%20Valid
      (bind _ascustom_player_controller_bp (Utilities|Casting|CastToCustomPlayerController_BP (Variables|/Game/Characters/AbstractCharacter.AbstractCharacter_C|GetCharacterController _asabstract_character)))
      (Variables|/Game/Controllers/PlayerControllers/CustomPlayerController_BP.CustomPlayerController_BP_C|SetAbilityCard _ascustom_player_controller_bp 0)
      (Default|RemoveInteractionNotification _ascustom_player_controller_bp))))

(event EventBeginPlay
  (Variables|Default|SetRotation (Transformation|GetWorldRotation (Variables|Default|GetCard))))

(event Collision|EventActorBeginOverlap
  (params (OtherActor :type Actor%20Object%20Reference)))

(event EventTick
  (params (DeltaSeconds :type Float%20%28single-precision%29))
  (bind _rotation (Variables|Default|GetRotation))
  (if (not (Variables|Default|GetisFinished))
    ;[1 1 1] Spinning rotation
    (bind _yaw_z__rotation (Timeline|AbilityRotation Play)
      (:Update
        (Transformation|SetWorldRotation (Variables|Default|GetCard) (Math|Rotator|MakeRotator (.roll _rotation) (.pitch _rotation) _yaw_z__rotation) false false))
      (:Finished
        (Variables|Default|SetisFinished true)))
    (else
      (Variables|Default|SetisFinished false)
      (Timeline|AbilityRotation PlayFromStart))))

(fn ConstructionScript)

(fn ClasstoName
  (params (AbilityType :type Cast%20Abilities%20BP%20Class%20Reference))
  (bind _returnvalue (Utilities|GetClassDisplayName AbilityType))
  (switch string _returnvalue
    (:Default
      (Development|PrintString _returnvalue))
    (:BladeRain_Cast_BP_C
      (Variables|Default|SetAbilityName "Blade Rain"))
    (:FireBall_BP_C
      (Variables|Default|SetAbilityName "Fire Blast"))
    (:Impalement_BP_C
      (Variables|Default|SetAbilityName "Impalement"))
    (:WallCast_BP_C
      (Variables|Default|SetAbilityName "Wall Rise"))))