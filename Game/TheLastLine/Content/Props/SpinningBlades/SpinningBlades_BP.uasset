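; Purchasable spinning blade trap that players activate with points to damage characters.
; Box overlap shows the player controller an interaction prompt with affordability and registers the trap as PropInRange.
; Activate checks points, cooldown and active state, deducts the cost, then a timeline yaws the blade and clears the active flag when finished.
; Box1 overlaps deal physical damage while active; ActivatedTime, used by the cooldown check, is never set here.
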(event OnComponentBeginOverlap(Box)
  (params (OverlappedComponent :type Primitive%20Component%20Object%20Reference) (OtherActor :type Actor%20Object%20Reference) (OtherComp :type Primitive%20Component%20Object%20Reference) (OtherBodyIndex :type Integer) (bFromSweep :type Boolean) (SweepResult :type Hit%20Result%20Structure%20%28by%20ref%29))
  ;[1 0.2702 0.3] Notify the player is overlapping triggerbox (Needs completion)
  (bind _asabstract_character (Utilities|Casting|CastToAbstractCharacter OtherActor))
  (bind _ascustom_player_controller (Utilities|Casting|CastToCustomPlayerController (Variables|/Game/Characters/AbstractCharacter.AbstractCharacter_C|GetCharacterController _asabstract_character)))
  (Default|DisplayInteraction _ascustom_player_controller (>= (Variables|/Game/Characters/AbstractCharacter.AbstractCharacter_C|GetPoints _asabstract_character) (Variables|Default|GetActivationCost)) "F by BladeSpinner")
  (Variables|/Game/Characters/PlayableCharacters/CustomPlayerController.CustomPlayerController_C|SetPropInRange _ascustom_player_controller self))

(event OnComponentBeginOverlap(Box1)
  (params (OverlappedComponent :type Primitive%20Component%20Object%20Reference) (OtherActor :type Actor%20Object%20Reference) (OtherComp :type Primitive%20Component%20Object%20Reference) (OtherBodyIndex :type Integer) (bFromSweep :type Boolean) (SweepResult :type Hit%20Result%20Structure%20%28by%20ref%29))
  ;[1 1 1] When blade touches character
  (if (Variables|Default|GetisActivated)
    (bind _asabstract_character (Utilities|Casting|CastToAbstractCharacter OtherActor))
    (Game|Damage|ApplyDamage _asabstract_character 1e+02 0 self "/Game/GameData/Damages/DamageType_Physical.DamageType_Physical_C")))

(event EventBeginPlay)

(event Collision|EventActorBeginOverlap
  (params (OtherActor :type Actor%20Object%20Reference)))

(event EventTick
  (params (DeltaSeconds :type Float%20%28single-precision%29)))

(event EventActivate
  (params (Player :type Abstract%20Character%20Object%20Reference))
  (bind _activationcost (Variables|Default|GetActivationCost))
  ;[1 1 1] Spinning blade
  ;;[1 0.6533 0.06447] Validate activation
  (if (>= (Variables|/Game/Characters/AbstractCharacter.AbstractCharacter_C|GetPoints Player) _activationcost)
    (if (CallFunction|IsReady)
      (if (not (Variables|Default|GetisActivated))
        (Variables|Default|SetisActivated true)
        (Variables|/Game/Characters/AbstractCharacter.AbstractCharacter_C|SetPoints Player (- (Variables|/Game/Characters/AbstractCharacter.AbstractCharacter_C|GetPoints Player) _activationcost))
        ;;[0.4102 1 0.2654] Spinning Animation
        (bind _bladerotation (Timeline|Timeline_0 PlayFromStart)
          (:Update
            (Transformation|SetWorldRotation (Variables|Default|Getblade) (Math|Rotator|MakeRotator 0.0 0.0 _bladerotation) false false))
          (:Finished
            (Variables|Default|SetisActivated false)))))))

(fn ConstructionScript
  (|CallParentFunction))

(fn IsReady
  (return (<= (Variables|Default|GetcooldownDuration) (- (Utilities|Time|GetGameTimeinSeconds) (Variables|Default|GetActivatedTime)))))