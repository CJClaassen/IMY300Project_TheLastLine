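; Devastator is a player-activated pounder trap, with a cooldown and activation cost, that slams and damages characters within its radius.
; Activate runs a Delay-timed sequence of animations, gear and impact sounds, and mesh collision changes, then resets.
; On impact, each overlapping AbstractCharacter takes physical damage inversely proportional to its distance from the trap, clamped to a maximum.
; An alternative radial-damage-with-falloff call is left disconnected.
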(event Custom|PlayGoUpSound
  (Utilities|IsValid (Variables|Default|GetGearSound)
    (:Is%20Valid
      _)
    (:Is%20Not%20Valid
      (bind _returnvalue (AddComponent|AddAudioComponent false))
      (Variables|Default|SetGearSound _returnvalue)
      (Audio|Components|Audio|Stop _returnvalue)))
  (Audio|Components|Audio|SetSound (Variables|Default|GetGearSound) "/Game/Sound/Pounder/GearsMove_Cue.GearsMove_Cue")
  (Transformation|SetWorldLocation (Variables|Default|GetGearSound) (Transformation|GetActorLocation) false false)
  (Audio|Components|Audio|SetVolumeMultiplier (Variables|Default|GetGearSound) (* (Default|GetSoundEffectVolume (CallFunction|GetGameMode)) 1.0) :!class /Script/Engine.AudioComponent)
  (Audio|Components|Audio|Play (Variables|Default|GetGearSound) 0.0))

(event Custom|StopGoUpSound
  (Audio|Components|Audio|Stop (Variables|Default|GetGearSound)))

(event EventBeginPlay
  (|CallParentFunction)
  (Variables|Default|SetTrapName "Devastator")
  (Variables|Default|SetbCanBeDamaged true)
  (Variables|/Script/Engine.PrimitiveComponent|SetbGenerateOverlapEvents (Variables|Default|GetDamage%20radius') false))

(event Collision|EventActorBeginOverlap
  (params (OtherActor :type Actor%20Object%20Reference)))

(event EventTick
  (params (DeltaSeconds :type Float%20%28single-precision%29))
  ;[1 1 1] Swap from blue to green material when ready
  (|CallParentFunction DeltaSeconds))

(event EventActivate
  (params (PlayerIndex :type Integer))
  ;[1 1 1] Handling prop activation
  (|CallParentFunction PlayerIndex)
  (if (CallFunction|IsReady)
    (Variables|Default|SetEarlyActivate false)
    (Variables|Default|SetActivatedTime (Utilities|Time|GetGameTimeinSeconds))
    ;;[1 1 1] Activation Animation
    (Components|Animation|PlayAnimation (Variables|Default|GetSkeletalMesh) "/Game/Traps/Devastator/Assets/Devastator_ActivateAnim.Devastator_ActivateAnim" false)
    (Utilities|FlowControl|Delay 0.2)
    (CallFunction|PlayGoUpSound)
    (Utilities|FlowControl|Delay 0.45)
    (CallFunction|StopGoUpSound)
    (Utilities|FlowControl|Delay 0.225)
    (Collision|SetCollisionEnabled (Variables|Default|GetSkeletalMesh) "PhysicsOnly")
    (Utilities|FlowControl|Delay 0.45)
    (Audio|PlaySoundatLocation "/Game/Sound/Pounder/PounderImpact_Cue.PounderImpact_Cue" (Transformation|GetActorLocation) "0, 0, 0" (* (Default|GetSoundEffectVolume (CallFunction|GetGameMode)) 4.0) 1.0 0.0 0 0 0)
    (CallFunction|PlayGoUpSound)
    ;;[1 1 1] Applying the damage
    (bind _output_get (Variables|Default|SetOverlapped%20actors (Collision|GetOverlappingActors (Variables|Default|GetDamageRadius) "/Game/Characters/AbstractCharacter.AbstractCharacter_C" :!class /Script/Engine.PrimitiveComponent)))
    (for _array_element _output_get
      (Game|Damage|ApplyDamage _array_element (Math|Float|Clamp(Float) (* 1e+02 (/ 1.0 (/ (Math|Vector|VectorLength (- (Transformation|GetActorLocation _array_element) (Transformation|GetActorLocation))) (Variables|/Script/Engine.SphereComponent|GetSphereRadius (Variables|Default|GetDamage%20radius'))))) 0.0 7.5e+02) 0 self "/Game/GameData/Damages/DamageType_Physical.DamageType_Physical_C"))
    ;;[1 1 1] ResetAnimation
    (Components|Animation|PlayAnimation (Variables|Default|GetSkeletalMesh) "/Game/Traps/Devastator/Assets/Devastator_ResetAnim.Devastator_ResetAnim" false)
    (Utilities|FlowControl|Delay 1.0)
    (Collision|SetCollisionEnabled (Variables|Default|GetSkeletalMesh) "QueryAndPhysics")
    (Utilities|FlowControl|Delay 1.2)
    (CallFunction|StopGoUpSound)
    (else
      (Development|PrintString "Still in cooldown"))))

(fn ConstructionScript
  (|CallParentFunction)
  (Variables|Default|SetCooldownTime 9e+01)
  (Variables|Default|SetActivationCost 350))

(fn SetObjectLocationRotation
  (params (Object :type Static%20Mesh%20Component%20Object%20Reference) (Location :type Vector) (Rotation :type Rotator))
  (bind _output_get (LocalVariables|SetStaticMesh Object))
  (Transformation|SetWorldLocationAndRotation _output_get Location Rotation false false))

(fn GetGameMode
  (bind _astop_down_game_mode (Utilities|Casting|CastToTopDownGameMode (Game|GetGameMode)))
  (return _astop_down_game_mode))