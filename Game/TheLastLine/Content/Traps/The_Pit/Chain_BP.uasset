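; Chain trap actor for The Pit that shoots a hook forward, drags a caught character back and kills it.
; ChainShoot plays the chain sound, waits a random delay, then drives movement with a shoot timeline followed by a pull timeline.
; HookPoint overlap hooks one not-yet-hooked AbstractCharacter, cutting the shot short.
; When the pull finishes, the victim takes lethal physical damage and the chain snaps back to its BeginPlay location.
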(event OnComponentBeginOverlap(HookPoint)
  (params (OverlappedComponent :type Primitive%20Component%20Object%20Reference) (OtherActor :type Actor%20Object%20Reference) (OtherComp :type Primitive%20Component%20Object%20Reference) (OtherBodyIndex :type Integer) (bFromSweep :type Boolean) (SweepResult :type Hit%20Result%20Structure%20%28by%20ref%29))
  (Utilities|IsValid (Variables|Default|GetHookedActor)
    (:Is%20Not%20Valid
      (bind _asabstract_character (Utilities|Casting|CastToAbstractCharacter OtherActor))
      (Utilities|IsValid (Variables|/Game/Characters/AbstractCharacter.AbstractCharacter_C|GetChainHook _asabstract_character)
        (:Is%20Not%20Valid
          (bind _output_get (Variables|Default|SetHookedActor _asabstract_character))
          (Default|SetHooked _asabstract_character (Variables|Default|GetHookPoint))
          (Audio|PlaySoundatLocation "/Game/Sound/Stab/StabIn_Cue.StabIn_Cue" (Transformation|GetActorLocation _output_get) "0, 0, 0" (* (Default|GetSoundEffectVolume (CallFunction|GetGameMode)) 4.0) 1.0 0.0 0 "/Game/Sound/Stab/Chains_Concurrency.Chains_Concurrency" 0)
          (Variables|Default|SetisHooked true))))))

(event Custom|ChainShoot
  (params (EventInstigator :type Controller%20Object%20Reference) (DamageCauser :type Actor%20Object%20Reference))
  (CallFunction|PlayChainSound)
  (Utilities|FlowControl|Delay (Math|Random|RandomFloatinRange 0.4 0.7))
  (bind _shootspeed (Timeline|ShootAnimation PlayFromStart)
    (:Update
      (Transformation|SetActorLocation (+ (* (Transformation|GetActorForwardVector) _shootspeed) (Transformation|GetActorLocation)) false false)
      (if (Variables|Default|GetisHooked)
        (Utilities|FlowControl|Sequence
          (:then_0
            (Timeline|ShootAnimation Stop))
          (:then_1
            (Audio|Components|Audio|Stop (Variables|Default|GetChainSound) :!label _label)
            (Audio|Components|Audio|Stop (Variables|Default|GetChainSound))
            (Utilities|FlowControl|Delay 0.2)
            (Audio|Components|Audio|Play (Variables|Default|GetChainSound) 0.5)
            (bind _newtrack_0 (Timeline|PullAnimation PlayFromStart)
              (:Update
                (Transformation|SetActorLocation (+ (* (Transformation|GetActorForwardVector) _newtrack_0) (Transformation|GetActorLocation)) false false))
              (:Finished
                (if (Variables|Default|GetisHooked)
                  (Variables|Default|SetisHooked false)
                  (Game|Damage|ApplyDamage (Variables|Default|GetHookedActor) 1e+05 EventInstigator DamageCauser "/Game/GameData/Damages/DamageType_Physical.DamageType_Physical_C"))
                (Transformation|SetActorLocation (Variables|Default|GetFixedLocation) false false)
                (Variables|Default|SetHookedActor 0)
                (Audio|Components|Audio|Stop (Variables|Default|GetChainSound))))))))
    (:Finished
      (goto _label))))

(event Custom|PlayChainSound
  (bind _chainsound (Variables|Default|GetChainSound))
  (Audio|Components|Audio|SetSound (Variables|Default|GetChainSound) "/Game/Sound/Traps/Chains/The_Pit_Cue.The_Pit_Cue")
  (Transformation|SetWorldLocation _chainsound (Transformation|GetActorLocation) false false)
  (Audio|Components|Audio|SetVolumeMultiplier _chainsound (Default|GetSoundEffectVolume (CallFunction|GetGameMode)) :!class /Script/Engine.AudioComponent)
  (Audio|Components|Audio|Play _chainsound 0.5))

(event EventBeginPlay
  (bind _returnvalue (AddComponent|AddAudioComponent false))
  (bind _output_get (Variables|Default|SetChainSound _returnvalue))
  (Audio|Components|Audio|Stop _output_get)
  (Variables|Default|SetFixedLocation (Transformation|GetActorLocation)))

(event Collision|EventActorBeginOverlap
  (params (OtherActor :type Actor%20Object%20Reference)))

(event EventTick
  (params (DeltaSeconds :type Float%20%28single-precision%29)))

(fn ConstructionScript)

(fn GetGameMode
  (bind _astop_down_game_mode (Utilities|Casting|CastToTopDownGameMode (Game|GetGameMode)))
  (return _astop_down_game_mode))