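; FeedingTrap_BP is "The Pit", a player-activated trap that fires chains, with a cooldown and no activation cost.
; On activation, if ready, it records the time, waits briefly, then calls ChainShoot on its three Chain_BP child actors, passing the activating player's controller as instigator and itself as damage causer.
; The construction script positions the activate-key widget at an offset from the actor's location.
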(event EventBeginPlay
  (|CallParentFunction)
  (Variables|Default|SetTrapName "The Pit")
  (Variables|Default|SetCooldownTime 3e+01)
  (Variables|Default|SetActivationCost 0)
  (Variables|Default|SetChainArray (Utilities|Array|MakeArray (Variables|Default|GetChildActor1) (Variables|Default|GetChildActor) (Variables|Default|GetChildActor2))))

(event EventActivate
  (params (PlayerIndex :type Integer))
  (|CallParentFunction PlayerIndex)
  (if (CallFunction|IsReady)
    (Variables|Default|SetActivatedTime (Utilities|Time|GetGameTimeinSeconds))
    (Utilities|FlowControl|Delay 0.5)
    (for _array_element (Variables|Default|GetChainArray)
      (bind _aschain_bp (Utilities|Casting|CastToChain_BP (Variables|/Script/Engine.ChildActorComponent|GetChildActor _array_element)))
      (Default|ChainShoot _aschain_bp (Game|GetPlayerController (Variables|Default|GetPlayerIndex)) self))))

(fn ConstructionScript
  (|CallParentFunction)
  (Transformation|SetWorldLocation (Variables|Default|GetActivateKeyWidget) (+ (Transformation|GetActorLocation) (Variables|Default|GetWidgetLocation)) false false))