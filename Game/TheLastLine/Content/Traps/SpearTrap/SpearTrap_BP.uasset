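; Player-activated spear trap that deals physical damage to characters inside its damage box, with a cooldown between uses.
; Overlapping the activation box registers it as the knight controller's prop in range and shows a prompt with the point cost.
; Activation waits briefly, pushes child spear actors along world X by timeline, applies damage, then retracts them with a second timeline.
; Tick swaps the activation radius material to indicate readiness.
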(event OnComponentBeginOverlap(ActivateBox)
  (params (OverlappedComponent :type Primitive%20Component%20Object%20Reference) (OtherActor :type Actor%20Object%20Reference) (OtherComp :type Primitive%20Component%20Object%20Reference) (OtherBodyIndex :type Integer) (bFromSweep :type Boolean) (SweepResult :type Hit%20Result%20Structure%20%28by%20ref%29))
  ;[1 1 1] Notifies the player in range of activation
  (bind _asknight_bp (Utilities|Casting|CastToKnight_BP OtherActor))
  ;;[1 1 1] Player in Range
  (Utilities|IsValid (Variables|/Game/Characters/AbstractCharacter.AbstractCharacter_C|GetCharacterController _asknight_bp)
    (:Is%20Valid
      (bind _ascustom_player_controller_bp (Utilities|Casting|CastToCustomPlayerController_BP (Variables|/Game/Characters/AbstractCharacter.AbstractCharacter_C|GetCharacterController _asknight_bp)))
      (Default|NotifyOfInteraction _ascustom_player_controller_bp "Activate spike trap" (Utilities|String|Append (Utilities|String|ToString(Integer) (Variables|Default|GetActivationCost)) " Pts"))
      (Variables|/Game/Controllers/PlayerControllers/CustomPlayerController_BP.CustomPlayerController_BP_C|SetPropInRange _ascustom_player_controller_bp self))
    (:Is%20Not%20Valid
      (bind _ascustom_player_controller_bp_2 (Utilities|Casting|CastToCustomPlayerController_BP (Game|GetPlayerController (Variables|/Game/Characters/AbstractCharacter.AbstractCharacter_C|GetplayerIndex _asknight_bp))))
      (Default|NotifyOfInteraction _ascustom_player_controller_bp_2 "Activate spike trap" (Utilities|String|Append (Utilities|String|ToString(Integer) (Variables|Default|GetActivationCost)) " Pts"))
      (Variables|/Game/Controllers/PlayerControllers/CustomPlayerController_BP.CustomPlayerController_BP_C|SetPropInRange _ascustom_player_controller_bp_2 self))))

(event OnComponentEndOverlap(ActivateBox)
  (params (OverlappedComponent :type Primitive%20Component%20Object%20Reference) (OtherActor :type Actor%20Object%20Reference) (OtherComp :type Primitive%20Component%20Object%20Reference) (OtherBodyIndex :type Integer))
  ;[1 1 1] Notifies the player in range of activation
  ;;[1 1 1] Player out of range
  (bind _asknight_bp (Utilities|Casting|CastToKnight_BP OtherActor))
  (bind _ascustom_player_controller_bp (Utilities|Casting|CastToCustomPlayerController_BP (Variables|/Game/Characters/AbstractCharacter.AbstractCharacter_C|GetCharacterController _asknight_bp))
    (:then
      (Variables|/Game/Controllers/PlayerControllers/CustomPlayerController_BP.CustomPlayerController_BP_C|SetPropInRange _ascustom_player_controller_bp 0)
      (Default|RemoveInteractionNotification _ascustom_player_controller_bp))
    (:CastFailed
      (bind _ascustom_player_controller_bp_2 (Utilities|Casting|CastToCustomPlayerController_BP (Game|GetPlayerController (Variables|/Game/Characters/AbstractCharacter.AbstractCharacter_C|GetplayerIndex _asknight_bp))))
      (Default|RemoveInteractionNotification _ascustom_player_controller_bp_2))))

(event EventBeginPlay)

(event Collision|EventActorBeginOverlap
  (params (OtherActor :type Actor%20Object%20Reference)))

(event EventTick
  (params (DeltaSeconds :type Float%20%28single-precision%29))
  ;[1 1 1] Swap from blue to green material when ready
  (if (CallFunction|IsReady)
    (if (not (Variables|Default|GethasAdded))
      (Variables|Default|SethasAdded true)
      (Rendering|Material|SetMaterial (Variables|Default|GetActivationRadius) 0 "/Game/GameData/VisualProps/RadiusIndicator/MInstance_ActivatingIndicator.MInstance_ActivatingIndicator"))
    (elif (Variables|Default|GetisActivated)
      (Rendering|Material|SetMaterial (Variables|Default|GetActivationRadius) 0 "/Game/GameData/VisualProps/RadiusIndicator/MInstance_AbilityIndicator.MInstance_AbilityIndicator")
      (Variables|Default|SethasAdded false))))

(event EventActivate
  (params (PlayerIndex :type Integer))
  ;[1 1 1] When the trap is activated
  (if (CallFunction|IsReady)
    (Variables|Default|SetActivatedTime (Utilities|Time|GetGameTimeinSeconds))
    (Utilities|FlowControl|Delay 0.5)
    (Variables|Default|SetisActivated true)
    ;;[1 1 1] Handle animation
    (bind _x_position (Timeline|UpdateLocation PlayFromStart)
      (:Update
        (for _array_element (Variables|EventVariables|GetSpears)
          (Transformation|SetActorLocation _array_element (Math|Vector|MakeVector (+ (.x (Transformation|GetActorLocation _array_element)) _x_position) (.y (Transformation|GetActorLocation _array_element)) (.z (Transformation|GetActorLocation _array_element))) false false)))
      (:Finished
        ;;[1 1 1] Apply damage to the overlapping abstract characters
        (for _array_element_2 (Collision|GetOverlappingActors (Variables|Default|GetDamageBox) "/Game/Characters/AbstractCharacter.AbstractCharacter_C" :!class /Script/Engine.PrimitiveComponent)
          (Game|Damage|ApplyDamage _array_element_2 (Variables|Default|GetBaseDamage) 0 0 "/Game/GameData/Damages/DamageType_Physical.DamageType_Physical_C"))
        ;;[1 1 1] Reset Trap animation
        (Utilities|FlowControl|Delay 2.0)
        (bind _x_position_2 (Timeline|Timeline_0 ReverseFromEnd)
          (:Update
            (for _array_element_3 (Variables|EventVariables|GetSpears)
              (Transformation|SetActorLocation _array_element_3 (Math|Vector|MakeVector (- (.x (Transformation|GetActorLocation _array_element_3)) _x_position_2) (.y (Transformation|GetActorLocation _array_element_3)) (.z (Transformation|GetActorLocation _array_element_3))) false false))))))
    (else
      (Development|PrintString "Still in cooldown"))))

(fn ConstructionScript
  (Variables|EventVariables|SetSpears (Actor|GetAllChildActors true)))