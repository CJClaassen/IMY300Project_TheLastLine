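; Trap prop that lets a Knight activate a linked Stone Golemn, which is assigned through LinkToGolemn.
; While the golem is inactive, trigger overlaps show or clear a prompt with its point cost on that player's controller and set or clear PropInRange.
; Activate wakes the golem and clears EarlyActivate.
; Tick swaps the activation radius material by readiness, and construction sets the cooldown and zeroes damage-radius emission.
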(event OnComponentBeginOverlap(TriggerRadius)
  (params (OverlappedComponent :type Primitive%20Component%20Object%20Reference) (OtherActor :type Actor%20Object%20Reference) (OtherComp :type Primitive%20Component%20Object%20Reference) (OtherBodyIndex :type Integer) (bFromSweep :type Boolean) (SweepResult :type Hit%20Result%20Structure%20%28by%20ref%29))
  (bind _stonegolemn (Variables|Default|GetStoneGolemn))
  (Utilities|IsValid _stonegolemn
    (:Is%20Valid
      (if (not (Variables|/Game/Characters/NPC/NeutralCharacter/StoneGolemn/Blueprint/StoneGolemn_BP.StoneGolemn_BP_C|GetisActivated _stonegolemn))
        (bind _asknight_bp (Utilities|Casting|CastToKnight_BP OtherActor))
        (bind _ascustom_player_controller_bp (Utilities|Casting|CastToCustomPlayerController_BP (Game|GetPlayerController (Variables|/Game/Characters/AbstractCharacter.AbstractCharacter_C|GetplayerIndex _asknight_bp))))
        (Default|NotifyOfInteraction _ascustom_player_controller_bp "Activate Stone Golemn " (Utilities|String|Append (Utilities|String|ToString(Integer) (Variables|/Game/Characters/NPC/NeutralCharacter/StoneGolemn/Blueprint/StoneGolemn_BP.StoneGolemn_BP_C|GetActivationCost (Variables|Default|GetStoneGolemn))) " Pts"))
        (Variables|/Game/Controllers/PlayerControllers/CustomPlayerController_BP.CustomPlayerController_BP_C|SetPropInRange _ascustom_player_controller_bp self)))))

(event OnComponentEndOverlap(TriggerRadius)
  (params (OverlappedComponent :type Primitive%20Component%20Object%20Reference) (OtherActor :type Actor%20Object%20Reference) (OtherComp :type Primitive%20Component%20Object%20Reference) (OtherBodyIndex :type Integer))
  (if (not (Variables|/Game/Characters/NPC/NeutralCharacter/StoneGolemn/Blueprint/StoneGolemn_BP.StoneGolemn_BP_C|GetisActivated (Variables|Default|GetStoneGolemn)))
    (bind _asknight_bp (Utilities|Casting|CastToKnight_BP OtherActor))
    (bind _ascustom_player_controller_bp (Utilities|Casting|CastToCustomPlayerController_BP (Game|GetPlayerController (Variables|/Game/Characters/AbstractCharacter.AbstractCharacter_C|GetplayerIndex _asknight_bp))))
    (Default|RemoveInteractionNotification _ascustom_player_controller_bp)
    (Variables|/Game/Controllers/PlayerControllers/CustomPlayerController_BP.CustomPlayerController_BP_C|SetPropInRange _ascustom_player_controller_bp 0)))

(event EventBeginPlay)

(event Collision|EventActorBeginOverlap
  (params (OtherActor :type Actor%20Object%20Reference)))

(event EventTick
  (params (DeltaSeconds :type Float%20%28single-precision%29))
  (bind _activationradius (Variables|Default|GetActivationRadius))
  ;[1 1 1] Swap from blue to green material when ready
  (if (CallFunction|IsReady)
    (Rendering|Material|SetMaterial _activationradius 0 "/Game/GameData/VisualProps/RadiusIndicator/MInstance_ActivatingIndicator.MInstance_ActivatingIndicator")
    (else
      (Rendering|Material|SetMaterial _activationradius 0 "/Game/GameData/VisualProps/RadiusIndicator/MInstance_AbilityIndicator.MInstance_AbilityIndicator"))))

(event EventActivate
  (params (PlayerIndex :type Integer))
  (Utilities|IsValid (Variables|Default|GetStoneGolemn)
    (:Is%20Valid
      (Default|WakeUp (Variables|Default|GetStoneGolemn))
      (Variables|Default|SetEarlyActivate false))))

(fn ConstructionScript
  (bind _returnvalue (Rendering|Material|CreateDynamicMaterialInstance (Variables|Default|GetDamageRadius) 0 "/Game/GameData/VisualProps/RadiusIndicator/MInstance_DamageIndicator.MInstance_DamageIndicator" "None" :!class /Script/Engine.PrimitiveComponent))
  (Rendering|Material|SetScalarParameterValue _returnvalue "Emission" 0.0 :!class /Script/Engine.MaterialInstanceDynamic)
  (Variables|Default|SetCooldownTime 1e+01))

(fn LinktoGolemn
  (params (Golemn :type Stone%20Golemn%20BP%20Object%20Reference))
  (Variables|Default|SetStoneGolemn Golemn))