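; Feeding trap Blueprint that launches a pair of chains forward when activated.
; On BeginPlay it spawns two Chain_BP actors behind, above and to either side of itself, storing them in a Chains array.
; Activate stores the player index, waits briefly, then plays the ShootAcceleration timeline, which moves each chain along its forward vector every update with sweep enabled.
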(event EventBeginPlay
  (bind _returnvalue (Transformation|GetActorTransform))
  (bind _returnvalue_2 (Transformation|GetActorRightVector))
  (bind _returnvalue_3 (Transformation|GetActorRightVector))
  (bind _returnvalue_4 (Transformation|GetActorForwardVector))
  (bind _returnvalue_5 (Transformation|GetActorForwardVector))
  (bind _returnvalue_6 (Transformation|GetActorTransform))
  (bind _returnvalue_7 (* _returnvalue_2 -1e+02))
  (bind _returnvalue_8 (* _returnvalue_3 1e+02))
  (bind _returnvalue_9 (* _returnvalue_4 -1e+02))
  (bind _returnvalue_10 (* _returnvalue_5 -1e+02))
  (bind _returnvalue_11 (+ _returnvalue_7 _returnvalue_10))
  (bind _returnvalue_12 (+ _returnvalue_8 _returnvalue_9))
  (bind _returnvalue_13 (+ _returnvalue_11 (.location _returnvalue_6)))
  (bind _returnvalue_14 (+ _returnvalue_12 (.location _returnvalue)))
  (|CallParentFunction)
  (bind _returnvalue_15 (Game|SpawnActorfromClass "/Game/Traps/Feedingtrap/Chain_BP.Chain_BP_C" (Math|Transform|MakeTransform (Math|Vector|MakeVector (.x _returnvalue_14) (.y _returnvalue_14) (+ (.z _returnvalue_14) 1e+02)) (.rotation _returnvalue) (.scale _returnvalue)) "Undefined" 0 0))
  (Utilities|Array|SetArrayElem (Variables|Default|GetChains) 0 _returnvalue_15 true)
  (bind _returnvalue_16 (Game|SpawnActorfromClass "/Game/Traps/Feedingtrap/Chain_BP.Chain_BP_C" (Math|Transform|MakeTransform (Math|Vector|MakeVector (.x _returnvalue_13) (.y _returnvalue_13) (+ (.z _returnvalue_13) 1e+02)) (.rotation _returnvalue_6) (.scale _returnvalue_6)) "Undefined" 0 0))
  (Utilities|Array|SetArrayElem (Variables|Default|GetChains) 1 _returnvalue_16 true))

(event EventActivate
  (params (PlayerIndex :type Integer))
  (Variables|Default|SetPlayerIndex PlayerIndex)
  (Utilities|FlowControl|Delay 0.5)
  (bind _accelaration (Timeline|ShootAcceleration PlayFromStart)
    (:Update
      (for _array_element (Variables|Default|GetChains)
        (Transformation|SetActorLocation _array_element (+ (Transformation|GetActorLocation _array_element) (* (Transformation|GetActorForwardVector _array_element) _accelaration)) true false)))))

(fn ConstructionScript
  (|CallParentFunction))