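; Spinning blade trap that a knight player can activate for a points cost, damaging characters that touch its blades.
; The trigger volume shows or clears the player's interaction prompt, and the indicator material reflects whether the trap is ready.
; Activation plays a looping spin animation and swing sound for a fixed duration.
; While spinning, a socket-attached blade volume deals physical damage on overlap, crediting PlayerIndex's controller.
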(event OnComponentBeginOverlap(TriggerVolume)
  (params (OverlappedComponent :type Primitive%20Component%20Object%20Reference) (OtherActor :type Actor%20Object%20Reference) (OtherComp :type Primitive%20Component%20Object%20Reference) (OtherBodyIndex :type Integer) (bFromSweep :type Boolean) (SweepResult :type Hit%20Result%20Structure%20%28by%20ref%29))
  ;[1 1 1] Notify the player is in range for activation
  ;;[1 1 1] For Tutorial purpose
  (if (Variables|Default|GetCanActivate)
    (bind _asknight_bp (Utilities|Casting|CastToKnight_BP OtherActor))
    ;;[1 1 1] Player in range
    (Utilities|IsValid (Variables|/Game/Characters/AbstractCharacter.AbstractCharacter_C|GetCharacterController _asknight_bp)
      (:Is%20Valid
        (bind _ascustom_player_controller_bp (Utilities|Casting|CastToCustomPlayerController_BP (Variables|/Game/Characters/AbstractCharacter.AbstractCharacter_C|GetCharacterController _asknight_bp)))
        (Default|NotifyOfInteraction _ascustom_player_controller_bp "Activate trap" (Utilities|String|Append (Utilities|String|ToString(Integer) (Variables|Default|GetActivationCost)) " Pts"))
        (Variables|/Game/Controllers/PlayerControllers/CustomPlayerController_BP.CustomPlayerController_BP_C|SetPropInRange _ascustom_player_controller_bp self))
      (:Is%20Not%20Valid
        (bind _ascustom_player_controller_bp_2 (Utilities|Casting|CastToCustomPlayerController_BP (Game|GetPlayerController (Variables|/Game/Characters/AbstractCharacter.AbstractCharacter_C|GetplayerIndex _asknight_bp))))
        (Default|NotifyOfInteraction _ascustom_player_controller_bp_2 "Activate trap" (Utilities|String|Append (Utilities|String|ToString(Integer) (Variables|Default|GetActivationCost)) " Pts"))
        (Variables|/Game/Controllers/PlayerControllers/CustomPlayerController_BP.CustomPlayerController_BP_C|SetPropInRange _ascustom_player_controller_bp_2 self)))))

(event OnComponentBeginOverlap(BladesVolume)
  (params (OverlappedComponent :type Primitive%20Component%20Object%20Reference) (OtherActor :type Actor%20Object%20Reference) (OtherComp :type Primitive%20Component%20Object%20Reference) (OtherBodyIndex :type Integer) (bFromSweep :type Boolean) (SweepResult :type Hit%20Result%20Structure%20%28by%20ref%29))
  ;[1 1 1] Apply damage upon overlap
  (if (Variables|Default|GetisSpinning)
    (bind _asabstract_character (Utilities|Casting|CastToAbstractCharacter OtherActor))
    (Game|Damage|ApplyDamage _asabstract_character (Variables|Default|GetBaseDamage) (Game|GetPlayerController (Variables|Default|GetPlayerIndex)) self "/Game/GameData/Damages/DamageType_Physical.DamageType_Physical_C")))

(event OnComponentEndOverlap(TriggerVolume)
  (params (OverlappedComponent :type Primitive%20Component%20Object%20Reference) (OtherActor :type Actor%20Object%20Reference) (OtherComp :type Primitive%20Component%20Object%20Reference) (OtherBodyIndex :type Integer))
  ;[1 1 1] Notify the player is in range for activation
  ;;[1 1 1] player out of range
  (if (Variables|Default|GetCanActivate)
    (bind _asknight_bp (Utilities|Casting|CastToKnight_BP OtherActor))
    (bind _ascustom_player_controller_bp (Utilities|Casting|CastToCustomPlayerController_BP (Variables|/Game/Characters/AbstractCharacter.AbstractCharacter_C|GetCharacterController _asknight_bp))
      (:then
        (Variables|/Game/Controllers/PlayerControllers/CustomPlayerController_BP.CustomPlayerController_BP_C|SetPropInRange _ascustom_player_controller_bp 0)
        (Default|RemoveInteractionNotification _ascustom_player_controller_bp))
      (:CastFailed
        (bind _ascustom_player_controller_bp_2 (Utilities|Casting|CastToCustomPlayerController_BP (Game|GetPlayerController (Variables|/Game/Characters/AbstractCharacter.AbstractCharacter_C|GetplayerIndex _asknight_bp))))
        (Default|RemoveInteractionNotification _ascustom_player_controller_bp_2)))))

(event Custom|PlaySound
  (if (Variables|Default|GetisSpinning)
    (bind _astop_down_game_mode (Utilities|Casting|CastToTopDownGameMode (Game|GetGameMode)))
    (Audio|PlaySoundatLocation _astop_down_game_mode "/Game/Traps/SpinningBlades/Sound/Swing_1.Swing_1" (Transformation|GetActorLocation) "0, 0, 0" 1.0 1.0 0.0 0 0 0)))

(event EventBeginPlay)

(event Collision|EventActorBeginOverlap
  (params (OtherActor :type Actor%20Object%20Reference)))

(event EventTick
  (params (DeltaSeconds :type Float%20%28single-precision%29))
  ;[1 1 1] Swap from blue to green material when ready
  (if (CallFunction|IsReady)
    (Rendering|Material|SetMaterial (Variables|Default|GetActivationRadius) 0 "/Game/GameData/VisualProps/RadiusIndicator/MInstance_ActivatingIndicator.MInstance_ActivatingIndicator")
    (else
      (Rendering|Material|SetMaterial (Variables|Default|GetActivationRadius) 0 "/Game/GameData/VisualProps/RadiusIndicator/MInstance_AbilityIndicator.MInstance_AbilityIndicator")
      (Variables|Default|SethasAdded false))))

(event EventActivate
  (params (PlayerIndex :type Integer))
  ;[1 1 1] Handling prop activation
  (|CallParentFunction PlayerIndex)
  (if (CallFunction|IsReady)
    (Variables|Default|SetEarlyActivate false)
    (Variables|Default|SetActivatedTime (Utilities|Time|GetGameTimeinSeconds))
    (Components|Animation|PlayAnimation (Variables|Default|GetSkeletalMesh) "/Game/Traps/SpinningBlades/Assets/SpinningBlade_AnimSpin.SpinningBlade_AnimSpin" true)
    (Variables|Default|SetisSpinning true)
    (CallFunction|PlaySound)
    (Utilities|Time|SetTimerbyEvent (delegate Custom|PlaySound) 0.5 true)
    (Utilities|FlowControl|Delay 1e+01)
    (Components|Animation|PlayAnimation (Variables|Default|GetSkeletalMesh) "/Game/Traps/SpinningBlades/Assets/SpinningBlade_AnimIdle.SpinningBlade_AnimIdle" false)
    (Variables|Default|SetisSpinning false)
    (else
      (Development|PrintString "Still in cooldown"))))

(fn ConstructionScript
  (bind _bladesvolume (Variables|Default|GetBladesVolume))
  (bind _returnvalue (Transformation|GetWorldRotation _bladesvolume))
  (|CallParentFunction)
  (Transformation|AttachComponentToComponent (Variables|Default|GetBladesVolume) (Variables|Default|GetSkeletalMesh) "blades_boneSocket" "SnapToTarget" "SnapToTarget" "KeepWorld" true)
  (Transformation|SetWorldRotation _bladesvolume (Math|Rotator|MakeRotator 0.0 (.pitch _returnvalue) (.yaw _returnvalue)) false false)
  (Variables|Default|SetCooldownTime 1e+01)
  (Variables|Default|SetActivationCost 150))

(fn SetObjectLocationRotation
  (params (Object :type Static%20Mesh%20Component%20Object%20Reference) (Location :type Vector) (Rotation :type Rotator))
  (bind _output_get (LocalVariables|SetStaticMesh Object))
  (Transformation|SetWorldLocationAndRotation _output_get Location Rotation false false))

(fn GetActivationRadius
  (return (Variables|/Script/Engine.SphereComponent|GetSphereRadius (Variables|Default|GetTriggerVolume))))